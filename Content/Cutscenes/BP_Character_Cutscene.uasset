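; BP_Character_Cutscene is a cutscene character that walks up to a referenced Cat and kneels.
; On BeginPlay it applies its own walk speed to CharacterMovement and loops a walking animation directly on the mesh.
; Cammina then uses AI Move To toward the Cat's PuntoDiArrivo component, if the Cat is valid, and plays a one-shot kneel animation when the move succeeds.
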(event Custom|Cammina
  (bind _cat (Variables|Default|GetCat)
    (:then
      (AI|AIMoveTo self (Transformation|GetWorldLocation (Variables|/Game/Cutscenes/BP_Cat_Cutscene.BP_Cat_Cutscene_C|GetPunto%20di%20arrivo _cat)) 0 5.0 false
        (:OnSuccess
          (Components|Animation|PlayAnimation (Variables|Character|GetMesh) "/Game/Cutscenes/Kneel_Anim_mixamo_com.Kneel_Anim_mixamo_com" false))))
    (:else)))

(event Custom|Set%20Velocity
  (Variables|/Script/Engine.CharacterMovementComponent|SetMaxWalkSpeed (Variables|Character|GetCharacterMovement) (Variables|Default|GetMax%20Walk%20Speed)))

(event EventBeginPlay
  (CallFunction|SetVelocity)
  (Components|Animation|PlayAnimation (Variables|Character|GetMesh) "/Game/Cutscenes/Walking_Cutscene.Walking_Cutscene" true)
  (CallFunction|Cammina))

(fn ConstructionScript)
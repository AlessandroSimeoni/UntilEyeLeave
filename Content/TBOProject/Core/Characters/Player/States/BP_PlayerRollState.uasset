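; BP_PlayerRollState is the player character state that handles rolling.
; StartRolling plays the roll montage on the main character's mesh at a configurable speed and calls TryEndRolling when the montage blends out.
; Invulnerability during the roll is disabled, leaving its toggles and a jump-state interrupt check as unconnected nodes.
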(event EventStartRolling
  (Animation|Montage|PlayMontage (Variables|/Script/Engine.Character|GetMesh (Variables|Default|GetMainCharacter)) (Variables|Default|GetRollAnimMontage) (Variables|Default|GetRollAnimationSpeed)
    (:OnBlendOut
      (Class|PlayerRollState|TryEndRolling))))
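; Player ledge grab state that mantles the main character onto ledges from mid-air or from the ground.
; Mid-air grabs snap the capsule to the wall, then play a mantle montage with component-relative Motion Warping targets, relaxing world collision until a notify.
; Grounded grabs play a jump montage with a notify-driven capsule shift forward and up.
; The state ends on mantle blend-out or grounded move completion.
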(event Custom|LedgeGrabAnimationProcess
  (bind _bp_maincharacter (Variables|Default|GetBP_MainCharacter))
  (bind _verticalledgehitresult (Variables|Default|GetVerticalLedgeHitResult))
  (bind _bp_maincharacter_2 (Variables|Default|GetBP_MainCharacter))
  (bind _bp_maincharacter_3 (Variables|Default|GetBP_MainCharacter))
  (bind _horizontalledgehitresult (Variables|Default|GetHorizontalLedgeHitResult))
  (bind _returnvalue (Transformation|GetActorRotation _bp_maincharacter))
  (bind (_bblockinghit _binitialoverlap _time _distance _location _impactpoint _normal _impactnormal _physmat _hitactor _hitcomponent) (Collision|BreakHitResult _verticalledgehitresult))
  (bind (_bblockinghit_2 _binitialoverlap_2 _time_2 _distance_2 _location_2 _impactpoint_2 _normal_2 _impactnormal_2 _physmat_2 _hitactor_2 _hitcomponent_2) (Collision|BreakHitResult _horizontalledgehitresult))
  (bind _capsulecomponent (Variables|/Script/Engine.Character|GetCapsuleComponent _bp_maincharacter_2))
  (bind _capsulecomponent_2 (Variables|/Script/Engine.Character|GetCapsuleComponent _bp_maincharacter_3))
  (EventDispatchers|UnbindallEventsfromMoveComponentCompleted (Variables|Default|GetBP_MainCharacter))
  (bind _returnvalue_2 (Class|MotionWarping|GetMotionWarpingComponent _bp_maincharacter))
  (Class|MotionWarpingComponent|AddorUpdateWarpTarget _returnvalue_2 (Utilities|Struct|MakeMotionWarpingTarget "Ledge Grab Up" "0.000000,0.000000,0.000000" _returnvalue _hitcomponent "None" true (CallFunction|GrabUpWarpTargetOffset (.z _impactpoint) _hitcomponent) "0.000000,0.000000,0.000000"))
  (Class|MotionWarpingComponent|AddorUpdateWarpTarget _returnvalue_2 (Utilities|Struct|MakeMotionWarpingTarget "Ledge Grab Forward" "0.000000,0.000000,0.000000" _returnvalue _hitcomponent_2 "None" true (CallFunction|GrabForwardWarpTargetOffset _impactpoint_2 _hitcomponent_2) "0.000000,0.000000,0.000000"))
  (Animation|Montage|PlayMontage (Variables|Default|GetCharacterMesh) "/Game/TBOProject/Art/MainCharacter/Animation/AM_MantleLedge.AM_MantleLedge" (Variables|Default|GetMidAirClimbPlayRate) 0.0 "StartGrab"
    (:then
      (Collision|SetCollisionResponsetoChannel _capsulecomponent_2 "ECC_WorldStatic" "ECR_Ignore")
      (Collision|SetCollisionResponsetoChannel _capsulecomponent_2 "ECC_WorldDynamic" "ECR_Overlap"))
    (:OnBlendOut
      (Class|PlayerLedgeGrabState|EndLedgeGrab))
    (:OnNotifyBegin
      (Collision|SetCollisionResponsetoChannel _capsulecomponent "ECC_WorldStatic" "ECR_Block")
      (Collision|SetCollisionResponsetoChannel _capsulecomponent "ECC_WorldDynamic" "ECR_Block"))))

(event Custom|OnGroundedMoveComponentEnd
  ;[1 0.6342 0.4948] Grounded Ledge Grab
  (EventDispatchers|UnbindallEventsfromMoveComponentCompleted (Variables|Default|GetBP_MainCharacter))
  (Class|PlayerLedgeGrabState|EndLedgeGrab))

(event EventStartMidAirLedgeGrab
  (bind _horizontalledgehitresult (Variables|Default|GetHorizontalLedgeHitResult))
  (bind _capsuledistancefromwall (Variables|Default|GetCapsuleDistanceFromWall))
  (bind (_bblockinghit _binitialoverlap _time _distance _location _impactpoint _normal _impactnormal) (Collision|BreakHitResult _horizontalledgehitresult))
  (bind _returnvalue (* _capsuledistancefromwall _impactnormal))
  (bind _returnvalue_2 (+ _impactpoint _returnvalue))
  (EventDispatchers|BindEventtoMoveComponentCompleted (Variables|Default|GetBP_MainCharacter) (delegate Custom|LedgeGrabAnimationProcess))
  (Default|MoveComponent (Variables|Default|GetBP_MainCharacter) (Variables|Default|GetCharacterCapsuleComponent) (Math|Vector|MakeVector (.x _returnvalue_2) (.y _returnvalue_2) (- (.z (.ImpactPoint (Collision|BreakHitResult (Variables|Default|GetVerticalLedgeHitResult)))) (Variables|Default|GetCapsuleVerticalOffsetFromLedge))) (Math|Rotator|MakeRotfromX (* _impactnormal -1.0)) 0.05))

(event EventOnInit
  (bind _maincharacter (Variables|Default|GetMainCharacter))
  ;[1 0.4792 0.4792] Initialize blueprint variables
  (bind _asbp_main_character (Utilities|Casting|CastToBP_MainCharacter _maincharacter))
  (bind _output_get (Variables|Default|SetBP_MainCharacter _asbp_main_character))
  (Variables|Default|SetCharacterCapsuleComponent (Variables|/Script/Engine.Character|GetCapsuleComponent _output_get))
  (Variables|Default|SetCharacterMesh (Variables|/Script/Engine.Character|GetMesh _maincharacter)))

(event EventStartGroundedLedgeGrab
  (bind _bp_maincharacter (Variables|Default|GetBP_MainCharacter))
  (bind _charactercapsulecomponent (Variables|Default|GetCharacterCapsuleComponent))
  (bind _charactermesh (Variables|Default|GetCharacterMesh))
  (bind _maincharacter (Variables|Default|GetMainCharacter))
  (bind _relativerotation (Variables|/Script/Engine.SceneComponent|GetRelativeRotation _charactercapsulecomponent))
  ;[1 0.6342 0.4948] Grounded Ledge Grab
  (EventDispatchers|BindEventtoMoveComponentCompleted (Variables|Default|GetBP_MainCharacter) (delegate Custom|OnGroundedMoveComponentEnd))
  ;;[1 0.6416 0.2292] Rotate Towards Ground Normal
  (Default|MoveComponent _bp_maincharacter _charactercapsulecomponent (Transformation|GetActorLocation _bp_maincharacter) _relativerotation 0.1)
  (Animation|Montage|PlayMontage _charactermesh "/Game/TBOProject/Art/MainCharacter/Animation/AM_RunningJump_Retarget.AM_RunningJump_Retarget" (Variables|Default|GetGroundedClimbPlayRate)
    (:OnNotifyBegin
      (Default|MoveComponent (Variables|Default|GetBP_MainCharacter) (Variables|Default|GetCharacterCapsuleComponent) (+ (+ (Transformation|GetWorldLocation (Variables|Default|GetCharacterCapsuleComponent)) (* (Variables|Default|GetGroundedEndingCapsuleForwardOffset) (Transformation|GetActorForwardVector _maincharacter))) (* (Transformation|GetActorUpVector _maincharacter) (Variables|Default|GetGroundedEndingCapsuleUpwardOffset))) _relativerotation 0.15))
    (:OnNotifyEnd
      (Class|AnimInstance|MontageStopwithBlendOut (Components|SkeletalMesh|GetAnimInstance _charactermesh) (Utilities|Struct|MakeAlphaBlendArgs 0 0.3 "HermiteCubic") "/Game/TBOProject/Art/MainCharacter/Animation/AM_RunningJump_Retarget.AM_RunningJump_Retarget"))))

(fn GrabUpWarpTargetOffset
  (params (ImpactPointZ :type Float%20%28double-precision%29) (HitComponent :type Primitive%20Component%20Object%20Reference))
  (bind _bp_maincharacter (Variables|Default|GetBP_MainCharacter))
  (bind _returnvalue (Transformation|GetActorLocation _bp_maincharacter))
  (bind _returnvalue_2 (Transformation|GetActorForwardVector _bp_maincharacter))
  (bind _returnvalue_3 (* _returnvalue_2 55.0))
  (bind _returnvalue_4 (+ _returnvalue _returnvalue_3))
  (return (Math|Transform|InverseTransformLocation (Transformation|GetWorldTransform HitComponent) (Math|Vector|MakeVector (.x _returnvalue_4) (.y _returnvalue_4) (+ ImpactPointZ 1e+01)))))

(fn GrabForwardWarpTargetOffset
  (params (ImpactPoint :type Vector) (HitComponent :type Primitive%20Component%20Object%20Reference))
  (bind _midairendingcapsuleforwardoffset (Variables|Default|GetMidAirEndingCapsuleForwardOffset))
  (bind _bp_maincharacter (Variables|Default|GetBP_MainCharacter))
  (bind _returnvalue (Transformation|GetActorForwardVector _bp_maincharacter))
  (bind _returnvalue_2 (* _midairendingcapsuleforwardoffset _returnvalue))
  (bind _returnvalue_3 (+ ImpactPoint _returnvalue_2))
  (return (Math|Transform|InverseTransformLocation (Transformation|GetWorldTransform HitComponent) (Math|Vector|MakeVector (.x _returnvalue_3) (.y _returnvalue_3) (+ (.z (Transformation|GetActorLocation _bp_maincharacter)) (- (Variables|/Script/Engine.CapsuleComponent|GetCapsuleHalfHeight (Variables|/Script/Engine.Character|GetCapsuleComponent _bp_maincharacter)) 88.0))))))
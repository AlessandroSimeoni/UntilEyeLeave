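; Gameplay ability for the second attack in the player's melee combo, activated by an event carrying the player combat state.
; It clears the Window1 tag, commits, and plays a grounded or mid-air montage at the event magnitude's rate.
; The combo-open event adds Window2 and signals that the window opened, while the window-end event or montage end ends the ability.
; Ending removes Window2 and, unless cancelled, tells the combat state to end the attack.
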(event Ability|EventOnEndAbility
  (params (bWasCancelled :type Boolean))
  (Ability|GameplayEffect|RemoveLooseGameplayTags (Ability|GetAvatarActorfromActorInfo) (Variables|Default|GetWindow2))
  (if (not bWasCancelled)
    (Class|PlayerCombatState|EndAttack (Variables|Default|GetAs%20BP%20Player%20Combat%20State))))

(event Ability|EventActivateAbilityFromEvent
  (params (EventData :type Gameplay%20Event%20Data%20Structure%20%28by%20ref%29))
  (Ability|GameplayEffect|RemoveLooseGameplayTags (Ability|GetAvatarActorfromActorInfo) (Variables|Default|GetWindow1))
  (bind _asbp_player_combat_state (Utilities|Casting|CastToBP_PlayerCombatState (.optionalobject EventData)))
  (Variables|Default|SetAs%20BP%20Player%20Combat%20State _asbp_player_combat_state)
  (Ability|CommitAbility)
  (Ability|SendGameplayEventtoActor (Ability|GetAvatarActorfromActorInfo) "(TagName=\"Event.CommitAttack\")")
  (|PlayMontageandWaitProxy "None" (select (AI|Components|NavMovement|IsMovingonGround (Pawn|GetMovementComponent (Variables|/Script/TBO_01.PlayerStateBase|GetMainCharacter (Variables|Default|GetAs%20BP%20Player%20Combat%20State)))) (Variables|Default|GetGroundedMontageToPlay) (Variables|Default|GetMidAirMontageToPlay)) (.eventmagnitude EventData) "None" true 1.0 0.0 false
    (:then
      (Ability|Tasks|WaitGameplayEvent "(TagName=\"Event.ComboWindowOpen\")" 0
        (:then
          (Ability|Tasks|WaitGameplayEvent "(TagName=\"Event.ComboWindowEnd\")" 0
            (:EventReceived
              (Ability|EndAbility))))
        (:EventReceived
          (Ability|GameplayEffect|AddLooseGameplayTags (Ability|GetAvatarActorfromActorInfo) (Variables|Default|GetWindow2))
          (Ability|SendGameplayEventtoActor (Ability|GetAvatarActorfromActorInfo) "(TagName=\"Event.AbilityComboWindowOpen\")"))))
    (:OnCompleted
      (Ability|EndAbility :!label _label))
    (:OnBlendOut
      (goto _label))
    (:OnInterrupted
      (Ability|CancelAbility)
      (goto _label))
    (:OnCancelled
      (goto _label))))
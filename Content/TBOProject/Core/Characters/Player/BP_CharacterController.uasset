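; Player controller that owns the HUD widget stack and drives journal, pause and game-over screens, plus debug cheats.
; JournalManager fragment events show either a timed trigger pop-up or a section-specific pickup widget that near-freezes time through global dilation.
; Menus are pushed onto activatable widget stacks and switch input to UI, with the journal opening on the manager's pending tab.
; Alt-key cheats teleport, heal, toggle immortality and grant coins, gated by the locomotion input context.
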(event Custom|OnFragmentCollected_Event
  (params (ENtryID :type Name) (Section :type EPageType%20Enum :default "Map") (IsTrigger :type Boolean))
  (if IsTrigger
    (CallFunction|RemoveHudStack)
    (bind _returnvalue (Class|CommonActivatableWidgetContainerBase|AddWidget (Variables|/Game/TBOProject/UI/JournalWidget/W_HUDStack.W_HUDStack_C|GetPopUpStack (Variables|Default|GetHud_StackWidget)) "/Game/TBOProject/UI/JournalWidget/W_FragmentPopUp.W_FragmentPopUp_C"))
    (Variables|Default|SetPopUpTrigger _returnvalue)
    (Utilities|Time|SetTimerbyFunctionName 0 "RemovePopUpStack" (Variables|Default|GetPopUpTime))
    (else
      (CallFunction|RemovePopUpStack)
      (CallFunction|RemoveHudStack)
      (if (Utilities|Enum|Equal(Enum) Section "Bestiary")
        (bind _returnvalue_2 (Class|CommonActivatableWidgetContainerBase|AddWidget (Variables|/Game/TBOProject/UI/JournalWidget/W_HUDStack.W_HUDStack_C|GetHudStack (Variables|Default|GetHud_StackWidget)) "/Game/TBOProject/UI/JournalWidget/W_FragmentPickUp.W_FragmentPickUp_C"))
        (Variables|Default|SetBestiariWidgetPickUp _returnvalue_2)
        (Utilities|Time|SetGlobalTimeDilation 0.0001)
        (elif (Utilities|Enum|Equal(Enum) Section "Lore")
          (bind _returnvalue_3 (Class|CommonActivatableWidgetContainerBase|AddWidget (Variables|/Game/TBOProject/UI/JournalWidget/W_HUDStack.W_HUDStack_C|GetHudStack (Variables|Default|GetHud_StackWidget)) "/Game/TBOProject/UI/JournalWidget/W_LorePickUp.W_LorePickUp_C"))
          (Variables|Default|SetLoreWidgetPickUp _returnvalue_3)
          (Utilities|Time|SetGlobalTimeDilation 0.0001)
          (else
            (bind _returnvalue_4 (Class|CommonActivatableWidgetContainerBase|AddWidget (Variables|/Game/TBOProject/UI/JournalWidget/W_HUDStack.W_HUDStack_C|GetHudStack (Variables|Default|GetHud_StackWidget)) "/Game/TBOProject/UI/JournalWidget/W_MapPickUp.W_MapPickUp_C"))
            (Variables|Default|SetMapWidgetPickUp _returnvalue_4)
            (Utilities|Time|SetGlobalTimeDilation 0.0001)))))))

(event Custom|OnPauseDeactivated_Event
  (EventDispatchers|UnbindEventfromBPonWidgetActivated (Variables|Default|GetPauseWidget) (delegate Custom|OnPauseDeactivated_Event))
  (Utilities|FlowControl|Delay 0.2)
  (Variables|Default|SetGameInPause false)
  (Variables|Default|SetbShowMouseCursor false)
  (Input|SetInputModeGameOnly self false))

(event EventBeginPlay
  (bind _returnvalue (Actor|GetActorOfClass "/Script/TBO_01.JournalManager"))
  (Variables|Default|SetJournalManager _returnvalue)
  (bind _returnvalue_2 (UserInterface|CreateWidget "/Game/TBOProject/UI/JournalWidget/W_HUDStack.W_HUDStack_C" self))
  (bind _output_get (Variables|Default|SetHud_StackWidget _returnvalue_2))
  (UserInterface|Viewport|AddtoViewport _output_get 0)
  (bind _journalmanager (Variables|Default|GetJournalManager)
    (:then
      (EventDispatchers|AssignOnFragmentCollected _journalmanager (delegate Custom|OnFragmentCollected_Event))
      (bind _returnvalue_3 (Class|CommonActivatableWidgetContainerBase|AddWidget (Variables|/Game/TBOProject/UI/JournalWidget/W_HUDStack.W_HUDStack_C|GetMenuStack (Variables|Default|GetHud_StackWidget)) "/Game/TBOProject/UI/JournalWidget/W_Journal.W_Journal_C"))
      (Class|CommonActivatableWidget|DeactivateWidget _returnvalue_3))
    (:else)))

(event EventShowGameOver
  (bind _returnvalue (Class|CommonActivatableWidgetContainerBase|AddWidget (Variables|/Game/TBOProject/UI/JournalWidget/W_HUDStack.W_HUDStack_C|GetMenuStack (Variables|Default|GetHud_StackWidget)) "/Game/TBOProject/UI/GameOver/W_GameOver.W_GameOver_C"))
  (Input|SetInputModeUIOnly self _returnvalue "DoNotLock" false))

(event EventToggleMenu
  (CallFunction|RemovePopUpStack)
  (CallFunction|RemoveHudStack)
  (bind _returnvalue (Class|CommonActivatableWidgetContainerBase|AddWidget (Variables|/Game/TBOProject/UI/JournalWidget/W_HUDStack.W_HUDStack_C|GetMenuStack (Variables|Default|GetHud_StackWidget)) "/Game/TBOProject/UI/JournalWidget/W_Journal.W_Journal_C"))
  (switch int (Variables|/Script/TBO_01.JournalManager|GetIndexToOpen (Variables|Default|GetJournalManager))
    (:0
      (Class|CommonTabListWidgetBase|SelectTabbyID (Variables|/Game/TBOProject/UI/JournalWidget/W_Journal.W_Journal_C|GetJTab _returnvalue) "Map" false))
    (:1
      (Class|CommonTabListWidgetBase|SelectTabbyID (Variables|/Game/TBOProject/UI/JournalWidget/W_Journal.W_Journal_C|GetJTab _returnvalue) "Bestiary" false))
    (:2
      (Class|CommonTabListWidgetBase|SelectTabbyID (Variables|/Game/TBOProject/UI/JournalWidget/W_Journal.W_Journal_C|GetJTab _returnvalue) "Lore" false)))
  (Variables|/Script/TBO_01.JournalManager|SetIndexToOpen (Variables|Default|GetJournalManager) 0)
  (Game|SetGamePaused true)
  (Variables|Default|SetbShowMouseCursor true)
  (Input|SetInputModeUIOnly self _returnvalue "DoNotLock" false))

(event EventToggleGamePause
  (if (not (Variables|Default|GetGameInPause))
    (Variables|Default|SetGameInPause true)
    (bind _returnvalue (Class|CommonActivatableWidgetContainerBase|AddWidget (Variables|/Game/TBOProject/UI/JournalWidget/W_HUDStack.W_HUDStack_C|GetMenuStack (Variables|Default|GetHud_StackWidget)) "/Game/TBOProject/UI/Pause/W_Pause.W_Pause_C"))
    (bind _output_get (Variables|Default|SetPauseWidget _returnvalue))
    (EventDispatchers|BindEventtoBPonWidgetDeactivated _output_get (delegate Custom|OnPauseDeactivated_Event))
    (Input|SetInputModeUIOnly self _output_get "DoNotLock" false)))

(event Input|KeyboardEvents|Alt8
  (params (Key :type Key%20Structure :default "None"))
  ;[0 0.02818 1] CHEATS
  ;;[0 1 0.9385] 99 Coins
  (:Pressed
    (if (.ReturnValue (Class|EnhancedInputSubsystemInterface|HasMappingContext (PlayerController|LocalPlayerSubsystems|GetEnhancedInputLocalPlayerSubsystem) "/Game/TBOProject/Core/Input/IMC_Locomotion.IMC_Locomotion"))
      (Class|MainCharacter|SetCoin (Variables|Default|GetPossessedMainCharacter) 99.0)
      (Default|SetCheatText (Variables|/Game/TBOProject/Core/Gamemodes/Play/GM_Play.GM_Play_C|GetHUDWidget (.AsGM%20Play (Utilities|Casting|CastToGM_Play (Game|GetGameMode)))) "Cheat Activated: 
Wealthness"))))

(event Input|KeyboardEvents|Alt6
  (params (Key :type Key%20Structure :default "None"))
  (bind _possessedmaincharacter (Variables|Default|GetPossessedMainCharacter))
  (bind _lifecomponent (Variables|/Script/TBO_01.MainCharacter|GetLifeComponent _possessedmaincharacter))
  ;[0 0.02818 1] CHEATS
  ;;[0 1 0.009654] Full Heal
  (:Pressed
    (if (.ReturnValue (Class|EnhancedInputSubsystemInterface|HasMappingContext (PlayerController|LocalPlayerSubsystems|GetEnhancedInputLocalPlayerSubsystem) "/Game/TBOProject/Core/Input/IMC_Locomotion.IMC_Locomotion"))
      (Class|LifeSystemComponent|ReceiveHeal _lifecomponent (Variables|/Script/TBO_01.LifeSystemComponent|GetMaxHealth _lifecomponent))
      (Default|SetCheatText (Variables|/Game/TBOProject/Core/Gamemodes/Play/GM_Play.GM_Play_C|GetHUDWidget (.AsGM%20Play (Utilities|Casting|CastToGM_Play (Game|GetGameMode)))) "Cheat Activated: 
Health restored"))))

(event Input|KeyboardEvents|Alt1
  (params (Key :type Key%20Structure :default "None"))
  ;[0 0.02818 1] CHEATS
  ;;[1 0.9943 0] Piazza centrale
  (:Pressed
    (if (and (not (Variables|Default|GetBossfightActivated)) (.ReturnValue (Class|EnhancedInputSubsystemInterface|HasMappingContext (PlayerController|LocalPlayerSubsystems|GetEnhancedInputLocalPlayerSubsystem) "/Game/TBOProject/Core/Input/IMC_Locomotion.IMC_Locomotion")))
      (CallFunction|TeleportCheat "12736.951908,-24274.868488,-300.000001")
      (Default|SetCheatText (Variables|/Game/TBOProject/Core/Gamemodes/Play/GM_Play.GM_Play_C|GetHUDWidget (.AsGM%20Play (Utilities|Casting|CastToGM_Play (Game|GetGameMode)))) "Cheat Activated: 
Teleported to Nightmare roots"))))

(event Input|KeyboardEvents|Alt2
  (params (Key :type Key%20Structure :default "None"))
  ;[0 0.02818 1] CHEATS
  ;;[1 0.9943 0] Primo checkpoint path Gio
  (:Pressed
    (if (and (not (Variables|Default|GetBossfightActivated)) (.ReturnValue (Class|EnhancedInputSubsystemInterface|HasMappingContext (PlayerController|LocalPlayerSubsystems|GetEnhancedInputLocalPlayerSubsystem) "/Game/TBOProject/Core/Input/IMC_Locomotion.IMC_Locomotion")))
      (CallFunction|TeleportCheat "16837.915280,-26302.437691,955.000000")
      (Default|SetCheatText (Variables|/Game/TBOProject/Core/Gamemodes/Play/GM_Play.GM_Play_C|GetHUDWidget (.AsGM%20Play (Utilities|Casting|CastToGM_Play (Game|GetGameMode)))) "Cheat Activated: 
Teleported to Tainted tree"))))

(event Input|KeyboardEvents|Alt3
  (params (Key :type Key%20Structure :default "None"))
  ;[0 0.02818 1] CHEATS
  ;;[1 0.9943 0] Secondo checkpoint path Fra
  (:Pressed
    (if (and (not (Variables|Default|GetBossfightActivated)) (.ReturnValue (Class|EnhancedInputSubsystemInterface|HasMappingContext (PlayerController|LocalPlayerSubsystems|GetEnhancedInputLocalPlayerSubsystem) "/Game/TBOProject/Core/Input/IMC_Locomotion.IMC_Locomotion")))
      (CallFunction|TeleportCheat "20042.451326,-17711.193689,-2370.436686")
      (Default|SetCheatText (Variables|/Game/TBOProject/Core/Gamemodes/Play/GM_Play.GM_Play_C|GetHUDWidget (.AsGM%20Play (Utilities|Casting|CastToGM_Play (Game|GetGameMode)))) "Cheat Activated: 
Teleported to Ragged hood"))))

(event Input|KeyboardEvents|Alt4
  (params (Key :type Key%20Structure :default "None"))
  ;[0 0.02818 1] CHEATS
  ;;[1 0.9943 0] Primo Checkpoint path Simo
  (:Pressed
    (if (and (not (Variables|Default|GetBossfightActivated)) (.ReturnValue (Class|EnhancedInputSubsystemInterface|HasMappingContext (PlayerController|LocalPlayerSubsystems|GetEnhancedInputLocalPlayerSubsystem) "/Game/TBOProject/Core/Input/IMC_Locomotion.IMC_Locomotion")))
      (CallFunction|TeleportCheat "22495.000000,-23494.999996,540.000000")
      (Default|SetCheatText (Variables|/Game/TBOProject/Core/Gamemodes/Play/GM_Play.GM_Play_C|GetHUDWidget (.AsGM%20Play (Utilities|Casting|CastToGM_Play (Game|GetGameMode)))) "Cheat Activated: 
Teleported to Gloomway stop"))))

(event Input|KeyboardEvents|Alt5
  (params (Key :type Key%20Structure :default "None"))
  ;[0 0.02818 1] CHEATS
  ;;[1 0.9943 0] Boss
  (:Pressed
    (if (and (not (Variables|Default|GetBossfightActivated)) (.ReturnValue (Class|EnhancedInputSubsystemInterface|HasMappingContext (PlayerController|LocalPlayerSubsystems|GetEnhancedInputLocalPlayerSubsystem) "/Game/TBOProject/Core/Input/IMC_Locomotion.IMC_Locomotion")))
      (CallFunction|TeleportCheat "-9802.769894,-23878.153450,5817.688750")
      (Default|SetCheatText (Variables|/Game/TBOProject/Core/Gamemodes/Play/GM_Play.GM_Play_C|GetHUDWidget (.AsGM%20Play (Utilities|Casting|CastToGM_Play (Game|GetGameMode)))) "Cheat Activated: 
Teleported to Trauma arisen"))))

(event Input|KeyboardEvents|Alt7
  (params (Key :type Key%20Structure :default "None"))
  (bind _possessedmaincharacter (Variables|Default|GetPossessedMainCharacter))
  (bind _lifecomponent (Variables|/Script/TBO_01.MainCharacter|GetLifeComponent _possessedmaincharacter))
  ;[0 0.02818 1] CHEATS
  ;;[1 0.439 0] Toggle Player Immortality
  (:Pressed
    (if (.ReturnValue (Class|EnhancedInputSubsystemInterface|HasMappingContext (PlayerController|LocalPlayerSubsystems|GetEnhancedInputLocalPlayerSubsystem) "/Game/TBOProject/Core/Input/IMC_Locomotion.IMC_Locomotion"))
      (bind _output_get (Variables|/Script/TBO_01.LifeSystemComponent|SetImmortal _lifecomponent (not (Variables|/Script/TBO_01.LifeSystemComponent|GetImmortal _lifecomponent))))
      (Default|SetCheatText (Variables|/Game/TBOProject/Core/Gamemodes/Play/GM_Play.GM_Play_C|GetHUDWidget (.AsGM%20Play (Utilities|Casting|CastToGM_Play (Game|GetGameMode)))) (select _output_get "Cheat Activated: 
Invicibility ON" "Cheat Activated: 
Invicibility OFF")))))

(fn ConstructionScript)

(fn RemoveHudStack
  (bind _lorewidgetpickup (Variables|Default|GetLoreWidgetPickUp))
  (bind _bestiariwidgetpickup (Variables|Default|GetBestiariWidgetPickUp))
  (bind _mapwidgetpickup (Variables|Default|GetMapWidgetPickUp))
  (Utilities|FlowControl|Sequence
    (:then_0
      (if (Utilities|IsValid _bestiariwidgetpickup)
        (Class|CommonActivatableWidget|DeactivateWidget _bestiariwidgetpickup)))
    (:then_1
      (if (Utilities|IsValid _lorewidgetpickup)
        (Class|CommonActivatableWidget|DeactivateWidget _lorewidgetpickup)))
    (:then_2
      (if (Utilities|IsValid _mapwidgetpickup)
        (Class|CommonActivatableWidget|DeactivateWidget _mapwidgetpickup)))))

(fn RemovePopUpStack
  (bind _popuptrigger (Variables|Default|GetPopUpTrigger))
  (if (Utilities|IsValid _popuptrigger)
    (Class|CommonActivatableWidget|DeactivateWidget _popuptrigger)))

(fn TeleportCheat
  (params (TeleportLocation :type Vector))
  (bind _returnvalue (Game|GetPlayerCharacter 0))
  (Transformation|SetActorLocation _returnvalue (+ TeleportLocation (Math|Vector|MakeVector 0.0 0.0 (Variables|/Script/Engine.CapsuleComponent|GetCapsuleHalfHeight (Variables|/Script/Engine.Character|GetCapsuleComponent _returnvalue)))) false false))
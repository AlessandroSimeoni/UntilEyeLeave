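; Player character Blueprint that attaches the bat weapon, plays heal and damage feedback, and freezes with the camera detached on death.
; BeginPlay loads the save to derive max health, weapon level with its mesh, and coins, then blinks capsule collision for camera modifiers.
; A looping timer traces downward to place a decal as a fake shadow.
; Helpers ease components to target transforms and hide weapon and shadow while sitting at checkpoints.
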(event OnDeath(LifeComponent)
  (params (This :type Scene%20Component%20Object%20Reference))
  (bind _charactermovement (Variables|Character|GetCharacterMovement))
  ;[1 1 1] HandleGameOver
  (bind _asgm_play (Utilities|Casting|CastToGM_Play (Game|GetGameMode)))
  (Class|GameCamera|Detach (Variables|/Game/TBOProject/Core/Gamemodes/Play/GM_Play.GM_Play_C|GetGameCamera _asgm_play))
  (Utilities|FlowControl|Delay 0.75)
  (Components|Movement|StopMovementImmediately _charactermovement)
  (Variables|/Script/Engine.CharacterMovementComponent|SetGravityScale _charactermovement 0.0))

(event Custom|OnMoveComponent
  (params (Component :type Scene%20Component%20Object%20Reference) (TargetLocation :type Vector) (TargetRotation :type Rotator) (OverTime :type Float%20%28double-precision%29))
  (Components|MoveComponentTo Component TargetLocation TargetRotation true true OverTime false)
  (Default|CallMoveComponentCompleted))

(event Custom|AttachWeaponToHand
  ;[1 1 1] Attach weapon to hand socket
  (Transformation|AttachComponentToComponent (Variables|Default|GetWeaponMesh_Test) (Variables|Character|GetMesh) "WeaponSocket" "SnapToTarget" "SnapToTarget" "SnapToTarget" true))

(event Custom|OnHealReceived_Event
  (params (This :type Scene%20Component%20Object%20Reference) (HealthReceived :type Float%20%28single-precision%29))
  (if (not (Variables|Default|GetIsBeginPlay))
    (Components|Activation|Activate (Variables|Default|GetHealingVFX) false)
    ;[1 1 1] Heal SFX
    (Audio|PlaySound2D "/Game/TBOProject/Media/Sound/MainCharacter/SFX_Player_Healing.SFX_Player_Healing" 1.0 1.0 0.0 0 0 false)))

(event Custom|CastShadow
  (bind _capsulecomponent (Variables|Default|GetCapsuleComponent))
  (bind _returnvalue (Transformation|GetWorldLocation _capsulecomponent))
  ;[1 1 1] Move decal to create a fake shadow effect
  ;;[0.1192 0.09891 0.5365] Fire event looping with timer
  (bind _outhit (Collision|LineTraceByChannel _returnvalue (- _returnvalue (Math|Vector|MakeVector 0.0 0.0 (Variables|Default|GetTrace%20Lenght))) "TraceTypeQuery1" false 0 "None" true "(R=1.000000,G=0.000000,B=0.000000,A=1.000000)" "(R=0.000000,G=1.000000,B=0.000000,A=1.000000)" 0.5))
  ;;[0.1192 0.09891 0.5365] Move the decal to the linetrace impact location
  (Transformation|SetWorldLocation (Variables|Default|GetShadow%20Decal) (.location _outhit) false false))

(event Custom|OnDamageTakenEvent
  (params (This :type Scene%20Component%20Object%20Reference) (DamageReceived :type Float%20%28single-precision%29))
  ;[1 1 1] Damage SFX
  (Audio|PlaySound2D "/Game/TBOProject/Media/Sound/MetasoundSystems/MS_PlayerDamaged.MS_PlayerDamaged" 1.0 1.0 0.0 0 0 false))

(event Custom|ChangeWeapon
  (params (Index :type Integer))
  ;[1 1 1] Weapon mesh change when level up
  (Components|StaticMesh|SetStaticMesh (Variables|Default|GetWeaponMesh_Test) (Utilities|Select :Index Index :Option%200 "/Game/TBOProject/Characters/Player/Weapon/SM_BaseballBat.SM_BaseballBat" :Option%201 "/Game/TBOProject/Characters/Player/Weapon/SM_BaseballBat.SM_BaseballBat" :Option%202 "/Game/TBOProject/Characters/Player/Weapon/SM_BaseballBatUpgraded.SM_BaseballBatUpgraded")))

(event EventBeginPlay
  (bind _capsulecomponent (Variables|Default|GetCapsuleComponent))
  (bind _lifecomponent (Variables|Default|GetLifeComponent))
  (Utilities|FlowControl|Sequence
    (:then_0
      (EventDispatchers|BindEventtoMoveComponentEvent (delegate Custom|OnMoveComponent))
      (CallFunction|AttachWeapontoHand)
      (EventDispatchers|AssignOnHealReceived _lifecomponent (delegate Custom|OnHealReceived_Event))
      (EventDispatchers|BindEventtoOnDamageTaken _lifecomponent (delegate Custom|OnDamageTakenEvent))
      ;[1 0.2703 0.1705] Load health/weapon level/coins
      (bind _returnvalue (Class|SaveSubsystem|LoadGame (Subsystems|GetSaveSubsystem)))
      (CallFunction|LoadHealth _returnvalue)
      (CallFunction|LoadWeaponLevel _returnvalue)
      (CallFunction|LoadCoin _returnvalue)
      (Variables|Default|SetIsBeginPlay false)
      ;[0.2722 0.8901 1] Collision blink for camera modifiers
      (Collision|SetCollisionEnabled _capsulecomponent "NoCollision")
      (Utilities|FlowControl|DelayUntilNextTick)
      (Collision|SetCollisionEnabled _capsulecomponent "QueryAndPhysics"))
    (:then_1
      ;[1 1 1] Move decal to create a fake shadow effect
      ;;[0.1192 0.09891 0.5365] Fire event looping with timer
      (Utilities|Time|SetTimerbyEvent (delegate Custom|CastShadow) 0.03 true))))

(fn ConstructionScript)

(fn MoveComponent
  (params (Component :type Scene%20Component%20Object%20Reference) (TargetLocation :type Vector) (TargetRotation :type Rotator) (OverTime :type Float%20%28double-precision%29))
  (Default|CallMoveComponentEvent Component TargetLocation TargetRotation OverTime))

(fn LoadHealth
  (params (TBOSaveGame :type TBO%20Save%20Game%20Object%20Reference))
  (bind _lifecomponent (Variables|Default|GetLifeComponent))
  (bind _output_get (Variables|/Script/TBO_01.LifeSystemComponent|SetMaxHealth _lifecomponent (+ (/ (Variables|/Script/TBO_01.TBOSaveGame|GetLifeShardsCollected TBOSaveGame) (Variables|Default|GetHealthIncreaseLifeShards)) (Variables|/Script/TBO_01.LifeSystemComponent|GetMaxHealth _lifecomponent))))
  (Class|LifeSystemComponent|ReceiveHeal _lifecomponent _output_get)
  (Class|PlayerHealthBar|ResizeHealthBar (Variables|/Script/TBO_01.HUDWidget|GetHealthBar (Variables|/Game/TBOProject/Core/Gamemodes/Play/GM_Play.GM_Play_C|GetHUDWidget (.AsGM%20Play (Utilities|Casting|CastToGM_Play (Game|GetGameMode)))))))

(fn LoadWeaponLevel
  (params (TBOSaveGame :type TBO%20Save%20Game%20Object%20Reference))
  (bind _output_get (Variables|Default|SetCurrentWeaponLevel (+ (/ (Variables|/Script/TBO_01.TBOSaveGame|GetWeaponPartsCollected TBOSaveGame) (Variables|Default|GetLevelIncreaseWeaponParts)) (Variables|Default|GetCurrentWeaponLevel))))
  (CallFunction|ChangeWeapon (Math|Float|Truncate _output_get)))

(fn HandleSittingatCheckpoints
  (params (StartSitting :type Boolean))
  (Development|SetHiddeninGame (Variables|Default|GetWeaponMesh_Test) StartSitting false)
  (Development|SetHiddeninGame (Variables|Default|GetShadow%20Decal) StartSitting false))

(fn LoadCoin
  (params (SaveGame :type TBO%20Save%20Game%20Object%20Reference))
  (bind _coinscollected (Variables|/Script/TBO_01.TBOSaveGame|GetCoinsCollected SaveGame))
  (Development|PrintString (Utilities|String|ToString(Integer) _coinscollected))
  (Class|MainCharacter|SetCoin (Math|Conversions|ToFloat(Integer) _coinscollected)))
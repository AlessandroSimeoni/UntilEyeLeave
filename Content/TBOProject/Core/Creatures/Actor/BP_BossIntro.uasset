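; BP_BossIntro runs the intro sequence for the B05 boss head when a character enters.
; If the boss controller is in its Sleeping phase, it changes the game camera's manual offset and disables the player controller's tick.
; A timer then advances the boss to its next phase and binds to its phase-change event.
; When Phase 1 is reported, it flips the camera's default-offset flag and re-enables the player controller's tick.
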(event Custom|OnPhaseChange_Event
  (params (BossPhase :type EBossPhase%20Enum :default "Sleep"))
  (switch Utilities|FlowControl|Switch|SwitchonEBossPhase BossPhase
    (:Phase1
      (Class|GameCamera|SetManualOffset (Variables|Default|GetGame%20Camera) (Variables|Default|GetOffset) false)
      (Actor|Tick|SetActorTickEnabled (Game|GetPlayerController 0) true))))

(event Custom|CustomEvent
  (bind _as_bp_b05_boss_head_controller (Variables|Default|GetAs%20BP%20B05%20Boss%20Head%20Controller))
  (Class|B05BossHeadController|NextPhase _as_bp_b05_boss_head_controller)
  (EventDispatchers|AssignOnPhaseChange _as_bp_b05_boss_head_controller (delegate Custom|OnPhaseChange_Event)))

(event EventOnCharacterEnter
  (params (GameCamera :type Game%20Camera%20Object%20Reference))
  (Variables|Default|SetGame%20Camera GameCamera)
  (bind _asbp_b05_boss_head_controller (Utilities|Casting|CastToBP_B05_BossHead_Controller (Pawn|GetController (Variables|Default|GetBossHead))))
  (bind _output_get (Variables|Default|SetAs%20BP%20B05%20Boss%20Head%20Controller _asbp_b05_boss_head_controller))
  (switch Utilities|FlowControl|Switch|SwitchonEBossPhase (Variables|/Script/TBO_01.B05_BossHead_Controller|GetCurrentPhase _output_get)
    (:Sleep
      (Class|GameCamera|SetManualOffset (Variables|Default|GetGame%20Camera) (Variables|Default|GetOffset) true)
      (Actor|Tick|SetActorTickEnabled (Game|GetPlayerController 0))
      (Utilities|Time|SetTimerbyEvent (delegate Custom|CustomEvent) (Variables|Default|GetTime)))))

(fn ConstructionScript)
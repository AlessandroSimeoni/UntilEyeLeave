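; Trigger actor that starts a target creature's scripted patrol when the main character overlaps it, firing only once.
; It binds to the creature's ScriptedController completion callback and releases its stop state.
; On completion it clears the creature's assigned spline patrol path, unpossesses it, then spawns a configured AI controller at its transform to possess it, handing over from scripted movement to AI.
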(event Custom|OnScriptedPatrolCompleted_Event
  (bind _targetcreature (Variables|Default|GetTargetCreature))
  (bind _returnvalue (Class|PatrolInterface|GetPatrolSplineComponent(Message) (Variables|Default|GetTargetCreature)))
  (Variables|/Script/TBO_01.PatrolSplineComponent|SetAssignedPatrolPath _returnvalue 0)
  (Pawn|UnPossess (stale Collision|EventActorBeginOverlap _asscripted_controller))
  (bind _returnvalue_2 (Game|SpawnActorfromClass (Variables|Default|GetAI%20Controller%20Class) (Transformation|GetActorTransform _targetcreature) "Undefined" "MultiplyWithRoot" 0 0))
  (Pawn|Possess _returnvalue_2 _targetcreature))

(event EventBeginPlay)

(event Collision|EventActorBeginOverlap
  (params (OtherActor :type Actor%20Object%20Reference))
  (if (not (Variables|Default|GetTriggered))
    (Utilities|Casting|CastToMainCharacter OtherActor)
    (bind _asscripted_controller (Utilities|Casting|CastToScriptedController (Pawn|GetController (Variables|Default|GetTargetCreature))))
    (EventDispatchers|AssignOnScriptedPatrolCompleted _asscripted_controller (delegate Custom|OnScriptedPatrolCompleted_Event))
    (Variables|Default|SetTriggered true)
    (Class|ScriptedController|SetStop _asscripted_controller false)
    (Development|PrintText "Overlap")))

(fn ConstructionScript)
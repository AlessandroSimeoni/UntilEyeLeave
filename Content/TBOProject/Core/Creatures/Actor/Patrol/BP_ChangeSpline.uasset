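; BP_ChangeSpline is a trigger actor that switches a creature's patrol route when the player walks into it.
; On the first overlap by MainCharacter it sets a one-shot flag, then gets the referenced Creature's patrol spline component.
; If both are valid, it clears the creature's blackboard "Position" value and assigns NewPatrolPath as the new patrol path.
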(event EventTick
  (params (DeltaSeconds :type Float%20%28single-precision%29)))

(event Collision|EventActorBeginOverlap
  (params (OtherActor :type Actor%20Object%20Reference))
  (bind _creature (Variables|Default|GetCreature))
  (if (not (Variables|Default|GetTriggered))
    (Utilities|Casting|CastToMainCharacter OtherActor)
    (Variables|Default|SetTriggered true)
    (Utilities|IsValid _creature
      (:Is%20Valid
        (bind _returnvalue (Class|PatrolInterface|GetPatrolSplineComponent _creature))
        (Utilities|IsValid _returnvalue
          (:Is%20Valid
            (AI|Components|Blackboard|ClearValue (AI|GetBlackboard (Pawn|GetController (Variables|Default|GetCreature))) (Utilities|Name|MakeLiteralName "Position"))
            (Variables|/Script/TBO_01.PatrolSplineComponent|SetAssignedPatrolPath _returnvalue (Variables|Default|GetNewPatrolPath))))))))

(fn ConstructionScript)
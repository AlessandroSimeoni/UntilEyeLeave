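; Trigger actor that switches a B01 Gianguscio creature to a new patrol path when it enters.
; On begin overlap it fetches the creature's patrol spline component and, after a short delay, assigns it NewPatrolPath.
; It also clears the Position blackboard key and sets IsPatrolPathAssigned on the creature's AI, then prints debug text.
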(event EventTick
  (params (DeltaSeconds :type Float%20%28single-precision%29)))

(event Collision|EventActorBeginOverlap
  (params (OtherActor :type Actor%20Object%20Reference))
  (bind _asbp_b01_gianguscio_creature_base (Utilities|Casting|CastToBP_B01_Gianguscio_CreatureBase OtherActor))
  (bind _returnvalue (Class|PatrolInterface|GetPatrolSplineComponent(Message) _asbp_b01_gianguscio_creature_base))
  (Utilities|FlowControl|Delay 0.2)
  (Utilities|IsValid _returnvalue
    (:Is%20Valid
      (AI|Components|Blackboard|ClearValue (AI|GetBlackboard (Pawn|GetController _asbp_b01_gianguscio_creature_base)) (Utilities|Name|MakeLiteralName "Position"))
      (Variables|/Script/TBO_01.PatrolSplineComponent|SetAssignedPatrolPath _returnvalue (Variables|Default|GetNewPatrolPath))
      (AI|Components|Blackboard|SetValueasBool (AI|GetBlackboard (Pawn|GetController _asbp_b01_gianguscio_creature_base)) (Utilities|Name|MakeLiteralName "IsPatrolPathAssigned") true)
      (Development|PrintText "gianguscio"))))

(fn ConstructionScript)
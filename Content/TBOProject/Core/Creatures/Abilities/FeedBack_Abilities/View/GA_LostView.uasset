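; GA_LostView is a creature feedback Gameplay Ability that plays the response for losing view.
; On activation it executes the GameplayCue.Lost cue on the avatar, located at the owning component's "Spotted" socket in component space.
; It then removes a set of non-replicated loose gameplay tags from the avatar, clears the spotted combat audio through the audio subsystem, and ends immediately.
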(event Ability|EventActivateAbility
  (GameplayCue|ExecuteGameplayCueOnActor(Burst) (Ability|GetAvatarActorfromActorInfo) "(TagName=\"GameplayCue.Lost\")" (Ability|GameplayCue|MakeGameplayCueParameters :Location (.location (Transformation|GetSocketTransform (Class|GameplayAbility|GetOwningComponentfromActorInfo) "Spotted" "RTS_Component"))))
  (Ability|GameplayEffect|RemoveLooseGameplayTags (Ability|GetAvatarActorfromActorInfo) (Variables|Default|GetGameplay%20Tags))
  (Class|AudioSubsystem|RemoveSpottedCombatAudio (Subsystems|GetAudioSubsystem))
  (Ability|EndAbility))

(event Ability|EventOnEndAbility
  (params (bWasCancelled :type Boolean)))
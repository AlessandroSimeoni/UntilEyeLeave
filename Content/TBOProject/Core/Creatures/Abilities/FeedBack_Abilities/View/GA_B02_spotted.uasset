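; Gameplay ability that plays a creature's "spotted" feedback, judging by its name and cue.
; On activation it executes the Spotted gameplay cue on the avatar, passing the "Spotted" socket's component-space location.
; It adds non-replicated loose gameplay tags to the avatar, registers spotted combat audio with the audio subsystem, then ends immediately without removing those tags.
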(event Ability|EventActivateAbility
  (GameplayCue|ExecuteGameplayCueOnActor(Burst) (Ability|GetAvatarActorfromActorInfo) "(TagName=\"GameplayCue.Spotted\")" (Ability|GameplayCue|MakeGameplayCueParameters :Location (.location (Transformation|GetSocketTransform (Class|GameplayAbility|GetOwningComponentfromActorInfo) "Spotted" "RTS_Component"))))
  (Ability|GameplayEffect|AddLooseGameplayTags (Ability|GetAvatarActorfromActorInfo) (Variables|Default|GetGameplay%20Tags))
  (Class|AudioSubsystem|AddSpottedCombatAudio (Subsystems|GetAudioSubsystem))
  (Ability|EndAbility))

(event Ability|EventOnEndAbility
  (params (bWasCancelled :type Boolean)))
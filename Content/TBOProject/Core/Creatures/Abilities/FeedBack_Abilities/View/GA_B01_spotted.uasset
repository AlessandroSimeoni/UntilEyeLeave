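; Gameplay ability that plays the "spotted" feedback for creature B01 (Gianguscio).
; Unless the avatar has Status.Shielded, it fires the Spotted gameplay cue, passing the component-space location of the "Spotted" socket.
; It then adds a configurable set of non-replicated loose tags, starts spotted combat audio if Status.BrokenShell is present, and ends immediately.
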(event Ability|EventActivateAbility
  (bind _returnvalue (Ability|GetAvatarActorfromActorInfo))
  (Development|PrintText "Gianguscio Hello")
  (if (GameplayTags|HasMatchingGameplayTag (Ability|GetAbilitySystemComponent (Ability|GetAvatarActorfromActorInfo)) "(TagName=\"Status.Shielded\")")
    _
    (else
      (GameplayCue|ExecuteGameplayCueOnActor(Burst) (Ability|GetAvatarActorfromActorInfo) "(TagName=\"GameplayCue.Spotted\")" (Ability|GameplayCue|MakeGameplayCueParameters :Location (.location (Transformation|GetSocketTransform (Class|GameplayAbility|GetOwningComponentfromActorInfo) "Spotted" "RTS_Component"))))))
  (Ability|GameplayEffect|AddLooseGameplayTags _returnvalue (Variables|Default|GetGameplay%20Tags))
  (if (GameplayTags|HasMatchingGameplayTag (Ability|GetAbilitySystemComponent _returnvalue) "(TagName=\"Status.BrokenShell\")")
    (Class|AudioSubsystem|AddSpottedCombatAudio (Subsystems|GetAudioSubsystem)))
  (Ability|EndAbility))

(event Ability|EventOnEndAbility
  (params (bWasCancelled :type Boolean)))
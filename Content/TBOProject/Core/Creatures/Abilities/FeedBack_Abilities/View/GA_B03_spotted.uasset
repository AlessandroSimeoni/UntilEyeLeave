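; Gameplay ability for the B03 Birdman creature's "spotted" reaction, which moves it into chasing with an aggro animation.
; On activation it applies the chasing gameplay effect, adds non-replicated loose tags to the avatar and registers spotted combat audio.
; It fires the Spotted gameplay cue using the component-space location of the "Spotted" socket, then plays the aggro montage and ends when that finishes or is interrupted.
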(event Ability|EventActivateAbility
  (Ability|ApplyGameplayEffectToOwner "/Game/TBOProject/Core/Creatures/Abilities/Effects/GE_B03_Chasing.GE_B03_Chasing_C")
  (Ability|GameplayEffect|AddLooseGameplayTags (Ability|GetAvatarActorfromActorInfo) (Variables|Default|GetGameplay%20Tags))
  (Class|AudioSubsystem|AddSpottedCombatAudio (Subsystems|GetAudioSubsystem))
  (GameplayCue|ExecuteGameplayCueOnActor(Burst) (Ability|GetAvatarActorfromActorInfo) "(TagName=\"GameplayCue.Spotted\")" (Ability|GameplayCue|MakeGameplayCueParameters :Location (.location (Transformation|GetSocketTransform (Class|GameplayAbility|GetOwningComponentfromActorInfo) "Spotted" "RTS_Component"))))
  (|PlayMontageandWaitProxy "None" "/Game/TBOProject/Art/Creatures/Birdman/AM_B03_Aggro_Birdman_Montage.AM_B03_Aggro_Birdman_Montage" 1.0 "None" true 1.0 0.0 false
    (:OnCompleted
      _)
    (:OnBlendOut
      _)
    (:OnInterrupted
      _)
    (:OnCancelled
      _))
  (Ability|EndAbility))

(event Ability|EventOnEndAbility
  (params (bWasCancelled :type Boolean)))
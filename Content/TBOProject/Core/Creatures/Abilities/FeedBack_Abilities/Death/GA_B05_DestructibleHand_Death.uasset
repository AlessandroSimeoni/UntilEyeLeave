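; Death gameplay ability for the B05 DestructibleHand creature.
; On activation it sets the "Stop" blackboard key to false and starts the death montage.
; A half-second delay from montage start, rather than montage completion, leads to ending the ability and calling Death on the Creature avatar.
; Interruption or cancellation of the montage runs that same ending without the delay.
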(event Ability|EventActivateAbility
  (AI|Components|Blackboard|SetValueasBool (AI|GetBlackboard (AI|GetAIController (Ability|GetAvatarActorfromActorInfo))) (Utilities|Name|MakeLiteralName "Stop") false)
  (|PlayMontageandWaitProxy "None" "/Game/TBOProject/Art/Creatures/Boss/Animation/PawRX/AM_B05_DestructibleHand_PawRX_LP_Death_Montage.AM_B05_DestructibleHand_PawRX_LP_Death_Montage" 1.0 "None" true 1.0 0.0 false
    (:then
      (Utilities|FlowControl|Delay 0.5))
    (:OnInterrupted
      _)
    (:OnCancelled
      _))
  (Ability|EndAbility)
  (bind _ascreature (Utilities|Casting|CastToCreature (Ability|GetAvatarActorfromActorInfo)))
  (Class|Creature|Death _ascreature true))
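; GA_B05_Death is the death gameplay ability for the B05 boss head.
; On activation it advances the boss controller to the next phase, applies the death effect and shakes the mesh.
; Meanwhile, a self-rescheduling Explosion event fires death cues at random points inside the head's explosion volume.
; When the shake finishes, it triggers a giant explosion cue, ends the ability, kills the creature and starts the final cutscene.
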(event Custom|Explosion
  (bind _as_bp_b05_boss_head (Variables|Default|GetAs%20BP%20B05%20Boss%20Head))
  (bind _explosionvolume (Variables|/Game/TBOProject/Core/Creatures/Character/B05_Boss/Head/BP_B05_BossHead.BP_B05_BossHead_C|GetExplosionVolume _as_bp_b05_boss_head))
  (GameplayCue|ExecuteGameplayCueOnActor(Burst) _as_bp_b05_boss_head "(TagName=\"GameplayCue.Death\")" (Ability|GameplayCue|MakeGameplayCueParameters :Location (+ (* (Math|Random|RandomFloatinRange 0.0 (Variables|/Script/Engine.SphereComponent|GetSphereRadius _explosionvolume)) (Math|Random|RandomUnitVector)) (Transformation|GetWorldLocation _explosionvolume))))
  (Ability|Tasks|WaitDelay (Math|Random|RandomFloatinRange 0.2 0.5)
    (:OnFinish
      (CallFunction|Explosion))))

(event Ability|EventActivateAbility
  (bind _asbp_b05_boss_head (Utilities|Casting|CastToBP_B05_BossHead (Ability|GetAvatarActorfromActorInfo)))
  (bind _output_get (Variables|Default|SetAs%20BP%20B05%20Boss%20Head _asbp_b05_boss_head))
  (bind _asbp_b05_boss_head_controller (Utilities|Casting|CastToBP_B05_BossHead_Controller (Pawn|GetController _output_get)))
  (Class|B05BossHeadController|NextPhase _asbp_b05_boss_head_controller)
  (Ability|ApplyGameplayEffectToOwner "/Game/TBOProject/Core/Creatures/Abilities/Effects/GE_Death.GE_Death_C")
  (|VibrateMesh (Class|GameplayAbility|GetOwningComponentfromActorInfo) 3.0 1e+01
    (:then
      (CallFunction|Explosion))
    (:OnFinished
      (Development|PrintText "End")
      (GameplayCue|ExecuteGameplayCueOnActor(Burst) (Variables|Default|GetAs%20BP%20B05%20Boss%20Head) "(TagName=\"GameplayCue.GiantExplosion\")" (Ability|GameplayCue|MakeGameplayCueParameters :Location (Transformation|GetWorldLocation (Variables|/Game/TBOProject/Core/Creatures/Character/B05_Boss/Head/BP_B05_BossHead.BP_B05_BossHead_C|GetExplosionVolume (Variables|Default|GetAs%20BP%20B05%20Boss%20Head)))))
      (Ability|EndAbility)
      (bind _ascreature (Utilities|Casting|CastToCreature (Ability|GetAvatarActorfromActorInfo)))
      (Class|Creature|Death _ascreature true)
      ;[1 0.6319 0.1795] Final Cutscenes
      (Default|StartFinalCutsceneSequence (.AsGM%20Play (Utilities|Casting|CastToGM_Play (Game|GetGameMode)))))))

(event Ability|EventOnEndAbility
  (params (bWasCancelled :type Boolean)))
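; Gameplay ability that runs the death of creature B06.
; On activation it clears spotted combat audio if the creature has the Status.Spotted tag, applies GE_Death to itself and plays the death montage.
; As the montage starts, it sets the AI blackboard Stop key, waits briefly, then ends the ability and calls Death on the Creature.
; Without a valid blackboard it ends immediately, skipping that Death call.
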(event Ability|EventActivateAbility
  (bind _returnvalue (Ability|GetAvatarActorfromActorInfo))
  (bind _returnvalue_2 (AI|GetAIController _returnvalue))
  (bind _returnvalue_3 (AI|GetBlackboard _returnvalue_2))
  (if (GameplayTags|HasMatchingGameplayTag (Ability|GetAbilitySystemComponent (Ability|GetAvatarActorfromActorInfo)) "(TagName=\"Status.Spotted\")")
    (Class|AudioSubsystem|RemoveSpottedCombatAudio (Subsystems|GetAudioSubsystem)))
  (Ability|ApplyGameplayEffectToOwner "/Game/TBOProject/Core/Creatures/Abilities/Effects/GE_Death.GE_Death_C")
  (|PlayMontageandWaitProxy "None" "/Game/TBOProject/Art/Creatures/Stealer/B06_Artist/Animation/B06_Death_Montage.B06_Death_Montage" 1.0 "None" true 1.0 0.0 false
    (:then
      (Utilities|IsValid _returnvalue_3
        (:Is%20Valid
          (AI|Components|Blackboard|SetValueasBool _returnvalue_3 (Utilities|Name|MakeLiteralName "Stop") true)
          (Ability|Tasks|WaitDelay 1.0
            (:OnFinish
              (Ability|EndAbility)
              (bind _ascreature (Utilities|Casting|CastToCreature (Ability|GetAvatarActorfromActorInfo)))
              (Class|Creature|Death _ascreature true))))
        (:Is%20Not%20Valid
          (Ability|EndAbility))))))

(event Ability|EventOnEndAbility
  (params (bWasCancelled :type Boolean)))
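; GA_B01_InstantDeath is a gameplay ability that kills the owning creature immediately.
; On activation it applies GE_Death twice and removes spotted combat audio if the avatar has Status.Spotted.
; It starts the B02 stunned montage but continues from the immediate exec pin without waiting.
; It then repeats the spotted audio check, ends the ability and calls Death on the Creature avatar.
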(event Ability|EventActivateAbility
  (Ability|ApplyGameplayEffectToOwner "/Game/TBOProject/Core/Creatures/Abilities/Effects/GE_Death.GE_Death_C")
  (if (GameplayTags|HasMatchingGameplayTag (Ability|GetAbilitySystemComponent (Ability|GetAvatarActorfromActorInfo)) "(TagName=\"Status.Spotted\")")
    (Class|AudioSubsystem|RemoveSpottedCombatAudio (Subsystems|GetAudioSubsystem)))
  (Ability|ApplyGameplayEffectToOwner "/Game/TBOProject/Core/Creatures/Abilities/Effects/GE_Death.GE_Death_C")
  (|PlayMontageandWaitProxy "None" "/Game/TBOProject/Art/Creatures/Mousetrap/AM_B02_Stunned.AM_B02_Stunned" 1.0 "None" true 1.0 0.0 false
    (:then
      (bind _returnvalue (GameplayTags|HasMatchingGameplayTag(Message) (Ability|GetAvatarActorfromActorInfo) "(TagName=\"Status.Spotted\")"))
      (if _returnvalue
        (Class|AudioSubsystem|RemoveSpottedCombatAudio (Subsystems|GetAudioSubsystem)))
      (Ability|EndAbility)
      (bind _ascreature (Utilities|Casting|CastToCreature (Ability|GetAvatarActorfromActorInfo)))
      (Class|Creature|Death _ascreature true))))

(event Ability|EventOnEndAbility
  (params (bWasCancelled :type Boolean)))
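; Gameplay ability that handles death of the B03 Birdman creature.
; On activation, it proceeds only if the avatar has the Status.Spotted tag, removing spotted combat audio and applying GE_Death to the owner.
; It starts a slowed death montage, then after a fixed delay, without waiting for the montage to finish, ends the ability and calls Death on the Creature avatar.
; No branch handles an unspotted avatar.
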(event Ability|EventActivateAbility
  (if (GameplayTags|HasMatchingGameplayTag (Ability|GetAbilitySystemComponent (Ability|GetAvatarActorfromActorInfo)) "(TagName=\"Status.Spotted\")")
    (Class|AudioSubsystem|RemoveSpottedCombatAudio (Subsystems|GetAudioSubsystem))
    (Ability|ApplyGameplayEffectToOwner "/Game/TBOProject/Core/Creatures/Abilities/Effects/GE_Death.GE_Death_C")
    (|PlayMontageandWaitProxy "None" "/Game/TBOProject/Art/Creatures/Birdman/AM_B03_Death_Birdman_Montage.AM_B03_Death_Birdman_Montage" 0.6 "None" true 1.0 0.0 false
      (:then
        (Ability|Tasks|WaitDelay 1.5
          (:OnFinish
            (Development|PrintText "End")
            (Ability|EndAbility)
            (bind _ascreature (Utilities|Casting|CastToCreature (Ability|GetAvatarActorfromActorInfo)))
            (Class|Creature|Death _ascreature true)))))))

(event Ability|EventOnEndAbility
  (params (bWasCancelled :type Boolean)))
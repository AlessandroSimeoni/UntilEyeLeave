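; Gameplay ability that plays the B05 creature's StepOnHand death reaction.
; On activation it prints a debug message, sets the AI blackboard's "Stop" key to false and plays the left-paw death montage.
; When the montage completes, is interrupted or is cancelled, it ends the ability and then calls Death on the avatar Creature.
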(event Ability|EventActivateAbility
  (Development|PrintString "slow Death" true true "(R=1.000000,G=0.000000,B=0.172846,A=1.000000)")
  (AI|Components|Blackboard|SetValueasBool (AI|GetBlackboard (AI|GetAIController (Ability|GetAvatarActorfromActorInfo))) (Utilities|Name|MakeLiteralName "Stop") false)
  (|PlayMontageandWaitProxy "None" "/Game/TBOProject/Art/Creatures/Boss/Animation/PawLX/AM_B05_StepOnHand_PawSX_LP_Death_Montage.AM_B05_StepOnHand_PawSX_LP_Death_Montage" 1.0 "None" true 1.0 0.0 false
    (:OnCompleted
      _)
    (:OnInterrupted
      _)
    (:OnCancelled
      _))
  (Ability|EndAbility)
  (bind _ascreature (Utilities|Casting|CastToCreature (Ability|GetAvatarActorfromActorInfo)))
  (Class|Creature|Death _ascreature true))
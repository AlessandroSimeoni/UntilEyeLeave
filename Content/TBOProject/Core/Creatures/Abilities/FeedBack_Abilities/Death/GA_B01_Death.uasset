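; GA_B01_Death is the gameplay ability that runs a creature's death sequence.
; On activation it applies GE_Death to the owner and, if the avatar has the Status.Spotted tag, removes the spotted combat audio.
; It starts the AM_Hit_Gianguscio montage, then after a short fixed delay, without waiting for the montage to finish, prints a debug message, ends the ability and calls Death on the Creature avatar.
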(event Ability|EventActivateAbility
  (Ability|ApplyGameplayEffectToOwner "/Game/TBOProject/Core/Creatures/Abilities/Effects/GE_Death.GE_Death_C")
  (if (GameplayTags|HasMatchingGameplayTag (Ability|GetAbilitySystemComponent (Ability|GetAvatarActorfromActorInfo)) "(TagName=\"Status.Spotted\")")
    (Class|AudioSubsystem|RemoveSpottedCombatAudio (Subsystems|GetAudioSubsystem)))
  (|PlayMontageandWaitProxy "None" "/Game/TBOProject/Art/Creatures/Gianguscio/AM_Hit_Gianguscio.AM_Hit_Gianguscio" 1.0 "None" true 1.0 0.0 false
    (:then
      (Ability|Tasks|WaitDelay 0.2
        (:OnFinish
          (Development|PrintText "End")
          (Ability|EndAbility)
          (bind _ascreature (Utilities|Casting|CastToCreature (Ability|GetAvatarActorfromActorInfo)))
          (Class|Creature|Death _ascreature true))))))

(event Ability|EventOnEndAbility
  (params (bWasCancelled :type Boolean)))
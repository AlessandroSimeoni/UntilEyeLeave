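; Gameplay ability that gives creature B05 a hit stun reaction, starting with its dog head melee hit montage.
; When the montage completes, is interrupted or is cancelled, it prints a debug message, briefly vibrates the owning mesh and adds loose gameplay tags to the avatar.
; The ability ends when the vibration finishes, and OnEndAbility removes the non-replicated tags.
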(event Ability|EventActivateAbility
  (|PlayMontageandWaitProxy "None" "/Game/TBOProject/Art/Creatures/Boss/Animation/Head/AM_B05_Head_DogHeadRig_MeleeHit_Montage.AM_B05_Head_DogHeadRig_MeleeHit_Montage" 1.0 "None" true 1.0 0.0 false
    (:OnCompleted
      _)
    (:OnInterrupted
      _)
    (:OnCancelled
      _))
  (Development|PrintText "HitStun")
  (|VibrateMesh (Class|GameplayAbility|GetOwningComponentfromActorInfo) 0.3 5.0
    (:then
      (Ability|GameplayEffect|AddLooseGameplayTags (Ability|GetAvatarActorfromActorInfo) (Variables|Default|GetGameplay%20Tags)))
    (:OnFinished
      (Ability|EndAbility))))

(event Ability|EventOnEndAbility
  (params (bWasCancelled :type Boolean))
  (Ability|GameplayEffect|RemoveLooseGameplayTags (Ability|GetAvatarActorfromActorInfo) (Variables|Default|GetGameplay%20Tags)))
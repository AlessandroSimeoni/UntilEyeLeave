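; Event-triggered gameplay ability that resolves the impact of creature B02's run charge.
; It spawns FX and sound at the hit origin and ends at once, branching on target type in OnEndAbility.
; Stealers get deflect feedback, destructible parts take a Hit, a charged Birdman triggers charge feedback, and most others receive HitMessage.
; Outcomes converge on crash knockback, self-stun and usually OpenEyes, skipped when HitMessage succeeds on a Pierce-tagged target.
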(event Ability|EventOnEndAbility
  (params (bWasCancelled :type Boolean))
  (bind _returnvalue (Ability|GetAbilitySystemComponentfromActorInfo))
  (bind _returnvalue_2 (Ability|GetAbilitySystemComponentfromActorInfo))
  (bind _returnvalue_3 (Class|AbilitySystemComponent|GetGameplayAttributeValue _returnvalue "(AttributeName=\"KnockBackIntensity\",Attribute=/Script/TBO_01.BaseCreatureAttributeSet:KnockBackIntensity,AttributeOwner=\"/Script/CoreUObject.Class'/Script/TBO_01.BaseCreatureAttributeSet'\")"))
  (bind _returnvalue_4 (Class|AbilitySystemComponent|GetGameplayAttributeValue _returnvalue "(AttributeName=\"CharacterLevel\",Attribute=/Script/TBO_01.BaseCreatureAttributeSet:CharacterLevel,AttributeOwner=\"/Script/CoreUObject.Class'/Script/TBO_01.BaseCreatureAttributeSet'\")"))
  (bind _asb06_stealer (Utilities|Casting|CastToB06_Stealer (Variables|Default|GetEvent%20Data%20Target))
    (:then
      (Ability|SendGameplayEventtoActor _asb06_stealer "(TagName=\"FeedBack.DeflectHit\")" (Utilities|Struct|MakeGameplayEventData "(TagName=\"FeedBack.DeflectHit\")" (Ability|GetAvatarActorfromActorInfo) 0 0 0 "()" "(GameplayTags=)" "(GameplayTags=)" 0.5 "()"))
      (Ability|SendGameplayEvent "(TagName=\"FeedBack.NockBack.CrashNockback\")" (Utilities|Struct|MakeGameplayEventData "(TagName=\"\")" (Variables|Default|GetEvent%20Data%20Instigator) (Variables|Default|GetEvent%20Data%20Target) 0 0 "()" "(GameplayTags=)" "(GameplayTags=)" 1.0 "()") :!label _label)
      (Abilities|TryActivateAbilitybyClass _returnvalue_2 "/Game/TBOProject/Core/Creatures/Abilities/FeedBack_Abilities/HitStun/GA_B02_Stun.GA_B02_Stun_C" true)
      (Abilities|TryActivateAbilitybyClass _returnvalue_2 "/Game/TBOProject/Core/Creatures/Abilities/Action_Abilities/GA_OpenEyes.GA_OpenEyes_C" true))
    (:CastFailed
      (Utilities|Casting|CastToMainCharacter (Variables|Default|GetEvent%20Data%20Target)
        (:then
          (Variables|Default|SetIsPiercing (Actor|ActorHasTag (Variables|Default|GetEvent%20Data%20Target) "Pierce") :!label _label_2)
          (bind _returnvalue_5 (Class|HittableActor|Hit(Message) (Variables|Default|GetEvent%20Data%20Target) (Math|Float|Truncate _returnvalue_4) (.ReturnValue (Class|AbilitySystemComponent|GetGameplayAttributeValue _returnvalue "(AttributeName=\"Attack\",Attribute=/Script/TBO_01.BaseCreatureAttributeSet:Attack,AttributeOwner=\"/Script/CoreUObject.Class'/Script/TBO_01.BaseCreatureAttributeSet'\")")) (Variables|Default|GetEvent%20Data%20Instigator) _returnvalue_3))
          (if _returnvalue_5
            (if (not (Variables|Default|GetIsPiercing))
              (goto _label))
            (else
              (goto _label))))
        (:CastFailed
          (bind _asbp_b03_birdman_shooter_creature_base (Utilities|Casting|CastToBP_B03_Birdman_ShooterCreatureBase (Variables|Default|GetEvent%20Data%20Target))
            (:then
              (if (GameplayTags|HasMatchingGameplayTag (Ability|GetAbilitySystemComponent _asbp_b03_birdman_shooter_creature_base) "(TagName=\"Status.Charged\")")
                (Ability|SendGameplayEvent "(TagName=\"FeedBack.Charge\")" (Utilities|Struct|MakeGameplayEventData "(TagName=\"\")" 0 0 0 0 "()" "(GameplayTags=)" "(GameplayTags=)" 1.0 "()"))
                (Ability|SendGameplayEvent "(TagName=\"FeedBack.NockBack.CrashNockback\")" (Utilities|Struct|MakeGameplayEventData "(TagName=\"\")" (Variables|Default|GetEvent%20Data%20Instigator) (Variables|Default|GetEvent%20Data%20Target) 0 0 "()" "(GameplayTags=)" "(GameplayTags=)" 1.0 "()"))
                (Abilities|TryActivateAbilitybyClass (Ability|GetAbilitySystemComponentfromActorInfo) "/Game/TBOProject/Core/Creatures/Abilities/FeedBack_Abilities/HitStun/GA_B02_Stun.GA_B02_Stun_C" true)
                (else
                  (goto _label))))
            (:CastFailed
              (bind _asdestructible_parts (Utilities|Casting|CastToDestructibleParts (Variables|Default|GetEvent%20Data%20Optional%20Object))
                (:then
                  (Class|HittableActor|Hit _asdestructible_parts (Math|Float|Truncate _returnvalue_4) 0.0 (Variables|Default|GetEvent%20Data%20Instigator) _returnvalue_3)
                  (goto _label))
                (:CastFailed
                  (goto _label_2))))))))))

(event Ability|EventActivateAbilityFromEvent
  (params (EventData :type Gameplay%20Event%20Data%20Structure%20%28by%20ref%29))
  (bind _returnvalue (Class|AbilitySystemBlueprintLibrary|EffectContextGetOrigin (.contexthandle EventData)))
  (Variables|Default|SetEvent%20Data%20Instigator (.instigator EventData))
  (Variables|Default|SetEvent%20Data%20Target (.target EventData))
  (Variables|Default|SetEvent%20Data%20Optional%20Object (.optionalobject EventData))
  (Class|NiagaraFunctionLibrary|SpawnSystematLocationwithParams (Utilities|Struct|MakeFXSystemSpawnParameters self (Variables|Default|GetFX) _returnvalue "0.000000,0.000000,0.000000" "1.000000,1.000000,1.000000" 0 "None" "KeepWorldPosition" true true "None" true false))
  (Audio|PlaySoundatLocation (Variables|Default|GetSFX) _returnvalue "0, 0, 0" 1.0 1.0 0.0 0 0 0 0)
  (Ability|EndAbility))
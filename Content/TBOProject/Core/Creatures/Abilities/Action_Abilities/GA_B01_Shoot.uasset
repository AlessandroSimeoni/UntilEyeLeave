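; Gameplay ability for the B01 (Gianguscio) creature's ranged attack, firing normal or charged projectiles, chosen by the Status.Charged tag.
; Once the target is within angle, it plays the shooting montage, whose gameplay events trigger focus cancel, an attack-hint cue and the shot.
; Every available muzzle fires with attribute-driven stats, applying backward root-motion recoil into a timed recovery montage.
; Ending the ability applies the GE_ShootingDelay effect to the owner.
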(event Ability|EventOnEndAbility
  (params (bWasCancelled :type Boolean))
  (Ability|ApplyGameplayEffectToOwner "/Game/TBOProject/Core/Creatures/Abilities/Effects/GE_ShootingDelay.GE_ShootingDelay_C"))

(event Ability|EventActivateAbilityFromEvent
  (params (EventData :type Gameplay%20Event%20Data%20Structure%20%28by%20ref%29))
  (bind _returnvalue (Ability|GetAbilitySystemComponentfromActorInfo))
  (bind _output_get (Variables|Default|SetTarget (.target EventData)))
  (|WaitUntilTargetAngle _output_get 7e+01 0.1
    (:OnTargetInAngle
      (|PlayMontageandWaitProxy "None" "/Game/TBOProject/Art/Creatures/Gianguscio/AM_Attack_Gianguscio_Shooting.AM_Attack_Gianguscio_Shooting" 1.0 "None" true 1.0 0.0 false
        (:then
          (Ability|Tasks|WaitGameplayEvent "(TagName=\"Event.StopRotate\")" 0
            (:then
              (if (GameplayTags|HasMatchingGameplayTag (Ability|GetAbilitySystemComponentfromActorInfo) "(TagName=\"Status.Charged\")")
                (Variables|Default|SetCurrentProjectile (Variables|Default|GetProjectileTypeCharged))
                (else
                  (Variables|Default|SetCurrentProjectile (Variables|Default|GetProjectileType))))
              (Ability|Tasks|WaitGameplayEvent "(TagName=\"Event.CommitAttack\")" 0
                (:EventReceived
                  (Abilities|TryActivateAbilitybyClass (Ability|GetAbilitySystemComponentfromActorInfo) "/Game/TBOProject/Core/Creatures/Abilities/Action_Abilities/GA_CancelFocus.GA_CancelFocus_C" false)
                  (bind _returnvalue_2 (Class|Shooter|GetMuzzlesController(Message) (Ability|GetAvatarActorfromActorInfo)))
                  (bind _returnvalue_3 (Class|MuzzlesController|GetAvailableMuzzles _returnvalue_2))
                  (for _array_element _returnvalue_3
                    (Class|Muzzle|Shoot _array_element (Variables|Default|GetCurrentProjectile) (.ReturnValue (Class|AbilitySystemComponent|GetGameplayAttributeValue _returnvalue "(AttributeName=\"BulletSpeed\",Attribute=/Script/TBO_01.ShooterCreatureAttributeSet:BulletSpeed,AttributeOwner=\"/Script/CoreUObject.Class'/Script/TBO_01.B01DestructibleAttributeSet'\")")) (Variables|Default|GetTarget) (.ReturnValue (Class|AbilitySystemComponent|GetGameplayAttributeValue _returnvalue "(AttributeName=\"Attack\",Attribute=/Script/TBO_01.BaseCreatureAttributeSet:Attack,AttributeOwner=\"/Script/CoreUObject.Class'/Script/TBO_01.BaseCreatureAttributeSet'\")")) (.ReturnValue (Class|AbilitySystemComponent|GetGameplayAttributeValue _returnvalue "(AttributeName=\"CharacterLevel\",Attribute=/Script/TBO_01.BaseCreatureAttributeSet:CharacterLevel,AttributeOwner=\"/Script/CoreUObject.Class'/Script/TBO_01.BaseCreatureAttributeSet'\")")) (.ReturnValue (Class|AbilitySystemComponent|GetGameplayAttributeValue _returnvalue "(AttributeName=\"KnockBackIntensity\",Attribute=/Script/TBO_01.BaseCreatureAttributeSet:KnockBackIntensity,AttributeOwner=\"/Script/CoreUObject.Class'/Script/TBO_01.BaseCreatureAttributeSet'\")")))
                    (Ability|Tasks|ApplyRootMotionConstantForce "None" (Math|Vector|NegateVector (Transformation|GetActorForwardVector (Ability|GetAvatarActorfromActorInfo))) (.ReturnValue (Class|AbilitySystemComponent|GetGameplayAttributeValue _returnvalue "(AttributeName=\"ShootRecoilStrength\",Attribute=/Script/TBO_01.ShooterCreatureAttributeSet:ShootRecoilStrength,AttributeOwner=\"/Script/CoreUObject.Class'/Script/TBO_01.B01DestructibleAttributeSet'\")")) 0.1 false 0 "MaintainLastRootMotionVelocity" "0, 0, 0" 0.0 true
                      (:then
                        (|PlayMontageandWaitProxy "None" "/Game/TBOProject/Art/Creatures/Gianguscio/AM_B01_Recovery_Gianguscio_Montage.AM_B01_Recovery_Gianguscio_Montage" 1.0 "None" true 1.0 0.0 false))
                      (:OnFinish
                        (Ability|Tasks|WaitDelay (.ReturnValue (Class|AbilitySystemComponent|GetGameplayAttributeValue _returnvalue "(AttributeName=\"ShootRecoilTime\",Attribute=/Script/TBO_01.ShooterCreatureAttributeSet:ShootRecoilTime,AttributeOwner=\"/Script/CoreUObject.Class'/Script/TBO_01.B01DestructibleAttributeSet'\")"))
                          (:OnFinish
                            (Ability|Animation|MontageJumptoSection (Components|SkeletalMesh|GetAnimInstance (.skeletalmeshcomponent (Ability|GetActorInfo))) "EndLoop" "/Game/TBOProject/Art/Creatures/Gianguscio/AM_B01_Recovery_Gianguscio_Montage.AM_B01_Recovery_Gianguscio_Montage")
                            (Ability|EndAbility)))))))))
            (:EventReceived
              (Abilities|TryActivateAbilitybyClass (Ability|GetAbilitySystemComponentfromActorInfo) "/Game/TBOProject/Core/Creatures/Abilities/Action_Abilities/GA_CancelFocus.GA_CancelFocus_C" false)
              (GameplayCue|ExecuteGameplayCueOnActor(Burst) (Ability|GetAvatarActorfromActorInfo) "(TagName=\"GameplayCue.AttackHint\")" (Ability|GameplayCue|MakeGameplayCueParameters :Location (.location (Transformation|GetSocketTransform (Class|GameplayAbility|GetOwningComponentfromActorInfo) "AttackHint" "RTS_Component")))))))))
    (:OnFailed
      (Ability|EndAbility))))
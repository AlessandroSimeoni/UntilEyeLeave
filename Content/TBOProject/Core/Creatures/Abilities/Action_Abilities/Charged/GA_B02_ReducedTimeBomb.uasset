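; Gameplay ability for a B02 creature that puts it into a near-explosion countdown, then detonates it.
; On activation it triggers GA_CloseEyes, swaps in a dynamic material with a set Period parameter, and adds the non-replicated Status.NearExplosion tag.
; It waits for a duration read from a float attribute, activates GA_B02_Explode and ends.
; An AttackHint gameplay cue call is present but never runs.
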(event Ability|EventActivateAbility
  (bind _returnvalue (Ability|GetActorInfo))
  (Abilities|TryActivateAbilitybyClass (Ability|GetAbilitySystemComponentfromActorInfo) "/Game/TBOProject/Core/Creatures/Abilities/Action_Abilities/GA_CloseEyes.GA_CloseEyes_C" true)
  (bind _returnvalue_2 (Rendering|Material|CreateDynamicMaterialInstance (Rendering|Material|GetMaterial (.skeletalmeshcomponent _returnvalue) 0) "None" "None" :!class /Script/Engine.KismetMaterialLibrary))
  (Rendering|Material|SetScalarParameterValue _returnvalue_2 "Period" 6.0 :!class /Script/Engine.MaterialInstanceDynamic)
  (Rendering|Material|SetMaterial (.skeletalmeshcomponent _returnvalue) 0 _returnvalue_2)
  (Ability|GameplayEffect|AddLooseGameplayTags (Ability|GetAvatarActorfromActorInfo) (GameplayTags|MakeLiteralGameplayTagContainer "(GameplayTags=((TagName=\"Status.NearExplosion\")))"))
  (Ability|Tasks|WaitDelay (.ReturnValue (Ability|Attribute|GetFloatAttributefromAbilitySystemComponent (Ability|GetAbilitySystemComponentfromActorInfo) "(AttributeName=\"ReducedTimerExplosionDuration\",Attribute=/Script/TBO_01.B02AttributeSet:ReducedTimerExplosionDuration,AttributeOwner=\"/Script/CoreUObject.Class'/Script/TBO_01.B02AttributeSet'\")"))
    (:OnFinish
      (Abilities|TryActivateAbilitybyClass (Ability|GetAbilitySystemComponentfromActorInfo) "/Game/TBOProject/Core/Creatures/Abilities/Action_Abilities/Charged/GA_B02_Explode.GA_B02_Explode_C" true)
      (Ability|EndAbility))))
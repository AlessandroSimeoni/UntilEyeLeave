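; Gameplay ability for the B02 creature's charged self-destruct explosion.
; On activation it fires an attack-hint cue, applies GE_Death and plays the charge montage.
; After a short delay it stops the AI via blackboard, swaps in a dynamic material, then vibrates and shrinks the mesh.
; It then spawns an attribute-driven BP_AOEDamage blast ahead of itself, clears spotted combat audio if tagged, and kills the creature.
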(event Ability|EventActivateAbility
  (bind _returnvalue (Ability|GetAbilitySystemComponentfromActorInfo))
  (bind _returnvalue_2 (Ability|GetAvatarActorfromActorInfo))
  (bind _returnvalue_3 (Ability|GetActorInfo))
  (bind _returnvalue_4 (Transformation|GetActorTransform _returnvalue_2))
  (GameplayCue|ExecuteGameplayCueOnActor(Burst) (Ability|GetAvatarActorfromActorInfo) "(TagName=\"GameplayCue.AttackHint\")" (Ability|GameplayCue|MakeGameplayCueParameters :Location (.location (Transformation|GetSocketTransform (Class|GameplayAbility|GetOwningComponentfromActorInfo) "AttackHint" "RTS_Component"))))
  (Ability|ApplyGameplayEffectToOwner "/Game/TBOProject/Core/Creatures/Abilities/Effects/GE_Death.GE_Death_C")
  (|PlayMontageandWaitProxy "None" "/Game/TBOProject/Art/Creatures/Mousetrap/AM_B02_Charge.AM_B02_Charge" 1.0 "None" true 1.0 0.0 false
    (:then
      (GameplayTasks|TaskWaitDelay 0 0.2
        (:then
          (AI|Components|Blackboard|SetValueasBool (AI|GetBlackboard (AI|GetAIController (.avataractor _returnvalue_3))) (Utilities|Name|MakeLiteralName "Stop") true)
          (bind _returnvalue_5 (Rendering|Material|CreateDynamicMaterialInstance (Variables|Default|GetMaterial) "None" "None" :!class /Script/Engine.KismetMaterialLibrary))
          (Rendering|Material|SetScalarParameterValue _returnvalue_5 "Period" 1e+01 :!class /Script/Engine.MaterialInstanceDynamic)
          (Rendering|Material|SetMaterial (.skeletalmeshcomponent _returnvalue_3) 0 _returnvalue_5)
          (|VibrateMesh (.skeletalmeshcomponent _returnvalue_3) (.ReturnValue (Ability|Attribute|GetFloatAttributefromAbilitySystemComponent _returnvalue "(AttributeName=\"ExplosionDelay\",Attribute=/Script/TBO_01.B02AttributeSet:ExplosionDelay,AttributeOwner=\"/Script/CoreUObject.Class'/Script/TBO_01.B02AttributeSet'\")")) 5.0
            (:OnFinished
              (|ShrinkMesh (.skeletalmeshcomponent _returnvalue_3) 0.1 0.0
                (:OnFinished
                  (bind _returnvalue_6 (Game|SpawnActorfromClass "/Game/TBOProject/Core/Creatures/Projectiles/AOE/BP_AOEDamage.BP_AOEDamage_C" (Math|Transform|MakeTransform (+ (* (Variables|Default|GetExplosionOffset) (Transformation|GetActorForwardVector _returnvalue_2)) (.location _returnvalue_4)) (.rotation _returnvalue_4) (.scale _returnvalue_4)) "Undefined" "MultiplyWithRoot" 0 0))
                  (Class|AOEDamage|Explode _returnvalue_6 (.ReturnValue (Ability|Attribute|GetFloatAttributefromAbilitySystemComponent _returnvalue "(AttributeName=\"CharacterLevel\",Attribute=/Script/TBO_01.BaseCreatureAttributeSet:CharacterLevel,AttributeOwner=\"/Script/CoreUObject.Class'/Script/TBO_01.BaseCreatureAttributeSet'\")")) (.ReturnValue (Ability|Attribute|GetFloatAttributefromAbilitySystemComponent _returnvalue "(AttributeName=\"Attack\",Attribute=/Script/TBO_01.BaseCreatureAttributeSet:Attack,AttributeOwner=\"/Script/CoreUObject.Class'/Script/TBO_01.BaseCreatureAttributeSet'\")")) (.ReturnValue (Ability|Attribute|GetFloatAttributefromAbilitySystemComponent _returnvalue "(AttributeName=\"ExplosionRadius\",Attribute=/Script/TBO_01.B02AttributeSet:ExplosionRadius,AttributeOwner=\"/Script/CoreUObject.Class'/Script/TBO_01.B02AttributeSet'\")")) (.ReturnValue (Ability|Attribute|GetFloatAttributefromAbilitySystemComponent _returnvalue "(AttributeName=\"KnockBackIntensity\",Attribute=/Script/TBO_01.BaseCreatureAttributeSet:KnockBackIntensity,AttributeOwner=\"/Script/CoreUObject.Class'/Script/TBO_01.BaseCreatureAttributeSet'\")")))
                  (if (GameplayTags|HasMatchingGameplayTag (Ability|GetAbilitySystemComponent (Ability|GetAvatarActorfromActorInfo)) "(TagName=\"Status.Spotted\")")
                    (Class|AudioSubsystem|RemoveSpottedCombatAudio (Subsystems|GetAudioSubsystem)))
                  (Ability|EndAbility)
                  (bind _ascreature (Utilities|Casting|CastToCreature (Ability|GetAvatarActorfromActorInfo)))
                  (Class|Creature|Death _ascreature false))))))))))

(event Ability|EventOnEndAbility
  (params (bWasCancelled :type Boolean)))
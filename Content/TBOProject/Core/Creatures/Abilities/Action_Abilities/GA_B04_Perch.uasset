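; Gameplay ability that lands the B04 creature on its altar to perch.
; It plays the landing montage, sets a "Nest" motion warp target from the altar transform held by the B04 controller, and notifies that controller that the altar is reached.
; When the montage completes, blends out, is interrupted or is cancelled, it switches movement to Walking and ends the ability.
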(event Ability|EventActivateAbility
  (bind _ascreature (Utilities|Casting|CastToCreature (Ability|GetAvatarActorfromActorInfo)))
  (bind _asb04_controller (Utilities|Casting|CastToB04_Controller (Pawn|GetController _ascreature)))
  (|PlayMontageandWaitProxy "None" "/Game/TBOProject/Art/Creatures/Cagebird/AM_B04_Landing.AM_B04_Landing" 1.0 "None" true 1.0 0.0 false
    (:then
      (Class|MotionWarpingComponent|AddorUpdateWarpTargetfromTransform (Actor|GetComponentbyClass (Ability|GetAvatarActorfromActorInfo) "/Script/MotionWarping.MotionWarpingComponent") "Nest" (Variables|/Script/TBO_01.B04_Controller|GetAltarTransform _asb04_controller))
      (Class|B04Controller|ReachedAltar _asb04_controller))
    (:OnCompleted
      (Pawn|Components|CharacterMovement|SetMovementMode (Variables|/Script/Engine.Character|GetCharacterMovement _ascreature) "MOVE_Walking" 0 :!label _label)
      (Ability|EndAbility))
    (:OnBlendOut
      (goto _label))
    (:OnInterrupted
      (goto _label))
    (:OnCancelled
      (goto _label))))
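; GA_Focus is a gameplay ability that makes an AI-controlled Creature focus on the target passed in the activating gameplay event.
; Activation switches the creature's movement mode on and sets AI focus through the avatar's instigator controller, then waits for a cancel to end the ability.
; Ending the ability switches the movement mode back and clears focus on the creature's own controller.
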(event Ability|EventOnEndAbility
  (params (bWasCancelled :type Boolean))
  (bind _ascreature (Utilities|Casting|CastToCreature (Ability|GetAvatarActorfromActorInfo)))
  (Class|Creature|SwitchMovementMode _ascreature false)
  (bind _asaicontroller (Utilities|Casting|CastToAIController (Pawn|GetController _ascreature)))
  (AI|ClearFocus _asaicontroller))

(event Ability|EventActivateAbilityFromEvent
  (params (EventData :type Gameplay%20Event%20Data%20Structure%20%28by%20ref%29))
  (bind _returnvalue (Ability|GetAvatarActorfromActorInfo))
  (Development|PrintText "focus")
  (bind _ascreature (Utilities|Casting|CastToCreature _returnvalue))
  (Class|Creature|SwitchMovementMode _ascreature true)
  (bind _asaicontroller (Utilities|Casting|CastToAIController (Pawn|GetController (Variables|/Script/Engine.Actor|GetInstigator _returnvalue))))
  (AI|SetFocus _asaicontroller (.target EventData))
  (|WaitCancel
    (:OnCancel
      (Ability|EndAbility))))
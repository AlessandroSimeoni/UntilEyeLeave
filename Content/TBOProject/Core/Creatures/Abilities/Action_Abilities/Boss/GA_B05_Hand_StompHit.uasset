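; Gameplay ability for the hit of boss B05's hand stomp, activated by a gameplay event.
; On activation it stores the event target, plays FX and sound at the effect context origin, then ends immediately.
; OnEndAbility sends non-creature targets and the main character a HitMessage built from the owner's attribute values.
; Other creatures are instantly killed through the InstantDeath tagged ability, while boss hands are ignored.
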(event Ability|EventOnEndAbility
  (params (bWasCancelled :type Boolean))
  (bind _returnvalue (Ability|GetAbilitySystemComponentfromActorInfo))
  (Utilities|Casting|CastToMainCharacter (Variables|Default|GetHitTarger)
    (:then
      (Class|HittableActor|Hit(Message) (Variables|Default|GetHitTarger) (Math|Float|Truncate (.ReturnValue (Class|AbilitySystemComponent|GetGameplayAttributeValue _returnvalue "(AttributeName=\"CharacterLevel\",Attribute=/Script/TBO_01.BaseCreatureAttributeSet:CharacterLevel,AttributeOwner=\"/Script/CoreUObject.Class'/Script/TBO_01.BaseCreatureAttributeSet'\")"))) (.ReturnValue (Class|AbilitySystemComponent|GetGameplayAttributeValue _returnvalue "(AttributeName=\"Attack\",Attribute=/Script/TBO_01.BaseCreatureAttributeSet:Attack,AttributeOwner=\"/Script/CoreUObject.Class'/Script/TBO_01.BaseCreatureAttributeSet'\")")) (.instigator (stale Ability|EventActivateAbilityFromEvent EventData)) (.ReturnValue (Class|AbilitySystemComponent|GetGameplayAttributeValue _returnvalue "(AttributeName=\"KnockBackIntensity\",Attribute=/Script/TBO_01.BaseCreatureAttributeSet:KnockBackIntensity,AttributeOwner=\"/Script/CoreUObject.Class'/Script/TBO_01.BaseCreatureAttributeSet'\")")) :!label _label))
    (:CastFailed
      (bind _ascreature (Utilities|Casting|CastToCreature (Variables|Default|GetHitTarger))
        (:then
          (Utilities|Casting|CastToB05_BossHand (Variables|Default|GetHitTarger)
            (:CastFailed
              (Development|PrintText (Utilities|Text|ToText(Object) (Variables|Default|GetHitTarger)))
              (Abilities|TryActivateAbilitiesbyTag (Ability|GetAbilitySystemComponent _ascreature) (GameplayTags|MakeLiteralGameplayTagContainer "(GameplayTags=((TagName=\"FeedBack.Death.InstantDeath\")))") true))))
        (:CastFailed
          (goto _label))))))

(event Ability|EventActivateAbilityFromEvent
  (params (EventData :type Gameplay%20Event%20Data%20Structure%20%28by%20ref%29))
  (bind _returnvalue (Class|AbilitySystemBlueprintLibrary|EffectContextGetOrigin (.contexthandle EventData)))
  (Variables|Default|SetHitTarger (.target EventData))
  (Class|NiagaraFunctionLibrary|SpawnSystematLocationwithParams (Utilities|Struct|MakeFXSystemSpawnParameters self (Variables|Default|GetFX) _returnvalue "0.000000,0.000000,0.000000" "1.000000,1.000000,1.000000" 0 "None" "KeepWorldPosition" true true "None" true false))
  (Audio|PlaySoundatLocation (Variables|Default|GetSFX) _returnvalue "0, 0, 0" 1.0 1.0 0.0 0 0 0 0)
  (Ability|EndAbility))
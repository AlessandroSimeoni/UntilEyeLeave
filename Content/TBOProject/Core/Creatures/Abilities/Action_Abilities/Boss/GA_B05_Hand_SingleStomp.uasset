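; Gameplay ability for boss B05's hand single stomp: the hand flies up, slams down and releases an expanding ring attack.
; FlyUp and Fall tasks drive the movement, while the stomp montage plays and a short additive root-motion force pushes the avatar downward.
; On landing, a forward-offset downward trace places BP_RingAttack, tuned by gameplay attributes for damage, destruction, size, timing and knockback.
; The montage jumps to Endloop, then the ability ends after a brief delay.
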(event Ability|EventActivateAbility
  (bind _returnvalue (Ability|GetAvatarActorfromActorInfo))
  (bind _returnvalue_2 (Ability|GetAbilitySystemComponentfromActorInfo))
  (bind _offset (Variables|Default|GetOffset))
  (bind _returnvalue_3 (Transformation|GetActorForwardVector _returnvalue))
  (bind _returnvalue_4 (Transformation|GetActorLocation _returnvalue))
  (bind _returnvalue_5 (* _returnvalue_3 _offset))
  (bind _returnvalue_6 (+ _returnvalue_5 _returnvalue_4))
  (|FlyUp "None" (.ReturnValue (Class|AbilitySystemComponent|GetGameplayAttributeValue (Ability|GetAbilitySystemComponentfromActorInfo) "(AttributeName=\"StompHeight\",Attribute=/Script/TBO_01.B05HandAttributeSet:StompHeight,AttributeOwner=\"/Script/CoreUObject.Class'/Script/TBO_01.B05HandAttributeSet'\")"))
    (:OnTaskFlyUpFinished
      (|Fall "None"
        (:then
          (|PlayMontageandWaitProxy "None" "/Game/TBOProject/Art/Creatures/Boss/Animation/PawLX/AM_B05_StepOnhand_Stomp.AM_B05_StepOnhand_Stomp" 1.0 "None" true 0.0 0.0 false
            (:then
              (Ability|Tasks|WaitDelay 0.1
                (:OnFinish
                  (Ability|Tasks|ApplyRootMotionConstantForce "None" "0.000000,0.000000,-10000.000000" 1e+04 0.1 true 0 "MaintainLastRootMotionVelocity"))))))
        (:OnFallFinished
          (bind _outhit (Collision|LineTraceByChannel _returnvalue_6 (- _returnvalue_6 "0.000000,0.000000,1000.000000") "TraceTypeQuery1" false (Utilities|Array|MakeArray _returnvalue) "Persistent"))
          (bind _returnvalue_7 (Game|SpawnActorfromClass "/Game/TBOProject/Core/Creatures/Projectiles/AOE/BP_RingAttack.BP_RingAttack_C" (Math|Conversions|ToTransform(Vector) (.impactpoint _outhit)) "Undefined" "MultiplyWithRoot" 0 0))
          (Class|AOERing|StartRingExpand _returnvalue_7 (.ReturnValue (Class|AbilitySystemComponent|GetGameplayAttributeValue _returnvalue_2 "(AttributeName=\"CharacterLevel\",Attribute=/Script/TBO_01.BaseCreatureAttributeSet:CharacterLevel,AttributeOwner=\"/Script/CoreUObject.Class'/Script/TBO_01.BaseCreatureAttributeSet'\")")) (.ReturnValue (Class|AbilitySystemComponent|GetGameplayAttributeValue _returnvalue_2 "(AttributeName=\"RingDamage\",Attribute=/Script/TBO_01.B05HandAttributeSet:RingDamage,AttributeOwner=\"/Script/CoreUObject.Class'/Script/TBO_01.B05HandAttributeSet'\")")) (.ReturnValue (Class|AbilitySystemComponent|GetGameplayAttributeValue _returnvalue_2 "(AttributeName=\"RingMaxExpansion\",Attribute=/Script/TBO_01.B05HandAttributeSet:RingMaxExpansion,AttributeOwner=\"/Script/CoreUObject.Class'/Script/TBO_01.B05HandAttributeSet'\")")) (.ReturnValue (Class|AbilitySystemComponent|GetGameplayAttributeValue _returnvalue_2 "(AttributeName=\"RingExpansionTime\",Attribute=/Script/TBO_01.B05HandAttributeSet:RingExpansionTime,AttributeOwner=\"/Script/CoreUObject.Class'/Script/TBO_01.B05HandAttributeSet'\")")) (.ReturnValue (Class|AbilitySystemComponent|GetGameplayAttributeValue _returnvalue_2 "(AttributeName=\"RingKnockBack\",Attribute=/Script/TBO_01.B05HandAttributeSet:RingKnockBack,AttributeOwner=\"/Script/CoreUObject.Class'/Script/TBO_01.B05HandAttributeSet'\")")))
          (Ability|Animation|MontageJumptoSection (Components|SkeletalMesh|GetAnimInstance (.skeletalmeshcomponent (Ability|GetActorInfo))) "Endloop" "/Game/TBOProject/Art/Creatures/Boss/Animation/PawLX/AM_B05_StepOnhand_Stomp.AM_B05_StepOnhand_Stomp")
          (Ability|Tasks|WaitDelay 0.3
            (:OnFinish
              (Ability|EndAbility))))))))

(event Ability|EventOnEndAbility
  (params (bWasCancelled :type Boolean)))
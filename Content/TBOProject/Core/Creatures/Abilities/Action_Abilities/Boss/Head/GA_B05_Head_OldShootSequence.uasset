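; Gameplay ability for the B05 boss head, named as an old shoot sequence, that fires a three-shot burst from muzzle 5.
; On activation it caches the avatar's muzzle controller and reads projectile speed, damage and both delay intervals from gameplay attributes.
; Chained WaitDelay tasks space the ShootMiddle calls by the burst interval.
; After the last shot, two interval delays start back-to-back without waiting, and the second ends the ability.
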(event Ability|EventActivateAbility
  (bind _returnvalue (Ability|GetAbilitySystemComponentfromActorInfo))
  (bind _returnvalue_2 (Class|Shooter|GetMuzzlesController(Message) (Ability|GetAvatarActorfromActorInfo)))
  (Variables|Default|SetMuzzle%20Controller _returnvalue_2)
  (Variables|Default|SetSpikeSpeed (.ReturnValue (Class|AbilitySystemComponent|GetGameplayAttributeValue _returnvalue "(AttributeName=\"ShootSpeedSpikePhase3\",Attribute=/Script/TBO_01.B05HeadAttributeSet:ShootSpeedSpikePhase3,AttributeOwner=\"/Script/CoreUObject.Class'/Script/TBO_01.B05HeadAttributeSet'\")")))
  (Variables|Default|SetAttack (.ReturnValue (Class|AbilitySystemComponent|GetGameplayAttributeValue _returnvalue "(AttributeName=\"Attack\",Attribute=/Script/TBO_01.BaseCreatureAttributeSet:Attack,AttributeOwner=\"/Script/CoreUObject.Class'/Script/TBO_01.BaseCreatureAttributeSet'\")")))
  (Variables|Default|SetInterval (.ReturnValue (Class|AbilitySystemComponent|GetGameplayAttributeValue _returnvalue "(AttributeName=\"ShootIntervalPhase3\",Attribute=/Script/TBO_01.B05HeadAttributeSet:ShootIntervalPhase3,AttributeOwner=\"/Script/CoreUObject.Class'/Script/TBO_01.B05HeadAttributeSet'\")")))
  (bind _output_get (Variables|Default|SetBurstShootInterval (.ReturnValue (Class|AbilitySystemComponent|GetGameplayAttributeValue _returnvalue "(AttributeName=\"BurstShootInterval\",Attribute=/Script/TBO_01.B05HeadAttributeSet:BurstShootInterval,AttributeOwner=\"/Script/CoreUObject.Class'/Script/TBO_01.B05HeadAttributeSet'\")"))))
  (Utilities|ShootMiddle)
  (Ability|Tasks|WaitDelay _output_get
    (:OnFinish
      (Utilities|ShootMiddle)
      (Ability|Tasks|WaitDelay _output_get
        (:OnFinish
          (Utilities|ShootMiddle)
          (Ability|Tasks|WaitDelay (Variables|Default|GetInterval)
            (:then
              (Ability|Tasks|WaitDelay (Variables|Default|GetInterval)
                (:OnFinish
                  (Ability|EndAbility))))))))))

(event Ability|EventOnEndAbility
  (params (bWasCancelled :type Boolean)))
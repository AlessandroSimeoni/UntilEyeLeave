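; Gameplay ability for the B05 boss head that fires its left eye as a projectile.
; After the eye-shoot montage completes, it fires BP_EyeProjectile through the avatar's muzzle controller, using attribute-driven speed, damage and knockback.
; On success it hides the eye mesh, plays a gameplay cue, passes the projectile to the head's AI controller and adds a missing-eye tag.
; It ends after an attribute-driven delay, or immediately on failure or montage interruption.
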(event Ability|EventActivateAbility
  (bind _returnvalue (Ability|GetAvatarActorfromActorInfo))
  (bind _returnvalue_2 (Ability|GetAbilitySystemComponentfromActorInfo))
  (|PlayMontageandWaitProxy "None" "/Game/TBOProject/Art/Creatures/Boss/Animation/Head/AM_B05_Head_AS_DogHead_EyeShoot_2_Montage.AM_B05_Head_AS_DogHead_EyeShoot_2_Montage" 1.0 "None" true 1.0 0.0 false
    (:OnCompleted
      (bind _returnvalue_3 (Class|Shooter|GetMuzzlesController(Message) _returnvalue))
      (bind _returnvalue_4 (Class|MuzzlesController|ShootwithMuzzle _returnvalue_3 2 "/Game/TBOProject/Core/Creatures/Projectiles/BP_EyeProjectile.BP_EyeProjectile_C" (.ReturnValue (Class|AbilitySystemComponent|GetGameplayAttributeValue _returnvalue_2 "(AttributeName=\"ShootSpeedEyePhase3\",Attribute=/Script/TBO_01.B05HeadAttributeSet:ShootSpeedEyePhase3,AttributeOwner=\"/Script/CoreUObject.Class'/Script/TBO_01.B05HeadAttributeSet'\")")) 0 (.ReturnValue (Class|AbilitySystemComponent|GetGameplayAttributeValue _returnvalue_2 "(AttributeName=\"Attack\",Attribute=/Script/TBO_01.BaseCreatureAttributeSet:Attack,AttributeOwner=\"/Script/CoreUObject.Class'/Script/TBO_01.BaseCreatureAttributeSet'\")")) 0.0 (.ReturnValue (Class|AbilitySystemComponent|GetGameplayAttributeValue _returnvalue_2 "(AttributeName=\"EyeKnockback\",Attribute=/Script/TBO_01.B05HeadAttributeSet:EyeKnockback,AttributeOwner=\"/Script/CoreUObject.Class'/Script/TBO_01.B05HeadAttributeSet'\")"))))
      (bind _asb05_boss_head_controller (Utilities|Casting|CastToB05_BossHead_Controller (AI|GetAIController _returnvalue))
        (:then
          (bind _output_get (Variables|Default|SetAs%20B05%20Boss%20Head%20Controller _asb05_boss_head_controller))
          (bind _asbp_eye_projectile (Utilities|Casting|CastToBP_EyeProjectile _returnvalue_4)
            (:then
              (Rendering|SetVisibility (Variables|/Script/TBO_01.B05_BossHead|GetLeftEye (Variables|/Script/TBO_01.B05_BossHead_Controller|GetBossHead (Variables|Default|GetAs%20B05%20Boss%20Head%20Controller))) false false)
              (GameplayCue|ExecuteGameplayCueOnActor(Burst) (Ability|GetAvatarActorfromActorInfo) "(TagName=\"GameplayCue.B05.ShootEye\")" (Ability|GameplayCue|MakeGameplayCueParameters :Location (Transformation|GetWorldLocation (Variables|/Script/TBO_01.B05_BossHead|GetLeftEye (Variables|/Script/TBO_01.B05_BossHead_Controller|GetBossHead (Variables|Default|GetAs%20B05%20Boss%20Head%20Controller)))) :Normal (Math|Vector|GetForwardVector (Variables|/Script/TBO_01.B05_BossHead|GetLeftEye (Variables|/Script/TBO_01.B05_BossHead_Controller|GetBossHead (Variables|Default|GetAs%20B05%20Boss%20Head%20Controller))))))
              (Class|B05BossHeadController|CheckEyeProjectile _output_get _asbp_eye_projectile)
              (Ability|GameplayEffect|AddLooseGameplayTags (Ability|GetAvatarActorfromActorInfo) (GameplayTags|MakeLiteralGameplayTagContainer "(GameplayTags=((TagName=\"Status.Boss.MissingEyeLX\")))"))
              (Ability|Tasks|WaitDelay (.ReturnValue (Class|AbilitySystemComponent|GetGameplayAttributeValue _returnvalue_2 "(AttributeName=\"SequenceIntervalPhase3\",Attribute=/Script/TBO_01.B05HeadAttributeSet:SequenceIntervalPhase3,AttributeOwner=\"/Script/CoreUObject.Class'/Script/TBO_01.B05HeadAttributeSet'\")"))
                (:OnFinish
                  _)))
            (:CastFailed
              _)))
        (:CastFailed
          _))
      (Ability|EndAbility))
    (:OnInterrupted
      (Ability|EndAbility :!label _label))
    (:OnCancelled
      (goto _label))))

(event Ability|EventOnEndAbility
  (params (bWasCancelled :type Boolean)))
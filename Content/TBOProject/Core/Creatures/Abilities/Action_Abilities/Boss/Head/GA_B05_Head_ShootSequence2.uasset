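; Gameplay ability for the B05 boss head's second shooting attack, firing a data-defined series of projectile volleys.
; It plays a pre-shoot montage, then gets the muzzle controller from the avatar.
; A self-calling Sequence event fires each ShootSequence entry's muzzles using ability system attributes for speed, damage and knockback, then waits that entry's delay.
; After the last entry, an after-shoot montage plays and the ability ends.
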(event Custom|Sequence
  (bind _returnvalue (Ability|GetAbilitySystemComponentfromActorInfo))
  (bind _shootsequence (Variables|Default|GetShootSequence))
  (bind _currentsequence (Variables|Default|GetCurrentSequence))
  (bind _shootsequencedata (Variables|/Script/TBO_01.ShootSequence|GetShootSequenceData _shootsequence))
  (bind _output (Utilities|Array|Get(acopy) _shootsequencedata _currentsequence))
  (Class|MuzzlesController|ShootwithMuzzles (Variables|Default|GetMuzzle) (.muzzleids _output) 0 (.ReturnValue (Class|AbilitySystemComponent|GetGameplayAttributeValue _returnvalue "(AttributeName=\"ShootSpeedSpikePhase1\",Attribute=/Script/TBO_01.B05HeadAttributeSet:ShootSpeedSpikePhase1,AttributeOwner=\"/Script/CoreUObject.Class'/Script/TBO_01.B05HeadAttributeSet'\")")) 0 (.ReturnValue (Class|AbilitySystemComponent|GetGameplayAttributeValue _returnvalue "(AttributeName=\"Attack\",Attribute=/Script/TBO_01.BaseCreatureAttributeSet:Attack,AttributeOwner=\"/Script/CoreUObject.Class'/Script/TBO_01.BaseCreatureAttributeSet'\")")) 0.0 (.randomangle _output) (.ReturnValue (Class|AbilitySystemComponent|GetGameplayAttributeValue _returnvalue "(AttributeName=\"KnockBackIntensity\",Attribute=/Script/TBO_01.BaseCreatureAttributeSet:KnockBackIntensity,AttributeOwner=\"/Script/CoreUObject.Class'/Script/TBO_01.BaseCreatureAttributeSet'\")")))
  (Ability|Tasks|WaitDelay (.delay _output)
    (:then
      (Math|Integer|IncrementInt (Variables|Default|GetCurrentSequence)))
    (:OnFinish
      (if (>= (Variables|Default|GetCurrentSequence) (Utilities|Array|Length _shootsequencedata))
        (|PlayMontageandWaitProxy "None" "/Game/TBOProject/Art/Creatures/Boss/Animation/Head/AM_B05_Head_DogHeadRig_AfterShoot_2_Montage.AM_B05_Head_DogHeadRig_AfterShoot_2_Montage" 1.0 "None" true 1.0 0.0 false
          (:OnCompleted
            _)
          (:OnInterrupted
            _)
          (:OnCancelled
            _))
        (Ability|EndAbility)
        (else
          (CallFunction|Sequence))))))

(event Ability|EventActivateAbility
  (|PlayMontageandWaitProxy "None" "/Game/TBOProject/Art/Creatures/Boss/Animation/Head/AM_B05_Head_DogHeadRig_PreShoot_2_Montage.AM_B05_Head_DogHeadRig_PreShoot_2_Montage" 1.0 "None" true 1.0 0.0 false
    (:OnCompleted
      (bind _returnvalue (Class|Shooter|GetMuzzlesController(Message) (Ability|GetAvatarActorfromActorInfo)))
      (Variables|Default|SetMuzzle _returnvalue)
      (CallFunction|Sequence))
    (:OnInterrupted
      (Ability|EndAbility :!label _label))
    (:OnCancelled
      (goto _label))))

(event Ability|EventOnEndAbility
  (params (bWasCancelled :type Boolean)))
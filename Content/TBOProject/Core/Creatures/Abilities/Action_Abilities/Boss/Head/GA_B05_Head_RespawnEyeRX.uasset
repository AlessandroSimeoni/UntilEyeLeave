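; Gameplay ability that respawns the right eye of the B05 boss head.
; On activation it makes the RightEye component visible and fires the B05 RespawnEye gameplay cue at that component's world location.
; It then removes the loose MissingEyeRX status tag from the avatar, without replication, and ends immediately.
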(event Ability|EventActivateAbility
  (bind _asb05_boss_head (Utilities|Casting|CastToB05_BossHead (Ability|GetAvatarActorfromActorInfo)))
  (Rendering|SetVisibility (Variables|/Script/TBO_01.B05_BossHead|GetRightEye _asb05_boss_head) true false)
  (GameplayCue|ExecuteGameplayCueOnActor(Burst) (Ability|GetAvatarActorfromActorInfo) "(TagName=\"GameplayCue.B05.RespawnEye\")" (Ability|GameplayCue|MakeGameplayCueParameters :Location (Transformation|GetWorldLocation (Variables|/Script/TBO_01.B05_BossHead|GetRightEye _asb05_boss_head))))
  (Ability|GameplayEffect|RemoveLooseGameplayTags (Ability|GetAvatarActorfromActorInfo) (GameplayTags|MakeLiteralGameplayTagContainer "(GameplayTags=((TagName=\"Status.Boss.MissingEyeRX\")))"))
  (Ability|EndAbility))

(event Ability|EventOnEndAbility
  (params (bWasCancelled :type Boolean)))
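; Gameplay ability that runs the intro of the B05 boss head and hands over to its first behavior change.
; It starts the dog head activation montage and immediately spawns a destructible hand and a step-on hand, each with a spawn gameplay cue.
; After a short delay it sets the hands to rest, waits for an attribute-driven duration, then advances the controller to the next phase and ends.
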(event Ability|EventActivateAbility
  (bind _asb05_boss_head (Utilities|Casting|CastToB05_BossHead (Ability|GetAvatarActorfromActorInfo)))
  (bind _output_get (Variables|Default|Set%20B05%20Boss%20Head _asb05_boss_head))
  (|PlayMontageandWaitProxy "None" "/Game/TBOProject/Art/Creatures/Boss/Animation/Head/AM_B05_DogHeadRig_Activation_Montage.AM_B05_DogHeadRig_Activation_Montage" 1.0 "None" true 1.0 0.0 false
    (:then
      (bind _returnvalue (Class|B05BossHead|SpawnDestructibleHand _output_get))
      (GameplayCue|ExecuteGameplayCueOnActor(Burst) _returnvalue "(TagName=\"GameplayCue.B05.Spawn\")" (Ability|GameplayCue|MakeGameplayCueParameters :Location (Transformation|GetActorLocation _returnvalue)))
      (bind _returnvalue_2 (Class|B05BossHead|SpawnSteponHand _output_get))
      (GameplayCue|ExecuteGameplayCueOnActor(Burst) _returnvalue_2 "(TagName=\"GameplayCue.B05.Spawn\")" (Ability|GameplayCue|MakeGameplayCueParameters :Location (Transformation|GetActorLocation _returnvalue_2)))
      (Ability|Tasks|WaitDelay 3.0
        (:OnFinish
          (Class|B05BossHead|SetHandstoRest (Variables|Default|Get%20B05%20Boss%20Head))
          (Ability|Tasks|WaitDelay (.ReturnValue (Class|AbilitySystemComponent|GetGameplayAttributeValue (Ability|GetAbilitySystemComponentfromActorInfo) "(AttributeName=\"IntroEndWaitTime\",Attribute=/Script/TBO_01.B05HeadAttributeSet:IntroEndWaitTime,AttributeOwner=\"/Script/CoreUObject.Class'/Script/TBO_01.B05HeadAttributeSet'\")"))
            (:OnFinish
              (bind _asb05_boss_head_controller (Utilities|Casting|CastToB05_BossHead_Controller (Pawn|GetController (Variables|Default|Get%20B05%20Boss%20Head))))
              (Class|B05BossHeadController|NextPhase _asb05_boss_head_controller)
              (Ability|EndAbility))))))))

(event Ability|EventOnEndAbility
  (params (bWasCancelled :type Boolean)))
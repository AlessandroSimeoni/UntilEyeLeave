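; Gameplay ability for the B05 boss head that spawns a B02 minion near the player.
; It plays a dog-head spawn montage, then on completion runs an EQS query picking from the best 5% of locations.
; The boss head spawns the minion at a result point, the head's AI controller records it as current, and a spawn gameplay cue fires on it.
; Interruption or a failed query ends the ability.
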(event Custom|QueryFinished
  (params (QueryInstance :type Env%20Query%20Instance%20Blueprint%20Wrapper%20Object%20Reference) (QueryStatus :type EEnvQueryStatus%20Enum :default "Processing"))
  (bind _as_b05_boss_head_controller (Variables|Default|GetAs%20B05%20Boss%20Head%20Controller))
  (bind (_resultlocations _returnvalue) (AI|EQS|GetQueryResultsasLocations QueryInstance))
  (if _returnvalue
    (bind _output_get (Variables|Default|SetLocation (.OutItem (Utilities|Array|Random _resultlocations))))
    (bind _returnvalue_2 (Class|B05BossHead|SpawnMinion (Variables|/Script/TBO_01.B05_BossHead_Controller|GetBossHead _as_b05_boss_head_controller) (Math|Transform|MakeTransform _output_get "0, 0, 0" "1.000000,1.000000,1.000000") (Variables|Default|GetCreature) (Variables|Default|GetController)))
    (Class|B05BossHeadController|SetCurrentMinion _as_b05_boss_head_controller _returnvalue_2)
    (GameplayCue|ExecuteGameplayCueOnActor(Burst) _returnvalue_2 "(TagName=\"GameplayCue.B05.Spawn\")" (Ability|GameplayCue|MakeGameplayCueParameters :Location (Variables|Default|GetLocation)))
    (Ability|EndAbility)
    (else
      (Ability|EndAbility))))

(event Ability|EventActivateAbility
  (bind _returnvalue (Ability|GetAvatarActorfromActorInfo))
  (|PlayMontageandWaitProxy "None" "/Game/TBOProject/Art/Creatures/Boss/Animation/Head/AM_B05_Head_DogHead_Spawn_1_Montage.AM_B05_Head_DogHead_Spawn_1_Montage" 1.0 "None" true 1.0 0.0 false
    (:OnCompleted
      (bind _returnvalue_2 (AI|EQS|RunEQSQuery "/Game/TBOProject/Core/Creatures/EQS/B05/EQS_SpawnNearPlayer.EQS_SpawnNearPlayer" _returnvalue "RandomBest5Pct"))
      (bind _asb05_boss_head_controller (Utilities|Casting|CastToB05_BossHead_Controller (AI|GetAIController _returnvalue))
        (:then
          (Variables|Default|SetAs%20B05%20Boss%20Head%20Controller _asb05_boss_head_controller)
          (EventDispatchers|BindEventtoOnQueryFinishedEvent _returnvalue_2 (delegate Custom|QueryFinished)))
        (:CastFailed
          (Ability|EndAbility))))
    (:OnInterrupted
      (Ability|EndAbility :!label _label))
    (:OnCancelled
      (goto _label))))

(event Ability|EventOnEndAbility
  (params (bWasCancelled :type Boolean)))
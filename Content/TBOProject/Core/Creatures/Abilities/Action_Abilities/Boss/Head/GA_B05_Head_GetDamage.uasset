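; Gameplay ability for the B05 boss head's damage reaction, which also advances the boss fight to its next phase.
; It tags the head as Status.Stunned and plays an eye-hit or hand-destruction montage chosen by the head AI controller's current phase.
; When the montage completes or is cancelled, it removes the tag, calls NextPhase on the controller and ends.
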(event Ability|EventActivateAbility
  (bind _returnvalue (Ability|GetAvatarActorfromActorInfo))
  (bind _returnvalue_2 (GameplayTags|MakeLiteralGameplayTagContainer "(GameplayTags=((TagName=\"Status.Stunned\")))"))
  (bind _asbp_b05_boss_head_controller (Utilities|Casting|CastToBP_B05_BossHead_Controller (AI|GetAIController (Ability|GetAvatarActorfromActorInfo)))
    (:then
      (Ability|GameplayEffect|AddLooseGameplayTags _returnvalue _returnvalue_2)
      (switch Utilities|FlowControl|Switch|SwitchonEBossPhase (Variables|/Script/TBO_01.B05_BossHead_Controller|GetCurrentPhase _asbp_b05_boss_head_controller)
        (:Phase1
          (Variables|Default|SetMontage%20to%20Play "/Game/TBOProject/Art/Creatures/Boss/Animation/Head/AM_B05_Head_DogHead_EyeBulletHit_1_Montage.AM_B05_Head_DogHead_EyeBulletHit_1_Montage"))
        (:Phase2
          (Variables|Default|SetMontage%20to%20Play "/Game/TBOProject/Art/Creatures/Boss/Animation/Head/AM_B05_Head_DogHeadRig_HandDestruction_Montage.AM_B05_Head_DogHeadRig_HandDestruction_Montage"))
        (:Phase3
          (Variables|Default|SetMontage%20to%20Play "/Game/TBOProject/Art/Creatures/Boss/Animation/Head/AM_B05_Head_DogHead_EyeBulletHit_2_Montage.AM_B05_Head_DogHead_EyeBulletHit_2_Montage")))
      (|PlayMontageandWaitProxy "None" (Variables|Default|GetMontage%20to%20Play) 1.0 "None" true 1.0 0.0 false
        (:OnCompleted
          _)
        (:OnCancelled
          _))
      (Ability|GameplayEffect|RemoveLooseGameplayTags _returnvalue _returnvalue_2)
      (Development|PrintString "NextPhase")
      (Class|B05BossHeadController|NextPhase _asbp_b05_boss_head_controller))
    (:CastFailed
      _))
  (Ability|EndAbility))

(event Ability|EventOnEndAbility
  (params (bWasCancelled :type Boolean)))
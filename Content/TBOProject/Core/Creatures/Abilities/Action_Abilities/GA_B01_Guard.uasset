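; Guard ability for creature B01 that holds a shielded stance until cancelled.
; Activation applies GE_Shielded, enables the creature's effect navigation, triggers GA_CancelFocus and plays the guard montage from its current position.
; On cancel it reverses the montage from that point, removing the shield and navigation effect immediately.
; When the reverse montage completes, it ends and tries to activate GA_B01_spotted.
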(event Ability|EventActivateAbility
  (bind _returnvalue (Ability|GetActorInfo))
  (bind _returnvalue_2 (Components|SkeletalMesh|GetAnimInstance (.skeletalmeshcomponent _returnvalue)))
  (bind _returnvalue_3 (Animation|Montage|MontageGetPosition _returnvalue_2 "/Game/TBOProject/Art/Creatures/Gianguscio/AM_Guard.AM_Guard"))
  (bind _returnvalue_4 (Ability|ApplyGameplayEffectToOwner "/Game/TBOProject/Core/Creatures/Abilities/Effects/GE_Shielded.GE_Shielded_C"))
  (bind _ascreature (Utilities|Casting|CastToCreature (.avataractor _returnvalue)))
  (Class|Creature|SetEffectNavigation _ascreature true)
  (Abilities|TryActivateAbilitybyClass (Ability|GetAbilitySystemComponentfromActorInfo) "/Game/TBOProject/Core/Creatures/Abilities/Action_Abilities/GA_CancelFocus.GA_CancelFocus_C" true)
  (Animation|Montage|PlayMontage (.skeletalmeshcomponent _returnvalue) "/Game/TBOProject/Art/Creatures/Gianguscio/AM_Guard.AM_Guard" 1.0 _returnvalue_3 "Default"
    (:then
      (|WaitCancel
        (:OnCancel
          (Animation|Montage|PlayMontage (.skeletalmeshcomponent _returnvalue) "/Game/TBOProject/Art/Creatures/Gianguscio/AM_Guard.AM_Guard" -1.0 _returnvalue_3 ""
            (:then
              (Ability|RemoveGameplayEffectFromOwnerWithHandle _returnvalue_4)
              (bind _ascreature_2 (Utilities|Casting|CastToCreature _ascreature))
              (Class|Creature|SetEffectNavigation _ascreature_2 false))
            (:OnCompleted
              (Ability|EndAbility)
              (Abilities|TryActivateAbilitybyClass (Ability|GetAbilitySystemComponent (Ability|GetAvatarActorfromActorInfo)) "/Game/TBOProject/Core/Creatures/Abilities/FeedBack_Abilities/View/GA_B01_spotted.GA_B01_spotted_C" true))))))))
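; Gameplay ability that teleports a flying creature to a new spot, by its name one near the player.
; On activation it runs the EQS_FlyingFollow query from the avatar in random-best-25% mode and waits for it to finish.
; It then teleports the Creature in Flying mode to a random result location, fires the Teleport gameplay cue and ends.
; A failed query or cast just ends the ability.
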(event Custom|QueryFinished
  (params (QueryInstance :type Env%20Query%20Instance%20Blueprint%20Wrapper%20Object%20Reference) (QueryStatus :type EEnvQueryStatus%20Enum :default "Processing"))
  (bind _returnvalue (Ability|GetAvatarActorfromActorInfo))
  (bind (_resultlocations _returnvalue_2) (AI|EQS|GetQueryResultsasLocations QueryInstance))
  (if _returnvalue_2
    (bind _ascreature (Utilities|Casting|CastToCreature _returnvalue)
      (:then
        (Class|Creature|Teleport _ascreature (.OutItem (Utilities|Array|Random _resultlocations)) "MOVE_Flying")
        (GameplayCue|ExecuteGameplayCueOnActor(Burst) _returnvalue "(TagName=\"GameplayCue.Teleport\")" (Ability|GameplayCue|MakeGameplayCueParameters 0.0))
        (Ability|EndAbility))
      (:CastFailed
        (Ability|EndAbility)))
    (else
      (Ability|EndAbility))))

(event Ability|EventActivateAbility
  (bind _returnvalue (AI|EQS|RunEQSQuery "/Game/TBOProject/Core/Creatures/EQS/B04/EQS_FlyingFollow.EQS_FlyingFollow" (Ability|GetAvatarActorfromActorInfo) "RandomBest25Pct"))
  (EventDispatchers|BindEventtoOnQueryFinishedEvent _returnvalue (delegate Custom|QueryFinished)))

(event Ability|EventOnEndAbility
  (params (bWasCancelled :type Boolean)))
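; Event-triggered gameplay ability for creature B06, named for coin stealing, that performs a forward lunge attack toward the event's target.
; It turns the avatar to face the target, plays the no-coin attack montage and fires an attack-hint gameplay cue.
; After a zero-length delay it applies a constant forward root motion force and an attack-delay effect on itself, ending when either force or montage finishes.
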(event Ability|EventOnEndAbility
  (params (bWasCancelled :type Boolean)))

(event Ability|EventActivateAbilityFromEvent
  (params (EventData :type Gameplay%20Event%20Data%20Structure%20%28by%20ref%29))
  (bind _returnvalue (Ability|GetAvatarActorfromActorInfo))
  (|RotateCharacter "None" (- (.yaw (Math|Rotator|FindLookatRotation (Transformation|GetActorLocation _returnvalue) (Transformation|GetActorLocation (.target EventData)))) (.yaw (Transformation|GetActorRotation _returnvalue))) 0.2 0
    (:OnRotationCompleted
      (|PlayMontageandWaitProxy "None" "/Game/TBOProject/Art/Creatures/Stealer/B06_Artist/NewAnimation/AS_B06_AttackNoCoin_Montage.AS_B06_AttackNoCoin_Montage" 1.0 "None" true 1.0 0.0 false
        (:then
          (Ability|Tasks|WaitDelay 0.0
            (:then
              (GameplayCue|ExecuteGameplayCueOnActor(Burst) (Ability|GetAvatarActorfromActorInfo) "(TagName=\"GameplayCue.AttackHint\")" (Ability|GameplayCue|MakeGameplayCueParameters :Location (.location (Transformation|GetSocketTransform (Class|GameplayAbility|GetOwningComponentfromActorInfo) "AttackHint" "RTS_Component")))))
            (:OnFinish
              (Ability|Tasks|ApplyRootMotionConstantForce "None" (Transformation|GetActorForwardVector (Ability|GetAvatarActorfromActorInfo)) 5e+02 1.5 false "/Game/TBOProject/Core/Eyes/FC_Fixed.FC_Fixed" "MaintainLastRootMotionVelocity" "0, 0, 0" 0.0 true
                (:then
                  (Ability|ApplyGameplayEffectToOwner "/Game/TBOProject/Core/Creatures/Abilities/Effects/GE_b06_AttackDelay.GE_b06_AttackDelay_C"))
                (:OnFinish
                  (Ability|EndAbility :!label _label))))))
        (:OnCompleted
          (goto _label))
        (:OnBlendOut
          (goto _label))
        (:OnCancelled
          (goto _label))))))

(event Ability|EventActivateAbility)
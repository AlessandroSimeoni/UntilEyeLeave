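; Event-triggered hit ability for B06 that delivers damage and can take a coin from the main character it hits.
; Activation plays FX and sound at the effect context origin, then ends immediately.
; OnEndAbility sends attribute-driven hits to DestructibleParts or through the target's HitMessage.
; For a valid MainCharacter with a positive attribute, it activates GA_B06_PickUpCoin unless tagged Currency.PickUpCoin, and applies GE_CoinDown to that character.
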(event Ability|EventOnEndAbility
  (params (bWasCancelled :type Boolean))
  (bind _returnvalue (Ability|GetAbilitySystemComponentfromActorInfo))
  (bind _returnvalue_2 (Class|AbilitySystemComponent|GetGameplayAttributeValue _returnvalue "(AttributeName=\"KnockBackIntensity\",Attribute=/Script/TBO_01.BaseCreatureAttributeSet:KnockBackIntensity,AttributeOwner=\"/Script/CoreUObject.Class'/Script/TBO_01.BaseCreatureAttributeSet'\")"))
  (bind _returnvalue_3 (Class|AbilitySystemComponent|GetGameplayAttributeValue _returnvalue "(AttributeName=\"CharacterLevel\",Attribute=/Script/TBO_01.BaseCreatureAttributeSet:CharacterLevel,AttributeOwner=\"/Script/CoreUObject.Class'/Script/TBO_01.BaseCreatureAttributeSet'\")"))
  (Development|PrintText "Hello" true true "(R=0.012786,G=1.000000,B=0.000000,A=1.000000)")
  (bind _asmain_character (Utilities|Casting|CastToMainCharacter (Variables|Default|GetEvent%20Data%20Target))
    (:then
      (Variables|Default|SetAs%20Main%20Character _asmain_character)
      (bind _returnvalue_4 (Class|HittableActor|Hit(Message) (Variables|Default|GetEvent%20Data%20Target) (Math|Float|Truncate _returnvalue_3) (.ReturnValue (Class|AbilitySystemComponent|GetGameplayAttributeValue _returnvalue "(AttributeName=\"Attack\",Attribute=/Script/TBO_01.BaseCreatureAttributeSet:Attack,AttributeOwner=\"/Script/CoreUObject.Class'/Script/TBO_01.BaseCreatureAttributeSet'\")")) (Variables|Default|GetEvent%20Data%20Instigator) _returnvalue_2 :!label _label))
      (if _returnvalue_4
        (Utilities|IsValid (Variables|Default|GetAs%20Main%20Character) :!label _label_2
          (:Is%20Valid
            (if (> (.ReturnValue (Class|AbilitySystemComponent|GetGameplayAttributeValue (Variables|/Script/TBO_01.MainCharacter|GetAbilitySystemComponent (Variables|Default|GetAs%20Main%20Character)) "(AttributeName=\"Coin\",Attribute=/Script/TBO_01.PlayerAttributeSet:Coin,AttributeOwner=\"/Script/CoreUObject.Class'/Script/TBO_01.PlayerAttributeSet'\")")) 0.0)
              (if (not (GameplayTags|HasAnyMatchingGameplayTags (Ability|GetAbilitySystemComponentfromActorInfo) (GameplayTags|MakeLiteralGameplayTagContainer "(GameplayTags=((TagName=\"Currency.PickUpCoin\")))")))
                (Abilities|TryActivateAbilitybyClass (Ability|GetAbilitySystemComponentfromActorInfo) "/Game/TBOProject/Core/Creatures/Abilities/Effects_Application/GA_B06_PickUpCoin.GA_B06_PickUpCoin_C" true)
                (GameplayEffects|ApplyGameplayEffectToSelf :self (Variables|/Script/TBO_01.MainCharacter|GetAbilitySystemComponent (Variables|Default|GetAs%20Main%20Character)) :GameplayEffectClass "/Game/TBOProject/Core/Characters/Player/Abilities/Effects/GE_CoinDown.GE_CoinDown_C")))))))
    (:CastFailed
      (bind _asdestructible_parts (Utilities|Casting|CastToDestructibleParts (Variables|Default|GetEvent%20Data%20Optional%20Object))
        (:then
          (Class|HittableActor|Hit _asdestructible_parts (Math|Float|Truncate _returnvalue_3) 0.0 (Variables|Default|GetEvent%20Data%20Instigator) _returnvalue_2)
          (goto _label_2))
        (:CastFailed
          (Variables|Default|SetIsPiercing (Actor|ActorHasTag (Variables|Default|GetEvent%20Data%20Target) "Pierce"))
          (goto _label))))))

(event Ability|EventActivateAbilityFromEvent
  (params (EventData :type Gameplay%20Event%20Data%20Structure%20%28by%20ref%29))
  (bind _returnvalue (Class|AbilitySystemBlueprintLibrary|EffectContextGetOrigin (.contexthandle EventData)))
  (Development|PrintText "Hit B06")
  (Variables|Default|SetEvent%20Data%20Instigator (.instigator EventData))
  (Variables|Default|SetEvent%20Data%20Target (.target EventData))
  (Variables|Default|SetEvent%20Data%20Optional%20Object (.optionalobject EventData))
  (Class|NiagaraFunctionLibrary|SpawnSystematLocationwithParams (Utilities|Struct|MakeFXSystemSpawnParameters self (Variables|Default|GetFX) _returnvalue "0.000000,0.000000,0.000000" "1.000000,1.000000,1.000000" 0 "None" "KeepWorldPosition" true true "None" true false))
  (Audio|PlaySoundatLocation (Variables|Default|GetSFX) _returnvalue "0, 0, 0" 1.0 1.0 0.0 0 0 0 0)
  (Ability|EndAbility))
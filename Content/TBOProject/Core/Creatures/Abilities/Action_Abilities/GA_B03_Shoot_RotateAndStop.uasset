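; Gameplay ability for the B03 Birdman creature's charged projectile attack, which focuses on the event's target, then cancels focus before firing.
; It closes the eyes, applies a charge effect and plays the attack montage, with attribute-driven delays pacing focus cancel, an attack-hint cue and montage section jumps.
; A commit event fires the muzzle shot using attribute-based stats and reopens the eyes.
; A recovery montage follows; ending removes the charge and applies a shooting delay.
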(event Ability|EventOnEndAbility
  (params (bWasCancelled :type Boolean))
  (Ability|ApplyGameplayEffectToOwner "/Game/TBOProject/Core/Creatures/Abilities/Effects/GE_ShootingDelay.GE_ShootingDelay_C")
  (Ability|RemoveGameplayEffectFromOwnerWithHandle (Variables|Default|GetEffectHandle)))

(event Ability|EventActivateAbilityFromEvent
  (params (EventData :type Gameplay%20Event%20Data%20Structure%20%28by%20ref%29))
  (bind _returnvalue (Ability|GetAbilitySystemComponentfromActorInfo))
  (bind _returnvalue_2 (Ability|GetAbilitySystemComponentfromActorInfo))
  (bind _returnvalue_3 (Ability|GetAbilitySystemComponentfromActorInfo))
  (bind _output_get (Variables|Default|SetTarget (.target EventData)))
  (Abilities|TryActivateAbilitybyClass _returnvalue "/Game/TBOProject/Core/Creatures/Abilities/Action_Abilities/GA_CloseEyes.GA_CloseEyes_C" true)
  (bind _returnvalue_4 (GameplayEffects|ApplyGameplayEffectToSelf :self _returnvalue :GameplayEffectClass "/Game/TBOProject/Core/Creatures/Abilities/Effects/Charge/GE_B03_Charge.GE_B03_Charge_C"))
  (Variables|Default|SetEffectHandle _returnvalue_4)
  (Ability|SendGameplayEvent "(TagName=\"Action.Focus\")" (Utilities|Struct|MakeGameplayEventData "(TagName=\"\")" 0 _output_get 0 0 "()" "(GameplayTags=)" "(GameplayTags=)" 0.0 "()"))
  (|PlayMontageandWaitProxy "None" "/Game/TBOProject/Art/Creatures/Birdman/AM_B03_Attack_Birdman_Montage.AM_B03_Attack_Birdman_Montage" 1.0 "None" true 1.0 0.0 false
    (:then
      (Ability|Tasks|WaitDelay (.ReturnValue (Class|AbilitySystemComponent|GetGameplayAttributeValue _returnvalue_2 "(AttributeName=\"ShootChargeTime\",Attribute=/Script/TBO_01.ShooterCreatureAttributeSet:ShootChargeTime,AttributeOwner=\"/Script/CoreUObject.Class'/Script/TBO_01.ShooterCreatureAttributeSet'\")"))
        (:OnFinish
          (Abilities|TryActivateAbilitybyClass _returnvalue_2 "/Game/TBOProject/Core/Creatures/Abilities/Action_Abilities/GA_CancelFocus.GA_CancelFocus_C" true)
          (Ability|Tasks|WaitDelay (.ReturnValue (Class|AbilitySystemComponent|GetGameplayAttributeValue _returnvalue_2 "(AttributeName=\"NonFocusDelayAfterCharge\",Attribute=/Script/TBO_01.ShooterCreatureAttributeSet:NonFocusDelayAfterCharge,AttributeOwner=\"/Script/CoreUObject.Class'/Script/TBO_01.ShooterCreatureAttributeSet'\")"))
            (:then
              (GameplayCue|ExecuteGameplayCueOnActor(Burst) (Ability|GetAvatarActorfromActorInfo) "(TagName=\"GameplayCue.AttackHint\")" (Ability|GameplayCue|MakeGameplayCueParameters :Location (.location (Transformation|GetSocketTransform (Class|GameplayAbility|GetOwningComponentfromActorInfo) "AttackHint" "RTS_Component")))))
            (:OnFinish
              (Ability|Animation|MontageJumptoSection (Components|SkeletalMesh|GetAnimInstance (.skeletalmeshcomponent (Ability|GetActorInfo))) "EndLoop" "/Game/TBOProject/Art/Creatures/Birdman/AM_B03_Attack_Birdman_Montage.AM_B03_Attack_Birdman_Montage")
              (Ability|Tasks|WaitGameplayEvent "(TagName=\"Event.CommitAttack\")" 0
                (:EventReceived
                  (bind _returnvalue_5 (Class|Shooter|GetMuzzlesController(Message) (Ability|GetAvatarActorfromActorInfo)))
                  (Class|MuzzlesController|ShootwithMuzzle _returnvalue_5 0 (Variables|Default|GetProjectileType) (.ReturnValue (Class|AbilitySystemComponent|GetGameplayAttributeValue _returnvalue_3 "(AttributeName=\"BulletSpeed\",Attribute=/Script/TBO_01.ShooterCreatureAttributeSet:BulletSpeed,AttributeOwner=\"/Script/CoreUObject.Class'/Script/TBO_01.B03AttributeSet'\")")) (Variables|Default|GetTarget) (.ReturnValue (Class|AbilitySystemComponent|GetGameplayAttributeValue _returnvalue_3 "(AttributeName=\"Attack\",Attribute=/Script/TBO_01.BaseCreatureAttributeSet:Attack,AttributeOwner=\"/Script/CoreUObject.Class'/Script/TBO_01.BaseCreatureAttributeSet'\")")) (.ReturnValue (Class|AbilitySystemComponent|GetGameplayAttributeValue _returnvalue_3 "(AttributeName=\"CharacterLevel\",Attribute=/Script/TBO_01.BaseCreatureAttributeSet:CharacterLevel,AttributeOwner=\"/Script/CoreUObject.Class'/Script/TBO_01.BaseCreatureAttributeSet'\")")) (.ReturnValue (Class|AbilitySystemComponent|GetGameplayAttributeValue _returnvalue_3 "(AttributeName=\"KnockBackIntensity\",Attribute=/Script/TBO_01.BaseCreatureAttributeSet:KnockBackIntensity,AttributeOwner=\"/Script/CoreUObject.Class'/Script/TBO_01.BaseCreatureAttributeSet'\")")))
                  (Abilities|TryActivateAbilitybyClass (Ability|GetAbilitySystemComponentfromActorInfo) "/Game/TBOProject/Core/Creatures/Abilities/Action_Abilities/GA_OpenEyes.GA_OpenEyes_C" true)
                  (Ability|Tasks|WaitDelay (.ReturnValue (Class|AbilitySystemComponent|GetGameplayAttributeValue _returnvalue_3 "(AttributeName=\"ShootRecoilTime\",Attribute=/Script/TBO_01.ShooterCreatureAttributeSet:ShootRecoilTime,AttributeOwner=\"/Script/CoreUObject.Class'/Script/TBO_01.B03AttributeSet'\")"))
                    (:OnFinish
                      (Ability|Animation|MontageJumptoSection (Components|SkeletalMesh|GetAnimInstance (.skeletalmeshcomponent (Ability|GetActorInfo))) "EndLoop" "/Game/TBOProject/Art/Creatures/Birdman/AM_B03_Recovery_Birdman_MontageLoop.AM_B03_Recovery_Birdman_MontageLoop"))))))))))
    (:OnBlendOut
      (|PlayMontageandWaitProxy "None" "/Game/TBOProject/Art/Creatures/Birdman/AM_B03_Recovery_Birdman_MontageLoop.AM_B03_Recovery_Birdman_MontageLoop" 1.0 "None" true 1.0 0.0 false
        (:OnCompleted
          _)
        (:OnBlendOut
          _)
        (:OnInterrupted
          _)
        (:OnCancelled
          _))
      (Ability|EndAbility))))
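; Event-triggered ranged attack ability for the B03 Birdman creature, firing a projectile at the event's target.
; An attribute-timed wait jumps the attack montage to EndLoop and shows an AttackHint cue, then Event.CommitAttack fires through the muzzle controller using attribute-driven stats.
; A second timed wait repeats the EndLoop jump.
; Montage blend-out plays recovery and activates GA_CloseEyes, and ending the ability applies GE_ShootingDelay to the owner.
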(event Ability|EventOnEndAbility
  (params (bWasCancelled :type Boolean))
  (Ability|ApplyGameplayEffectToOwner "/Game/TBOProject/Core/Creatures/Abilities/Effects/GE_ShootingDelay.GE_ShootingDelay_C"))

(event Ability|EventActivateAbilityFromEvent
  (params (EventData :type Gameplay%20Event%20Data%20Structure%20%28by%20ref%29))
  (bind _returnvalue (Ability|GetAbilitySystemComponentfromActorInfo))
  (Variables|Default|SetTarget (.target EventData))
  (|PlayMontageandWaitProxy "None" "/Game/TBOProject/Art/Creatures/Birdman/AM_B03_Attack_Birdman_Montage.AM_B03_Attack_Birdman_Montage" 1.0 "None" true 1.0 0.0 false
    (:then
      (Ability|Tasks|WaitDelay (.ReturnValue (Class|AbilitySystemComponent|GetGameplayAttributeValue (Ability|GetAbilitySystemComponentfromActorInfo) "(AttributeName=\"ShootChargeTime\",Attribute=/Script/TBO_01.ShooterCreatureAttributeSet:ShootChargeTime,AttributeOwner=\"/Script/CoreUObject.Class'/Script/TBO_01.ShooterCreatureAttributeSet'\")"))
        (:OnFinish
          (Ability|Animation|MontageJumptoSection (Components|SkeletalMesh|GetAnimInstance (.skeletalmeshcomponent (Ability|GetActorInfo))) "EndLoop" "/Game/TBOProject/Art/Creatures/Birdman/AM_B03_Attack_Birdman_Montage.AM_B03_Attack_Birdman_Montage")
          (GameplayCue|ExecuteGameplayCueOnActor(Burst) (Ability|GetAvatarActorfromActorInfo) "(TagName=\"GameplayCue.AttackHint\")" (Ability|GameplayCue|MakeGameplayCueParameters :Location (.location (Transformation|GetSocketTransform (Class|GameplayAbility|GetOwningComponentfromActorInfo) "AttackHint" "RTS_Component"))))
          (Ability|Tasks|WaitGameplayEvent "(TagName=\"Event.CommitAttack\")" 0
            (:EventReceived
              (bind _returnvalue_2 (Class|Shooter|GetMuzzlesController(Message) (Ability|GetAvatarActorfromActorInfo)))
              (Class|MuzzlesController|ShootwithMuzzle _returnvalue_2 0 (Variables|Default|GetProjectileType) (.ReturnValue (Class|AbilitySystemComponent|GetGameplayAttributeValue _returnvalue "(AttributeName=\"BulletSpeed\",Attribute=/Script/TBO_01.ShooterCreatureAttributeSet:BulletSpeed,AttributeOwner=\"/Script/CoreUObject.Class'/Script/TBO_01.B03AttributeSet'\")")) (Variables|Default|GetTarget) (.ReturnValue (Class|AbilitySystemComponent|GetGameplayAttributeValue _returnvalue "(AttributeName=\"Attack\",Attribute=/Script/TBO_01.BaseCreatureAttributeSet:Attack,AttributeOwner=\"/Script/CoreUObject.Class'/Script/TBO_01.BaseCreatureAttributeSet'\")")) (.ReturnValue (Class|AbilitySystemComponent|GetGameplayAttributeValue _returnvalue "(AttributeName=\"CharacterLevel\",Attribute=/Script/TBO_01.BaseCreatureAttributeSet:CharacterLevel,AttributeOwner=\"/Script/CoreUObject.Class'/Script/TBO_01.BaseCreatureAttributeSet'\")")) (.ReturnValue (Class|AbilitySystemComponent|GetGameplayAttributeValue _returnvalue "(AttributeName=\"KnockBackIntensity\",Attribute=/Script/TBO_01.BaseCreatureAttributeSet:KnockBackIntensity,AttributeOwner=\"/Script/CoreUObject.Class'/Script/TBO_01.BaseCreatureAttributeSet'\")")))
              (Ability|Tasks|WaitDelay (.ReturnValue (Class|AbilitySystemComponent|GetGameplayAttributeValue _returnvalue "(AttributeName=\"ShootRecoilTime\",Attribute=/Script/TBO_01.ShooterCreatureAttributeSet:ShootRecoilTime,AttributeOwner=\"/Script/CoreUObject.Class'/Script/TBO_01.B03AttributeSet'\")"))
                (:OnFinish
                  (Ability|Animation|MontageJumptoSection (Components|SkeletalMesh|GetAnimInstance (.skeletalmeshcomponent (Ability|GetActorInfo))) "EndLoop" "/Game/TBOProject/Art/Creatures/Birdman/AM_B03_Attack_Birdman_Montage.AM_B03_Attack_Birdman_Montage"))))))))
    (:OnBlendOut
      (|PlayMontageandWaitProxy "None" "/Game/TBOProject/Art/Creatures/Birdman/AM_B03_Recovery_Birdman_Montage.AM_B03_Recovery_Birdman_Montage" 1.0 "None" true 1.0 0.0 false
        (:then
          (Abilities|TryActivateAbilitybyClass (Ability|GetAbilitySystemComponentfromActorInfo) "/Game/TBOProject/Core/Creatures/Abilities/Action_Abilities/GA_CloseEyes.GA_CloseEyes_C" true)
          (Development|PrintText "Close"))
        (:OnCompleted
          (Ability|EndAbility :!label _label))
        (:OnBlendOut
          (goto _label))
        (:OnInterrupted
          (goto _label))
        (:OnCancelled
          (goto _label))))))
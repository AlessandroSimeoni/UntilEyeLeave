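; Gameplay ability that teleports the B04 creature to the nest position stored on its B04 controller.
; It fires the Teleport gameplay cue on the avatar both before and after the move, which lands in walking mode.
; It then overwrites the blackboard's DistanceToPlayer with a large value and ends, though EndAbility runs only when that blackboard is valid.
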(event Ability|EventActivateAbility
  (bind _returnvalue (Ability|GameplayCue|MakeGameplayCueParameters 0.0))
  (bind _ascreature (Utilities|Casting|CastToCreature (Ability|GetAvatarActorfromActorInfo)))
  (bind _asb04_controller (Utilities|Casting|CastToB04_Controller (Pawn|GetController _ascreature)))
  (GameplayCue|ExecuteGameplayCueOnActor(Burst) (Ability|GetAvatarActorfromActorInfo) "(TagName=\"GameplayCue.Teleport\")" _returnvalue)
  (Class|Creature|Teleport _ascreature (Variables|/Script/TBO_01.B04_Controller|GetNestPosition _asb04_controller) "MOVE_Walking")
  (GameplayCue|ExecuteGameplayCueOnActor(Burst) (Ability|GetAvatarActorfromActorInfo) "(TagName=\"GameplayCue.Teleport\")" _returnvalue)
  (Utilities|IsValid (AI|GetBlackboard _asb04_controller)
    (:Is%20Valid
      (AI|Components|Blackboard|SetValueasFloat (AI|GetBlackboard _asb04_controller) (Utilities|Name|MakeLiteralName "DistanceToPlayer") 3e+04)
      (Ability|EndAbility))))
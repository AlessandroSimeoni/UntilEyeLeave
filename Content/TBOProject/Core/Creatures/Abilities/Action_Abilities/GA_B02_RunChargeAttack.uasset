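; Gameplay ability for creature B02's running charge attack: a telegraphed wind-up followed by a forward lunge.
; Attribute-driven delays time the looping charge montage, triggering GA_CancelFocus and an AttackHint cue before jumping to EndLoop.
; On blend-out, the attack montage plays with forward constant-force root motion, whose strength and duration come from attributes.
; The ability ends when that force finishes or the charge is interrupted or cancelled.
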(event Ability|EventActivateAbility
  (bind _returnvalue (Ability|GetAbilitySystemComponentfromActorInfo))
  (|PlayMontageandWaitProxy "None" "/Game/TBOProject/Art/Creatures/Mousetrap/AM_B02_Charge.AM_B02_Charge" 1.0 "None" true 1.0 0.0 false
    (:then
      (Ability|Tasks|WaitDelay (.ReturnValue (Class|AbilitySystemComponent|GetGameplayAttributeValue (Ability|GetAbilitySystemComponentfromActorInfo) "(AttributeName=\"AttackChargeTime\",Attribute=/Script/TBO_01.B02AttributeSet:AttackChargeTime,AttributeOwner=\"/Script/CoreUObject.Class'/Script/TBO_01.B02AttributeSet'\")"))
        (:OnFinish
          (Abilities|TryActivateAbilitybyClass (Ability|GetAbilitySystemComponentfromActorInfo) "/Game/TBOProject/Core/Creatures/Abilities/Action_Abilities/GA_CancelFocus.GA_CancelFocus_C" true)
          (GameplayCue|ExecuteGameplayCueOnActor(Burst) (Ability|GetAvatarActorfromActorInfo) "(TagName=\"GameplayCue.AttackHint\")" (Ability|GameplayCue|MakeGameplayCueParameters :Location (.location (Transformation|GetSocketTransform (Class|GameplayAbility|GetOwningComponentfromActorInfo) "AttackHint" "RTS_Component"))))
          (Ability|Tasks|WaitDelay (.ReturnValue (Class|AbilitySystemComponent|GetGameplayAttributeValue (Ability|GetAbilitySystemComponentfromActorInfo) "(AttributeName=\"NonFocusDelayAfterCharge\",Attribute=/Script/TBO_01.B02AttributeSet:NonFocusDelayAfterCharge,AttributeOwner=\"/Script/CoreUObject.Class'/Script/TBO_01.B02AttributeSet'\")"))
            (:OnFinish
              (Ability|Animation|MontageJumptoSection (Components|SkeletalMesh|GetAnimInstance (.skeletalmeshcomponent (Ability|GetActorInfo))) "EndLoop" "/Game/TBOProject/Art/Creatures/Mousetrap/AM_B02_Charge.AM_B02_Charge"))))))
    (:OnCompleted
      (Development|PrintText "Charge Complete"))
    (:OnBlendOut
      (|PlayMontageandWaitProxy "None" "/Game/TBOProject/Art/Creatures/Mousetrap/AM_B02_ChargeAttack.AM_B02_ChargeAttack" 1.0 "None" true 1.0 0.0 false
        (:then
          (Ability|Tasks|ApplyRootMotionConstantForce "None" (Transformation|GetActorForwardVector (Ability|GetAvatarActorfromActorInfo)) (* (.ReturnValue (Class|AbilitySystemComponent|GetGameplayAttributeValue _returnvalue "(AttributeName=\"AttackingSpeed\",Attribute=/Script/TBO_01.B02AttributeSet:AttackingSpeed,AttributeOwner=\"/Script/CoreUObject.Class'/Script/TBO_01.B02AttributeSet'\")")) 1e+03) (.ReturnValue (Class|AbilitySystemComponent|GetGameplayAttributeValue _returnvalue "(AttributeName=\"AttackDuration\",Attribute=/Script/TBO_01.B02AttributeSet:AttackDuration,AttributeOwner=\"/Script/CoreUObject.Class'/Script/TBO_01.B02AttributeSet'\")")) false 0 "MaintainLastRootMotionVelocity" "0, 0, 0" 0.0 true
            (:OnFinish
              (Ability|EndAbility))))))
    (:OnInterrupted
      (Ability|EndAbility :!label _label))
    (:OnCancelled
      (goto _label))))

(event Ability|EventOnEndAbility
  (params (bWasCancelled :type Boolean)))
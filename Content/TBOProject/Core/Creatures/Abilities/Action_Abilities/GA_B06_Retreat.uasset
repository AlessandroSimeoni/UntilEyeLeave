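; Gameplay ability that makes the B06 creature retreat in a scared state.
; On activation it adds a non-replicated loose Status.Scared tag to the avatar and plays the retreat montage.
; A delay, timed by a gameplay attribute, starts alongside the montage and ends the ability, which removes the tag.
; An alternative idle-retreat montage node is present but unconnected.
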(event Ability|EventActivateAbility
  (Ability|GameplayEffect|AddLooseGameplayTags (Ability|GetAvatarActorfromActorInfo) (GameplayTags|MakeLiteralGameplayTagContainer "(GameplayTags=((TagName=\"Status.Scared\")))"))
  (|PlayMontageandWaitProxy "None" "/Game/TBOProject/Art/Creatures/Stealer/B06_Artist/NewAnimation/AM_B06_Retreat_Montage.AM_B06_Retreat_Montage" 1.0 "None" true 1.0 0.0 false
    (:then
      (Ability|Tasks|WaitDelay (.ReturnValue (Class|AbilitySystemComponent|GetGameplayAttributeValue (Ability|GetAbilitySystemComponentfromActorInfo) "(AttributeName=\"ShieldedDuration\",Attribute=/Script/TBO_01.B06AttributeSet:ShieldedDuration,AttributeOwner=\"/Script/CoreUObject.Class'/Script/TBO_01.B06AttributeSet'\")"))
        (:OnFinish
          (Ability|EndAbility))))))

(event Ability|EventOnEndAbility
  (params (bWasCancelled :type Boolean))
  (Ability|GameplayEffect|RemoveLooseGameplayTags (Ability|GetAvatarActorfromActorInfo) (GameplayTags|MakeLiteralGameplayTagContainer "(GameplayTags=((TagName=\"Status.Scared\")))")))
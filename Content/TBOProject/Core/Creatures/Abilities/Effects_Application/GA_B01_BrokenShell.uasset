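; Gameplay ability that handles the B01 creature's shell breaking.
; On activation it disables effect navigation on the Creature avatar and applies the GE_B01_Broken gameplay effect to the owner.
; If the owner has the Status.Spotted tag, it adds spotted combat audio through the audio subsystem.
; It then ends immediately and removes the loose Status.Shielded tag from the avatar without replication.
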(event Ability|EventActivateAbility
  (bind _ascreature (Utilities|Casting|CastToCreature (Ability|GetAvatarActorfromActorInfo))
    (:then
      (Class|Creature|SetEffectNavigation _ascreature false))
    (:CastFailed
      _))
  (Ability|ApplyGameplayEffectToOwner "/Game/TBOProject/Core/Creatures/Abilities/Effects/GE_B01_Broken.GE_B01_Broken_C")
  (if (GameplayTags|HasMatchingGameplayTag (Ability|GetAbilitySystemComponent (Ability|GetAvatarActorfromActorInfo)) "(TagName=\"Status.Spotted\")")
    (Class|AudioSubsystem|AddSpottedCombatAudio (Subsystems|GetAudioSubsystem)))
  (Ability|EndAbility)
  (Ability|GameplayEffect|RemoveLooseGameplayTags (Ability|GetAvatarActorfromActorInfo) (GameplayTags|MakeLiteralGameplayTagContainer "(GameplayTags=((TagName=\"Status.Shielded\")))")))

(event Ability|EventOnEndAbility
  (params (bWasCancelled :type Boolean)))
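; Gameplay ability for the B06 AI creature that makes it react to a detected coin and take possession of it.
; On activation it sets the blackboard Stop flag, activates GA_OpenEyes, applies the pick-up effect and plays the coin-detected montage.
; The with-coin effect applies as the montage starts; completion, interruption or cancellation all set CoinPossessed and end the ability.
; Ending clears Stop; without a valid blackboard the ability ends immediately.
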(event Ability|EventActivateAbility
  (bind _returnvalue (Ability|GetAvatarActorfromActorInfo))
  (bind _returnvalue_2 (Ability|GetAvatarActorfromActorInfo))
  (bind _returnvalue_3 (AI|GetAIController _returnvalue))
  (bind _returnvalue_4 (AI|GetAIController _returnvalue_2))
  (bind _returnvalue_5 (AI|GetBlackboard _returnvalue_3))
  (bind _returnvalue_6 (AI|GetBlackboard _returnvalue_4))
  (Utilities|IsValid _returnvalue_5
    (:Is%20Valid
      (AI|Components|Blackboard|SetValueasBool _returnvalue_5 (Utilities|Name|MakeLiteralName "Stop") true)
      (Abilities|TryActivateAbilitybyClass (Ability|GetAbilitySystemComponentfromActorInfo) "/Game/TBOProject/Core/Creatures/Abilities/Action_Abilities/GA_OpenEyes.GA_OpenEyes_C" true)
      (Ability|ApplyGameplayEffectToOwner "/Game/TBOProject/Core/Creatures/Abilities/Effects/GE_B06_PickUpCoin.GE_B06_PickUpCoin_C")
      (|PlayMontageandWaitProxy "None" "/Game/TBOProject/Art/Creatures/Stealer/B06_Mike/Animation/B06_CoinDetected_Montage.B06_CoinDetected_Montage" 1.0 "None" true 1.0 0.0 false
        (:then
          (Ability|ApplyGameplayEffectToOwner "/Game/TBOProject/Core/Creatures/Abilities/Effects/GE_B06_WithCoin.GE_B06_WithCoin_C"))
        (:OnCompleted
          (Utilities|IsValid _returnvalue_6 :!label _label
            (:Is%20Valid
              (AI|Components|Blackboard|SetValueasBool _returnvalue_6 (Utilities|Name|MakeLiteralName "CoinPossessed") true))
            (:Is%20Not%20Valid
              _))
          (Ability|EndAbility))
        (:OnInterrupted
          (goto _label))
        (:OnCancelled
          (goto _label))))
    (:Is%20Not%20Valid
      (Ability|EndAbility))))

(event Ability|EventOnEndAbility
  (params (bWasCancelled :type Boolean))
  (bind _returnvalue (Ability|GetAvatarActorfromActorInfo))
  (bind _returnvalue_2 (AI|GetAIController _returnvalue))
  (bind _returnvalue_3 (AI|GetBlackboard _returnvalue_2))
  (Utilities|IsValid _returnvalue_3
    (:Is%20Valid
      (AI|Components|Blackboard|SetValueasBool _returnvalue_3 (Utilities|Name|MakeLiteralName "Stop") false))))
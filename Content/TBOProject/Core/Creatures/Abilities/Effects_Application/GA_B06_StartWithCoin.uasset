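; Gameplay ability that starts creature B06 in a state where it already holds a coin.
; On activation it triggers the GA_OpenEyes ability and applies the GE_B06_WithCoin effect to its owner.
; If the avatar's AI controller has a valid blackboard, it sets CoinPossessed to true and applies GE_B06_PickUpCoin, then ends.
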(event Ability|EventActivateAbility
  (bind _returnvalue (Ability|GetAvatarActorfromActorInfo))
  (bind _returnvalue_2 (AI|GetAIController _returnvalue))
  (bind _returnvalue_3 (AI|GetBlackboard _returnvalue_2))
  (Abilities|TryActivateAbilitybyClass (Ability|GetAbilitySystemComponentfromActorInfo) "/Game/TBOProject/Core/Creatures/Abilities/Action_Abilities/GA_OpenEyes.GA_OpenEyes_C" true)
  (Ability|ApplyGameplayEffectToOwner "/Game/TBOProject/Core/Creatures/Abilities/Effects/GE_B06_WithCoin.GE_B06_WithCoin_C")
  (Utilities|IsValid _returnvalue_3
    (:Is%20Valid
      (AI|Components|Blackboard|SetValueasBool _returnvalue_3 (Utilities|Name|MakeLiteralName "CoinPossessed") true)
      (Ability|ApplyGameplayEffectToOwner "/Game/TBOProject/Core/Creatures/Abilities/Effects/GE_B06_PickUpCoin.GE_B06_PickUpCoin_C"))
    (:Is%20Not%20Valid
      _))
  (Ability|EndAbility))
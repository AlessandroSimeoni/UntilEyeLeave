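; GA_B02_Charge is the gameplay ability that puts creature B02 into its charge state.
; On activation it halts the AI through the "Stop" blackboard key, applies the charge effect to itself and emits a charge noise event.
; It starts the hit-stun montage and immediately triggers the TimeBomb ability alongside it.
; The ability ends when the montage finishes or is interrupted, and ending clears the "Stop" key.
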(event Ability|EventOnEndAbility
  (params (bWasCancelled :type Boolean))
  (AI|Components|Blackboard|SetValueasBool (Variables|Default|GetBlackBoard) (Utilities|Name|MakeLiteralName "Stop") false))

(event Ability|EventActivateAbilityFromEvent
  (params (EventData :type Gameplay%20Event%20Data%20Structure%20%28by%20ref%29))
  (bind _returnvalue (Ability|GetAvatarActorfromActorInfo))
  (bind _output_get (Variables|Default|SetBlackBoard (AI|GetBlackboard (AI|GetAIController (Ability|GetAvatarActorfromActorInfo)))))
  (AI|Components|Blackboard|SetValueasBool _output_get (Utilities|Name|MakeLiteralName "Stop") true)
  (Ability|ApplyGameplayEffectToOwner "/Game/TBOProject/Core/Creatures/Abilities/Effects/Charge/GE_B02_Charge.GE_B02_Charge_C")
  (Class|AISenseHearing|ReportNoiseEvent (Transformation|GetActorLocation _returnvalue) 1.0 _returnvalue 2.5e+03 (Utilities|Name|EnumtoName (Variables|Default|GetChargeNoise)))
  (|PlayMontageandWaitProxy "None" "/Game/TBOProject/Art/Creatures/Mousetrap/AM_B02_HitStun.AM_B02_HitStun" 1.0 "None" true 1.0 0.0 false
    (:then
      (Abilities|TryActivateAbilitybyClass (Ability|GetAbilitySystemComponentfromActorInfo) "/Game/TBOProject/Core/Creatures/Abilities/Action_Abilities/Charged/GA_B02_TimeBomb.GA_B02_TimeBomb_C" true))
    (:OnCompleted
      (Ability|EndAbility :!label _label))
    (:OnBlendOut
      (goto _label))
    (:OnInterrupted
      (goto _label))
    (:OnCancelled
      (goto _label))))
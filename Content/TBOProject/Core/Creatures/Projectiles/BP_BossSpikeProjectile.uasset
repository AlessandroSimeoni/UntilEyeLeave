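; Boss spike projectile that animates through a load phase and a shoot phase using two timelines.
; LoadProjectile slides it along its forward vector over a given load time, snaps it to the target position and broadcasts that loading is over.
; StartShoot nudges it forward incrementally by a curve, then broadcasts ready-to-shoot, activates its Niagara effect and plays the bullet sound.
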(event EventLoadProjectile
  (params (LoadTime :type Float%20%28single-precision%29) (TargetPosition :type Vector :default "0, 0, 0"))
  (Actor|Tick|SetActorTickEnabled true)
  (Components|Tick|SetComponentTickEnabled (Variables|Default|GetNiagara) false)
  (bind _output_get (Variables|Default|SetStartingLocation (Transformation|GetActorLocation)))
  (bind _output_get_2 (Variables|Default|SetLoadMovementLength (Math|Vector|VectorLength (- _output_get TargetPosition))))
  (Components|Timeline|SetPlayRate (Variables|Default|GetLoadProjectileTimeline) (/ 1.0 LoadTime))
  (bind _loadtrack (Timeline|LoadProjectileTimeline PlayFromStart)
    (:Update
      (Transformation|SetActorLocation (+ (* (Transformation|GetActorForwardVector) (* _loadtrack _output_get_2)) (Variables|Default|GetStartingLocation)) false false))
    (:Finished
      (Transformation|SetActorLocation TargetPosition false false)
      (Class|SpikeProjectile|BroadcastLoadOver))))

(event EventStartShoot
  (Components|Tick|SetComponentTickEnabled (Variables|Default|GetNiagara) true)
  (bind _shoottrack (Timeline|ShootTimeline Play)
    (:Update
      (Transformation|SetActorLocation (+ (* (Transformation|GetActorForwardVector) _shoottrack) (Transformation|GetActorLocation)) false false))
    (:Finished
      (Class|SpikeProjectile|BroadcastReadytoShoot)
      (Components|Activation|Activate (Variables|Default|GetNiagara) false)
      (Audio|PlaySoundatLocation "/Game/TBOProject/Media/Sound/MetasoundSystems/MS_Boss_Bullet.MS_Boss_Bullet" (Transformation|GetActorLocation) "0, 0, 0" 1e+01 1.0 0.0 0 0 0 0))))

(fn ConstructionScript)
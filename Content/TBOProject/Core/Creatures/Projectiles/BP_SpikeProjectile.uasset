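; BP_SpikeProjectile is a creature spike projectile that moves in two timeline-driven phases: loading into position, then shooting.
; LoadProjectile scales the timeline's play rate by LoadTime, slides along the forward vector by the distance to TargetPosition, snaps there and broadcasts LoadOver.
; StartShoot adds a curve-driven forward offset to the current location each update, then broadcasts ReadyToShoot.
; All movement sets location directly without sweeping.
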(event EventLoadProjectile
  (params (LoadTime :type Float%20%28single-precision%29) (TargetPosition :type Vector :default "0, 0, 0"))
  (bind _output_get (Variables|Default|SetStartingLocation (Transformation|GetActorLocation)))
  (bind _output_get_2 (Variables|Default|SetLoadMovementLength (Math|Vector|VectorLength (- _output_get TargetPosition))))
  (Components|Timeline|SetPlayRate (Variables|Default|GetLoadProjectileTimeline) (/ 1.0 LoadTime))
  (bind _loadtrack (Timeline|LoadProjectileTimeline PlayFromStart)
    (:Update
      (Transformation|SetActorLocation (+ (* (Transformation|GetActorForwardVector) (* _loadtrack _output_get_2)) (Variables|Default|GetStartingLocation)) false false))
    (:Finished
      (Transformation|SetActorLocation TargetPosition false false)
      (Class|SpikeProjectile|BroadcastLoadOver))))

(event EventStartShoot
  (bind _shoottrack (Timeline|ShootTimeline PlayFromStart)
    (:Update
      (Transformation|SetActorLocation (+ (* (Transformation|GetActorForwardVector) _shoottrack) (Transformation|GetActorLocation)) false false))
    (:Finished
      (Class|SpikeProjectile|BroadcastReadytoShoot))))

(fn ConstructionScript)
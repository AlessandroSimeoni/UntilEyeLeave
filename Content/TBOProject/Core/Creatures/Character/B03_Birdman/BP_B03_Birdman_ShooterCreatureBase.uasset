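; Base Blueprint for the B03 Birdman shooter creature, handling its reaction to a broken shell or shield through BrokenSheel.
; BrokenSheel prints a gameplay attribute for debugging, then sets walk speed and yaw rotation rate from Ability System attribute values.
; It then activates GA_B01_Stun, a stun ability with a B01 prefix, with remote activation disallowed.
; The construction script only calls the parent.
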(fn ConstructionScript
  (|CallParentFunction))

(fn BrokenSheel
  (bind _charactermovement (Variables|Character|GetCharacterMovement))
  (bind _abilitysystemcomponent (Variables|Default|GetAbilitySystemComponent))
  (bind _returnvalue (Class|AbilitySystemComponent|GetGameplayAttributeValue _abilitysystemcomponent "(AttributeName=\"BrokenWalkSpeed\",Attribute=/Script/TBO_01.B01DestructibleAttributeSet:BrokenWalkSpeed,AttributeOwner=\"/Script/CoreUObject.Class'/Script/TBO_01.B01DestructibleAttributeSet'\")"))
  (Development|PrintText (Utilities|Text|ToText(Float) _returnvalue "HalfToEven"))
  (Variables|/Script/Engine.CharacterMovementComponent|SetMaxWalkSpeed _charactermovement _returnvalue)
  (Variables|/Script/Engine.CharacterMovementComponent|SetRotationRate _charactermovement (Math|Rotator|MakeRotator 0.0 0.0 (.ReturnValue (Class|AbilitySystemComponent|GetGameplayAttributeValue _abilitysystemcomponent "(AttributeName=\"BrokenWalkRotationSpeed\",Attribute=/Script/TBO_01.B01DestructibleAttributeSet:BrokenWalkRotationSpeed,AttributeOwner=\"/Script/CoreUObject.Class'/Script/TBO_01.B01DestructibleAttributeSet'\")"))))
  (Abilities|TryActivateAbilitybyClass (Variables|Default|GetAbilitySystemComponent) "/Game/TBOProject/Core/Creatures/Abilities/FeedBack_Abilities/HitStun/GA_B01_Stun.GA_B01_Stun_C" false))
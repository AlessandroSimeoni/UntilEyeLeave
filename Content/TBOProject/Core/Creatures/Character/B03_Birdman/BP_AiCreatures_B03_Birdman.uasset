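; AI controller for the B03 Birdman creature that runs its behavior tree and reacts to hearing and losing actors.
; Losing the player applies the Searching gameplay effect through GAS; RemoveSearchingTag, despite its name, applies the same effect and stores its handle.
; A Charged Sound from a creature sets the ChargedCreature blackboard key, tracks that creature and activates the view ability.
; When a tracked creature dies, the key switches to a random remaining one or clears.
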(event Custom|OnDeath_Event
  (params (Actor :type Actor%20Object%20Reference) (Instigator :type Actor%20Object%20Reference))
  (bind _returnvalue (Utilities|Name|MakeLiteralName "ChargedCreature"))
  (bind _blackboard (Variables|Default|GetBlackboard))
  (bind _chargedcreatures (Variables|Default|GetChargedCreatures))
  (bind _outitem (Utilities|Array|Random _chargedcreatures))
  (Utilities|Array|RemoveItem _chargedcreatures Actor)
  (Utilities|IsValid _outitem
    (:Is%20Valid
      (AI|Components|Blackboard|SetValueasObject _blackboard _returnvalue _outitem))
    (:Is%20Not%20Valid
      (AI|Components|Blackboard|ClearValue _blackboard _returnvalue))))

(event EventActorHeared
  (params (HearedActor :type Actor%20Object%20Reference) (NoiseType :type ENoiseAction%20Enum :default "None") (IsValid :type Boolean))
  (|CallParentFunction HearedActor NoiseType IsValid)
  (bind _ascreature (Utilities|Casting|CastToCreature HearedActor))
  (switch Utilities|FlowControl|Switch|SwitchonENoiseAction NoiseType
    (:ChargedSound
      (AI|Components|Blackboard|SetValueasObject (Variables|Default|GetBlackboard) (Utilities|Name|MakeLiteralName "ChargedCreature") HearedActor)
      (EventDispatchers|AssignOnDeath _ascreature (delegate Custom|OnDeath_Event))
      (Utilities|Array|AddUnique (Variables|Default|GetChargedCreatures) HearedActor)
      (Abilities|TryActivateAbilitybyClass (Ability|GetAbilitySystemComponent (Pawn|GetControlledPawn)) "/Game/TBOProject/Core/Creatures/Abilities/FeedBack_Abilities/View/GA_B03_ChargedCreatureView.GA_B03_ChargedCreatureView_C" true))))

(event EventBeginPlay
  (|CallParentFunction)
  (AI|RunBehaviorTree "/Game/TBOProject/Core/Creatures/BehaviorTree/Tree/B03_Tree/BT_B03_Birdman.BT_B03_Birdman")
  (Utilities|FlowControl|Delay 0.2))

(event EventActorLost
  (params (LostActor :type Actor%20Object%20Reference))
  (if (== LostActor (Game|GetPlayerCharacter 0))
    (GameplayEffects|ApplyGameplayEffectToSelf :self (Ability|GetAbilitySystemComponent (Pawn|GetControlledPawn)) :GameplayEffectClass "/Game/TBOProject/Core/Creatures/Abilities/Effects/GE_B03_Searching.GE_B03_Searching_C")))

(fn ConstructionScript
  (|CallParentFunction))

(fn RemoveSearchingTag
  (bind _returnvalue (GameplayEffects|ApplyGameplayEffectToSelf :self (Ability|GetAbilitySystemComponent (Pawn|GetControlledPawn)) :GameplayEffectClass "/Game/TBOProject/Core/Creatures/Abilities/Effects/GE_B03_Searching.GE_B03_Searching_C"))
  (Variables|Default|SetActiveSearchingEffect _returnvalue))
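; Destructible variant of the B01 Gianguscio shooter creature, with a shell that can be broken.
; BeginPlay registers the destructible part components and binds a cached Chaos collection to the GeometryCollection, which is destroyed when a break event fires.
; BrokenSheel activates broken-shell and stun abilities, plays the cached fracture with a placeholder sound, and switches collision from the intact box to the Broken component, letting pawns through the capsule.
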(event Custom|OnChaosBreakEvent_Event
  (params (BreakEvent :type Chaos%20Break%20Event%20Structure%20%28by%20ref%29))
  (Components|DestroyComponent (Variables|Default|GetGeometryCollection)))

(event EventBeginPlay
  (bind _b01destructiblepart (Variables|Default|GetB01DestructiblePart))
  (bind _geometrycollection (Variables|Default|GetGeometryCollection))
  (Class|DestructibleParts|RegisterComponent _b01destructiblepart (Variables|Default|GetStaticMesh))
  (Class|DestructibleParts|RegisterComponent _b01destructiblepart _b01destructiblepart)
  (Class|ChaosCacheHandler|InitializeCollection (Variables|Default|GetChaosCacheHandler) _geometrycollection "/Game/TBOProject/Art/Chaos/B01/CCC_B01_Pot.CCC_B01_Pot")
  (EventDispatchers|AssignOnChaosBreakEvent _geometrycollection (delegate Custom|OnChaosBreakEvent_Event)))

(event Collision|EventActorBeginOverlap
  (params (OtherActor :type Actor%20Object%20Reference))
  (|CallParentFunction OtherActor) ; This node is disabled and will not be called.\nDrag off pins to build functionality.
)

(event EventTick
  (params (DeltaSeconds :type Float%20%28single-precision%29)))

(fn ConstructionScript
  (|CallParentFunction))

(fn BrokenSheel
  (Abilities|TryActivateAbilitybyClass (Variables|Default|GetAbilitySystemComponent) "/Game/TBOProject/Core/Creatures/Abilities/Effects_Application/GA_B01_BrokenShell.GA_B01_BrokenShell_C" false)
  (Variables|/Script/Engine.PrimitiveComponent|SetCanCharacterStepUpOn (Variables|Default|GetCapsuleComponent) "ECB_No")
  (Abilities|TryActivateAbilitybyClass (Variables|Default|GetAbilitySystemComponent) "/Game/TBOProject/Core/Creatures/Abilities/FeedBack_Abilities/HitStun/GA_B01_Stun.GA_B01_Stun_C" false)
  (Rendering|SetVisibility (Variables|Default|GetGeometryCollection) true false)
  (Class|ChaosCacheHandler|Play (Variables|Default|GetChaosCacheHandler) 1.5)
  ;[1 1 1] cambiare suono
  (Audio|PlaySoundatLocation "/Game/TBOProject/Media/Sound/CreaturesSound_Placeholder/C01_AllVariants/SFX_C01_BreakableShell.SFX_C01_BreakableShell" (Transformation|GetWorldLocation (Variables|Default|GetCapsuleComponent)) "0, 0, 0" 1.0 1.0 0.0 0 0 0 0)
  (Collision|SetCollisionEnabled (Variables|Default|GetBox) "NoCollision")
  (Collision|SetCollisionResponsetoChannel (Variables|Default|GetCapsuleComponent) "ECC_Pawn" "ECR_Ignore")
  (Collision|SetCollisionEnabled (Variables|Default|GetBroken) "QueryAndPhysics"))
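; AI controller for the destructible Gianguscio (B01) shooter creature, running its behavior tree and driving its guard state through the IsGuarding blackboard key.
; Guarding starts from the pawn's StartInGuard setting, toggles on hurt box damage, and is forced on by valid scary sounds or trigger box damage other than 1.
; Destruction damage breaks the pawn's shell and swaps to the Broken behavior tree, carrying the Player blackboard value across.
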(event EventBeginPlay
  (|CallParentFunction)
  (AI|RunBehaviorTree "/Game/TBOProject/Core/Creatures/BehaviorTree/Tree/B01_Tree/BT_B01_Gianguscio.BT_B01_Gianguscio")
  (bind _asbp_b01_destructible_gianguscio_shooter_creature_base (Utilities|Casting|CastToBP_B01_Destructible_Gianguscio_ShooterCreatureBase (Pawn|GetControlledPawn)))
  (AI|Components|Blackboard|SetValueasBool (Variables|Default|GetBlackboard) (Utilities|Name|MakeLiteralName "IsGuarding") (Variables|/Game/TBOProject/Core/Creatures/Character/B01_Gianguscio/BP_B01_Destructible_Gianguscio_ShooterCreatureBase.BP_B01_Destructible_Gianguscio_ShooterCreatureBase_C|GetStartInGuard _asbp_b01_destructible_gianguscio_shooter_creature_base)))

(event EventActorHeared
  (params (HearedActor :type Actor%20Object%20Reference) (NoiseType :type ENoiseAction%20Enum :default "None") (IsValid :type Boolean))
  (|CallParentFunction HearedActor NoiseType IsValid)
  (switch Utilities|FlowControl|Switch|SwitchonENoiseAction NoiseType
    (:ScarySound
      (if IsValid
        (AI|Components|Blackboard|SetValueasBool (Variables|Default|GetBlackboard) (Utilities|Name|MakeLiteralName "IsGuarding") true)))))

(event EventTriggerBoxDamage
  (params (Attacker :type Actor%20Object%20Reference) (DamageType :type EDamageAction%20Enum :default "None") (DamageValue :type Float%20%28single-precision%29))
  (if (!= DamageValue 1.0)
    (AI|Components|Blackboard|SetValueasBool (Variables|Default|GetBlackboard) (Utilities|Name|MakeLiteralName "IsGuarding") true)))

(event EventActorDamage
  (params (Attacker :type Actor%20Object%20Reference) (DamageType :type EDamageAction%20Enum :default "None") (DamageValue :type Float%20%28single-precision%29))
  (switch Utilities|FlowControl|Switch|SwitchonEDamageAction DamageType
    (:HurtBoxDamage
      (AI|Components|Blackboard|SetValueasBool (Variables|Default|GetBlackboard) (Utilities|Name|MakeLiteralName "IsGuarding") (not (ScalableFloat|GetValueasBool (Variables|Default|GetBlackboard) (Utilities|Name|MakeLiteralName "IsGuarding")))))
    (:DestructionDamage
      (CallFunction|SetBroken))))

(fn ConstructionScript
  (|CallParentFunction))

(fn SetBroken
  (LocalVariables|SetBlackBoardPlayer (AI|Components|Blackboard|GetValueasObject (AI|GetBlackboard 0) (Utilities|Name|MakeLiteralName "Player")))
  (AI|Logic|StopLogic (Variables|Default|GetBrainComponent) "")
  (bind _asbp_b01_destructible_gianguscio_shooter_creature_base (Utilities|Casting|CastToBP_B01_Destructible_Gianguscio_ShooterCreatureBase (Pawn|GetControlledPawn)))
  (Default|BrokenSheel _asbp_b01_destructible_gianguscio_shooter_creature_base)
  (AI|RunBehaviorTree "/Game/TBOProject/Core/Creatures/BehaviorTree/Tree/B01_Tree/BT_B01_Broken.BT_B01_Broken")
  (AI|Components|Blackboard|SetValueasObject (AI|GetBlackboard 0) (Utilities|Name|MakeLiteralName "Player") (LocalVariables|GetBlackBoardPlayer)))
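; AI controller for the B06 Stealer creature that runs its behavior tree and reacts to the sound of coins.
; A heard coin becomes the Blackboard "Coin" target, joins a tracked list, and triggers the heard-coin Gameplay Ability and Rage effect on the pawn.
; When a tracked coin is destroyed, its destroy delegate removes it and retargets a random remaining coin, or clears the key if none is valid.
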(event Custom|OnDestroyed_Event
  (params (DestroyedActor :type Actor%20Object%20Reference))
  (bind _returnvalue (Utilities|Name|MakeLiteralName "Coin"))
  (bind _blackboard (Variables|Default|GetBlackboard))
  (bind _chargedcreatures (Variables|Default|GetChargedCreatures))
  (bind _outitem (Utilities|Array|Random _chargedcreatures))
  (Utilities|Array|RemoveItem _chargedcreatures DestroyedActor)
  (Utilities|IsValid _outitem
    (:Is%20Valid
      (AI|Components|Blackboard|SetValueasObject _blackboard _returnvalue _outitem))
    (:Is%20Not%20Valid
      (AI|Components|Blackboard|ClearValue _blackboard _returnvalue))))

(event EventActorHeared
  (params (HearedActor :type Actor%20Object%20Reference) (NoiseType :type ENoiseAction%20Enum :default "None") (IsValid :type Boolean))
  (bind _returnvalue (Pawn|GetControlledPawn))
  (bind _returnvalue_2 (Ability|GetAbilitySystemComponent _returnvalue))
  (|CallParentFunction HearedActor NoiseType IsValid)
  (Utilities|Casting|CastToCoin HearedActor)
  (switch Utilities|FlowControl|Switch|SwitchonENoiseAction NoiseType
    (:CoinSound
      (AI|Components|Blackboard|SetValueasObject (Variables|Default|GetBlackboard) (Utilities|Name|MakeLiteralName "Coin") HearedActor)
      (Game|AssignOnDestroyed HearedActor (delegate Custom|OnDestroyed_Event))
      (Utilities|Array|AddUnique (Variables|Default|GetChargedCreatures) HearedActor)
      (Abilities|TryActivateAbilitybyClass _returnvalue_2 "/Game/TBOProject/Core/Creatures/Abilities/FeedBack_Abilities/View/GA_B06_Heared_Coin.GA_B06_Heared_Coin_C" true)
      (GameplayEffects|ApplyGameplayEffectToSelf :self _returnvalue_2 :GameplayEffectClass "/Game/TBOProject/Core/Creatures/Abilities/Effects/GE_B06_Rage.GE_B06_Rage_C"))))

(event EventBeginPlay
  (|CallParentFunction)
  (AI|RunBehaviorTree "/Game/TBOProject/Core/Creatures/BehaviorTree/Tree/B06_tree/BT_B06_Stealer.BT_B06_Stealer"))

(fn ConstructionScript
  (|CallParentFunction))
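; Base Blueprint for creatures that reacts to damage on their eyes and to the loss of all eyes, using the Gameplay Ability System.
; An eye hit activates the hit-stun feedback ability by tag and flashes the damage component, with no active damage-amount check.
; When all eyes die, it activates the slow-death ability and sends itself a knockback gameplay event carrying the instigator.
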(event EventOnEyeHit
  (params (Eye :type Eye%20Scene%20Component%20Object%20Reference) (Damage :type Float%20%28single-precision%29) (ActorInstigator :type Actor%20Object%20Reference) (Force :type Float%20%28single-precision%29))
  (Abilities|TryActivateAbilitiesbyTag (Variables|Default|GetAbilitySystemComponent) (GameplayTags|MakeLiteralGameplayTagContainer "(GameplayTags=((TagName=\"FeedBack.HitStun\")))") true)
  (Class|DamageFlash|FlashDamage (Variables|Default|GetDamageFlashComponent)))

(event Collision|EventActorBeginOverlap
  (params (OtherActor :type Actor%20Object%20Reference)))

(event EventOnAllEyesDeath
  (params (Eye :type Eye%20Scene%20Component%20Object%20Reference) (ActorInstigator :type Actor%20Object%20Reference))
  (Abilities|TryActivateAbilitiesbyTag (Variables|Default|GetAbilitySystemComponent) (GameplayTags|MakeLiteralGameplayTagContainer "(GameplayTags=((TagName=\"FeedBack.Death.SlowDeath\")))") true)
  (Ability|SendGameplayEventtoActor self "(TagName=\"FeedBack.NockBack.DamageKnockback\")" (Utilities|Struct|MakeGameplayEventData "(TagName=\"\")" ActorInstigator 0 0 0 "()" "(GameplayTags=)" "(GameplayTags=)" 1.0 "()")))

(fn ConstructionScript)
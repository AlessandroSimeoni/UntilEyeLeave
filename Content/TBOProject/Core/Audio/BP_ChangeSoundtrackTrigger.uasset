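; BP_ChangeSoundtrackTrigger is a trigger actor that changes the game's music when the main character enters or leaves its area.
; On BeginPlay it casts player pawn 0 to BP_MainCharacter and caches that reference.
; Overlap begin and end events compare the other actor to it, then pass their own music selector to the AudioSubsystem's ChangeMusic.
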(event EventBeginPlay
  ;[1 1 1] Set Main Character Reference
  (CallFunction|SetMainCharacterReference))

(event Collision|EventActorBeginOverlap
  (params (OtherActor :type Actor%20Object%20Reference))
  ;[1 1 1] Set music on begin overlap
  (if (== OtherActor (Variables|Default|GetAs%20BP%20Main%20Character))
    (Class|AudioSubsystem|ChangeMusic (Subsystems|GetAudioSubsystem) (Variables|Music|GetMusicSelectorBeginOverlap))))

(event Collision|EventActorEndOverlap
  (params (OtherActor :type Actor%20Object%20Reference))
  ;[1 1 1] Set music on end overlap
  (if (== OtherActor (Variables|Default|GetAs%20BP%20Main%20Character))
    (Class|AudioSubsystem|ChangeMusic (Subsystems|GetAudioSubsystem) (Variables|Music|GetMusicSelectorEndOverlap))))

(fn ConstructionScript)

(fn SetMainCharacterReference
  (bind _asbp_main_character (Utilities|Casting|CastToBP_MainCharacter (Game|Player|GetPlayerPawn 0)))
  (Utilities|IsValid _asbp_main_character
    (:Is%20Valid
      (Variables|Default|SetAs%20BP%20Main%20Character _asbp_main_character))))
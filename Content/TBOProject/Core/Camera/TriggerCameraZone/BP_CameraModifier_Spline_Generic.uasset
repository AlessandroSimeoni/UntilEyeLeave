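; Camera trigger zone that applies a spline-based modifier to the game camera while a character is inside.
; On enter it passes its Spline, the world positions of its Start and End points, and settings for dolly, spring arm adaptation and movement speeds to the GameCamera.
; On exit it removes the modifier and resets camera rotation and length.
; The zone only forwards configuration, leaving the camera motion itself to GameCamera.
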(event EventOnCharacterEnter
  (params (GameCamera :type Game%20Camera%20Object%20Reference))
  (Class|GameCamera|AddSplineModifier GameCamera (Variables|Default|GetSpline) (Transformation|GetWorldLocation (Variables|Default|GetStart)) (Transformation|GetWorldLocation (Variables|Default|GetEnd)) (Variables|Default|GetUse%20Start%20End%20Point%20Distance) (Variables|Default|GetAdapt%20Spring%20Arm%20Lenght) (Variables|Default|GetDolly) (Variables|Default|GetDolly%20Aligned) (Variables|Default|GetRotation%20Speed) (Variables|Default|GetLenght%20Speed) (Variables|Default|GetSpline%20Movement%20Speed)))

(event EventOnCharacterExit
  (params (GameCamera :type Game%20Camera%20Object%20Reference))
  (Class|GameCamera|RemoveSplineModifier GameCamera true true))

(fn ConstructionScript)
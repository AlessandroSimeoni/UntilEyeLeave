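; General-purpose camera trigger zone modifier that adjusts the game camera's length, rotation and offset when a character enters or exits.
; On enter, per-property Modify flags decide which configured values are applied to the passed-in camera.
; On exit, independent Reset flags restore default length and rotation, while the offset reset re-sends the same offset with UseDefaultOffset false, the inverse of entry.
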(event EventBeginPlay)

(event Collision|EventActorBeginOverlap
  (params (OtherActor :type Actor%20Object%20Reference)))

(event EventTick
  (params (DeltaSeconds :type Float%20%28single-precision%29)))

(event EventOnCharacterEnter
  (params (GameCamera :type Game%20Camera%20Object%20Reference))
  (Utilities|FlowControl|Sequence
    (:then_0
      (if (Variables|Lenght|GetModify%20Lenght)
        (Class|GameCamera|ChangeLenght GameCamera (Variables|Lenght|GetLenght))))
    (:then_1
      (if (Variables|Rotation|GetModify%20Rotation)
        (Class|GameCamera|ChangeRotation GameCamera (Variables|Rotation|GetRotation))))
    (:then_2
      (if (Variables|OffSet|GetModify%20Offset)
        (Class|GameCamera|SetManualOffset GameCamera (Variables|OffSet|GetOffSet) true)))))

(event EventOnCharacterExit
  (params (GameCamera :type Game%20Camera%20Object%20Reference))
  (Utilities|FlowControl|Sequence
    (:then_0
      (if true
        (if (Variables|Lenght|GetReset%20Lenght)
          (Class|GameCamera|SetLenghttoDefault GameCamera))))
    (:then_1
      (if true
        (if (Variables|Rotation|GetReset%20Rotation)
          (Class|GameCamera|SetRotationtoDeafult GameCamera))))
    (:then_2
      (if true
        (if (Variables|OffSet|GetReset%20OffSet)
          (Class|GameCamera|SetManualOffset GameCamera (Variables|OffSet|GetOffSet) false))))))

(fn ConstructionScript)
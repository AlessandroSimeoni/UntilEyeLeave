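; BP_HealingItem_FullHeart is a full-heart healing item Blueprint that adds a two-stage magnetic pickup motion.
; On MagneticPickUp, a timeline lerps it from its current location to the supplied pull-away point.
; A second timeline then lerps it from there toward the Character's live location, so it homes in on a moving target.
; The graph contains only this movement, with no healing or destroy logic.
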(event EventMagneticPickUp
  (params (PullAwayLocation :type Vector :default "0, 0, 0"))
  (Variables|Default|SetCachedLocation (Transformation|GetActorLocation))
  (bind _pullawaytrack (Timeline|PullAwayTimeline PlayFromStart)
    (:Update
      (Transformation|SetActorLocation (Math|Vector|Lerp(Vector) (Variables|Default|GetCachedLocation) PullAwayLocation _pullawaytrack) false false))
    (:Finished
      (Variables|Default|SetCachedLocation (Transformation|GetActorLocation))
      (bind _pushtoplayertrack (Timeline|PushToPlayerTimeline PlayFromStart)
        (:Update
          (Transformation|SetActorLocation (Math|Vector|Lerp(Vector) (Variables|Default|GetCachedLocation) (Transformation|GetActorLocation (Variables|Default|GetCharacter)) _pushtoplayertrack) false false))))))

(fn ConstructionScript)
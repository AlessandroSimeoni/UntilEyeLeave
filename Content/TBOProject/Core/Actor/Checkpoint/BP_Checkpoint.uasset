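; Checkpoint actor that gives save feedback and lets the player sit to open a teleport map.
; Save feedback shows HUD UI, plays a sound, steadies the flickering light and spins the stop sign.
; Interact locks input, hides the HUD, switches to the sitting camera behind a fade and pauses on the map, opened by montage notify.
; Closing the map or teleporting fades back to the game camera, restoring control and HUD.
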(event Custom|TeleportPlayer
  (bind _character (Variables|Default|GetCharacter))
  ;[0.06314 0.3466 1] Teleport handling
  (EventDispatchers|UnbindEventfromOnBlackScreen (Variables|Default|GetFadeWidget) (delegate Custom|TeleportPlayer))
  (Animation|Montage|MontageStop (Components|SkeletalMesh|GetAnimInstance (Variables|/Script/Engine.Character|GetMesh (Variables|Default|GetCharacter))) 0.0 "/Game/TBOProject/Art/MainCharacter/Animation/AM_Sitting.AM_Sitting")
  (Game|Player|SetViewTargetwithBlend (Game|GetPlayerController 0) (Variables|/Game/TBOProject/Core/Gamemodes/Play/GM_Play.GM_Play_C|GetGameCamera (.AsGM%20Play (Utilities|Casting|CastToGM_Play (Game|GetGameMode)))) 0.0 "VTBlend_Cubic" 1.0 false)
  (Transformation|SetActorLocationAndRotation _character (+ (stale Custom|HandleTeleportRequest TeleportLocation) (Math|Vector|MakeVector 0.0 0.0 (Variables|/Script/Engine.CapsuleComponent|GetCapsuleHalfHeight (Variables|/Script/Engine.Character|GetCapsuleComponent (Variables|Default|GetCharacter))))) (Transformation|GetWorldRotation (Variables|Default|GetRespawnLocation)))
  (Default|HandleSittingatCheckpoints (.AsBP%20Main%20Character (Utilities|Casting|CastToBP_MainCharacter _character)) false))

(event Custom|OnFadeOver_Event
  (bind _returnvalue (Game|GetPlayerController 0))
  (bind _asbp_character_controller (Utilities|Casting|CastToBP_CharacterController _returnvalue))
  ;[0.06314 0.3466 1] Teleport handling
  (EventDispatchers|UnbindEventfromOnFadeOver (stale Custom|HandleTeleportRequest _output_get) (delegate Custom|OnFadeOver_Event))
  (Widget|RemovefromParent (stale Custom|HandleTeleportRequest _output_get))
  ;[1 0.2599 0.1602] Remove Fade widget, enable input and player movement & show HUD
  (Class|CharacterController|ToggleInput _asbp_character_controller true)
  (Pawn|Components|CharacterMovement|SetMovementMode (Variables|/Script/Engine.Character|GetCharacterMovement (Variables|Default|GetCharacter)) "MOVE_Walking" 0)
  (Widget|SetVisibility (Variables|/Game/TBOProject/Core/Gamemodes/Play/GM_Play.GM_Play_C|GetHUDWidget (.AsGM%20Play (Utilities|Casting|CastToGM_Play (Game|GetGameMode)))) "Visible")
  (Widget|SetRenderOpacity (Variables|/Game/TBOProject/UI/JournalWidget/W_HUDStack.W_HUDStack_C|GetHudStack (Variables|/Game/TBOProject/Core/Characters/Player/BP_CharacterController.BP_CharacterController_C|GetHud_StackWidget _asbp_character_controller)) 1.0)
  (Variables|SittingInteraction|SetInteracted false)
  (Utilities|FlowControl|Delay (Variables|SittingInteraction|GetCameraBlendTime))
  (if (not (Variables|SittingInteraction|GetInteracted))
    (Components|Activation|Deactivate (Variables|Default|GetSittingCamera))))

(event Custom|ClearFadeWidget
  (bind _fadewidget (Variables|Default|GetFadeWidget))
  ;[1 0.3432 0.3333] Remove first fade widget
  (EventDispatchers|UnbindEventfromOnFadeOver _fadewidget (delegate Custom|ClearFadeWidget))
  (Widget|RemovefromParent _fadewidget))

(event Custom|StartStading
  (bind _targetpositionforstandanimation (Variables|Default|GetTargetPositionForStandAnimation))
  ;[0.241 0.4097 1] Standing montage
  (Animation|Montage|MontageStop (Components|SkeletalMesh|GetAnimInstance (Variables|/Script/Engine.Character|GetMesh (Variables|Default|GetCharacter))) 0.0 "/Game/TBOProject/Art/MainCharacter/Animation/AM_Sitting.AM_Sitting")
  (Transformation|SetActorLocationAndRotation (Variables|Default|GetCharacter) (Transformation|GetWorldLocation _targetpositionforstandanimation) (Transformation|GetWorldRotation _targetpositionforstandanimation))
  (Animation|Montage|PlayMontage (Variables|/Script/Engine.Character|GetMesh (Variables|Default|GetCharacter)) "/Game/TBOProject/Art/MainCharacter/Animation/AM_Stand.AM_Stand" 1.0 0.0 ""
    (:OnNotifyBegin
      ;[1 0.912 0.4225] Second Fade
      (bind _returnvalue (UserInterface|CreateWidget "/Game/TBOProject/UI/Cutscene/W_Fade.W_Fade_C"))
      (bind _output_get (Variables|Default|SetFadeWidget _returnvalue))
      (Variables|/Game/TBOProject/UI/Cutscene/W_Fade.W_Fade_C|SetFadePlayRate _output_get (Variables|SittingInteraction|GetCheckpointInteractionFadePlayRate))
      (Variables|/Game/TBOProject/UI/Cutscene/W_Fade.W_Fade_C|SetStartWithFadeOutIn _output_get true)
      (EventDispatchers|BindEventtoOnBlackScreen _output_get (delegate Custom|ResetCharacter))
      (EventDispatchers|BindEventtoOnFadeOver _output_get (delegate Custom|EndCheckpointInteraction))
      (UserInterface|Viewport|AddtoViewport _output_get 0))))

(event Custom|ResetCharacter
  (bind _respawnlocation (Variables|Default|GetRespawnLocation))
  (bind _character (Variables|Default|GetCharacter))
  ;[0.3012 1 0.107] Reposition character in front of the checkpoint and show weapon/decal
  (EventDispatchers|UnbindEventfromOnBlackScreen (stale Custom|StartStading _output_get) (delegate Custom|ResetCharacter))
  (Game|Player|SetViewTargetwithBlend (Game|GetPlayerController 0) (Variables|/Game/TBOProject/Core/Gamemodes/Play/GM_Play.GM_Play_C|GetGameCamera (.AsGM%20Play (Utilities|Casting|CastToGM_Play (Game|GetGameMode)))) (Variables|SittingInteraction|GetCameraBlendTime) "VTBlend_Linear" 1.0 false)
  (Transformation|SetActorLocationAndRotation _character (+ (Transformation|GetWorldLocation _respawnlocation) (Math|Vector|MakeVector 0.0 0.0 (Variables|/Script/Engine.CapsuleComponent|GetCapsuleHalfHeight (Variables|/Script/Engine.Character|GetCapsuleComponent (Variables|Default|GetCharacter))))) (Transformation|GetWorldRotation _respawnlocation))
  (Default|HandleSittingatCheckpoints (.AsBP%20Main%20Character (Utilities|Casting|CastToBP_MainCharacter _character)) false))

(event Custom|EndCheckpointInteraction
  (bind _returnvalue (Game|GetPlayerController 0))
  (bind _fadewidget (Variables|Default|GetFadeWidget))
  (bind _asbp_character_controller (Utilities|Casting|CastToBP_CharacterController _returnvalue))
  ;[1 0.2599 0.1602] Remove Fade widget, enable input and player movement & show HUD
  (EventDispatchers|UnbindEventfromOnFadeOver _fadewidget (delegate Custom|EndCheckpointInteraction))
  (Widget|RemovefromParent _fadewidget)
  (Class|CharacterController|ToggleInput _asbp_character_controller true)
  (Pawn|Components|CharacterMovement|SetMovementMode (Variables|/Script/Engine.Character|GetCharacterMovement (Variables|Default|GetCharacter)) "MOVE_Walking" 0)
  (Widget|SetVisibility (Variables|/Game/TBOProject/Core/Gamemodes/Play/GM_Play.GM_Play_C|GetHUDWidget (.AsGM%20Play (Utilities|Casting|CastToGM_Play (Game|GetGameMode)))) "Visible")
  (Widget|SetRenderOpacity (Variables|/Game/TBOProject/UI/JournalWidget/W_HUDStack.W_HUDStack_C|GetHudStack (Variables|/Game/TBOProject/Core/Characters/Player/BP_CharacterController.BP_CharacterController_C|GetHud_StackWidget _asbp_character_controller)) 1.0)
  (Variables|SittingInteraction|SetInteracted false)
  (Utilities|FlowControl|Delay (Variables|SittingInteraction|GetCameraBlendTime))
  (if (not (Variables|SittingInteraction|GetInteracted))
    (Components|Activation|Deactivate (Variables|Default|GetSittingCamera))))

(event Custom|FakeSaveFeedback
  ;[1 0.2469 0.2469] FAKE SAVE UI FEEDBACK
  (bind _asgm_play (Utilities|Casting|CastToGM_Play (Game|GetGameMode)))
  (Default|SaveUIFeedback (Variables|/Game/TBOProject/Core/Gamemodes/Play/GM_Play.GM_Play_C|GetHUDWidget _asgm_play))
  ;[1 1 1] play sound
  (Audio|PlaySound2D "/Game/TBOProject/Media/Sound/Events/SFX_CheckpointSave.SFX_CheckpointSave" 0.05 1.0 0.0 0 0)
  ;[1 1 1] Stop light flickering
  (Rendering|Components|Light|SetLightFunctionMaterial (Variables|Default|GetBottom_RectLight) 0)
  (Utilities|FlowControl|DoOnce false
    (:Completed
      (bind _intensity (Timeline|LightIntensity PlayFromStart)
        (:Update
          (Rendering|Components|Light|SetIntensity (Variables|Default|GetBottom_RectLight) _intensity))))))

(event Custom|PositionCharacterAndCamera
  (bind _returnvalue (Game|GetPlayerController 0))
  (bind _targetpositionforsitanimation (Variables|Default|GetTargetPositionForSitAnimation))
  (bind _character (Variables|Default|GetCharacter))
  ;[0.4942 0.487 1] Sit Montage & hide player's weapon/decal
  (EventDispatchers|UnbindEventfromOnBlackScreen (stale EventInteract _output_get) (delegate Custom|PositionCharacterAndCamera))
  (Components|Activation|Activate (Variables|Default|GetSittingCamera) false)
  (Game|Player|SetViewTargetwithBlend (Game|GetPlayerController 0) self (Variables|SittingInteraction|GetCameraBlendTime) "VTBlend_Cubic" 1.0 false)
  (Transformation|SetActorLocationAndRotation _character (Transformation|GetWorldLocation _targetpositionforsitanimation) (Transformation|GetWorldRotation _targetpositionforsitanimation))
  (Default|HandleSittingatCheckpoints (.AsBP%20Main%20Character (Utilities|Casting|CastToBP_MainCharacter _character)) true)
  (Animation|Montage|PlayMontage (Variables|/Script/Engine.Character|GetMesh _character) "/Game/TBOProject/Art/MainCharacter/Animation/AM_Sitting.AM_Sitting" 1.0 0.0 ""
    (:OnNotifyBegin
      ;[0.4791 0.9901 1] OpenMap
      (bind _asbp_character_controller (Utilities|Casting|CastToBP_CharacterController (Game|GetPlayerController 0)))
      (Variables|/Script/TBO_01.CharacterController|SetCanTeleport _asbp_character_controller true)
      (bind _returnvalue_2 (Class|CommonActivatableWidgetContainerBase|AddWidget (Variables|/Game/TBOProject/UI/JournalWidget/W_HUDStack.W_HUDStack_C|GetMenuStack (Variables|/Game/TBOProject/Core/Characters/Player/BP_CharacterController.BP_CharacterController_C|GetHud_StackWidget _asbp_character_controller)) "/Game/TBOProject/UI/JournalWidget/MapWidget/W_CheckpointMap.W_CheckpointMap_C"))
      (EventDispatchers|UnbindEventfromBPonWidgetDeactivated _returnvalue_2 (delegate Custom|StartStading))
      (EventDispatchers|BindEventtoBPonWidgetDeactivated _returnvalue_2 (delegate Custom|StartStading))
      (EventDispatchers|BindEventtoTeleportRequested _returnvalue_2 (delegate Custom|HandleTeleportRequest))
      (Game|SetGamePaused true)
      (Variables|/Script/Engine.PlayerController|SetbShowMouseCursor _returnvalue true)
      (Input|SetInputModeUIOnly _returnvalue _returnvalue_2 "DoNotLock" false))))

(event Custom|HandleTeleportRequest
  (params (TeleportLocation :type Vector))
  ;[0.06314 0.3466 1] Teleport handling
  (EventDispatchers|UnbindEventfromTeleportRequested (stale Custom|PositionCharacterAndCamera _returnvalue_2) (delegate Custom|HandleTeleportRequest))
  (EventDispatchers|UnbindEventfromBPonWidgetDeactivated (stale Custom|PositionCharacterAndCamera _returnvalue_2) (delegate Custom|StartStading))
  (Class|AnimInstance|MontagePause (Components|SkeletalMesh|GetAnimInstance (Variables|/Script/Engine.Character|GetMesh (Variables|Default|GetCharacter))) "/Game/TBOProject/Art/MainCharacter/Animation/AM_Sitting.AM_Sitting")
  (bind _returnvalue (UserInterface|CreateWidget "/Game/TBOProject/UI/Cutscene/W_Fade.W_Fade_C"))
  (bind _output_get (Variables|Default|SetFadeWidget _returnvalue))
  (Variables|/Game/TBOProject/UI/Cutscene/W_Fade.W_Fade_C|SetFadePlayRate _output_get 1.0)
  (Variables|/Game/TBOProject/UI/Cutscene/W_Fade.W_Fade_C|SetStartWithFadeOutIn _output_get true)
  (EventDispatchers|BindEventtoOnBlackScreen _output_get (delegate Custom|TeleportPlayer))
  (EventDispatchers|AssignOnFadeOver _output_get (delegate Custom|OnFadeOver_Event))
  (UserInterface|Viewport|AddtoViewport _output_get 0))

(event EventBeginPlay
  ;[1 1 1] Set light material (flickering) at begin play
  (Rendering|Components|Light|SetIntensity (Variables|Default|GetBottom_RectLight) 5e+02)
  (Rendering|Components|Light|SetLightFunctionMaterial (Variables|Default|GetBottom_RectLight) "/Game/TBOProject/Art/Enviroment/Materials/M_LightFlickering.M_LightFlickering")
  (Utilities|FlowControl|Delay 0.5)
  (Variables|/Script/Engine.PrimitiveComponent|SetbGenerateOverlapEvents (Variables|Default|GetSaveArea) true))

(event EventInteract
  (bind _returnvalue (Game|GetPlayerController 0))
  (bind _character (Variables|Default|GetCharacter))
  (bind _asbp_character_controller (Utilities|Casting|CastToBP_CharacterController _returnvalue))
  (bind _charactermovement (Variables|/Script/Engine.Character|GetCharacterMovement _character))
  ;[0.2901 0.8291 1] Disable input, stop player and hide HUD
  (Utilities|IsValid _character
    (:Is%20Valid
      (Variables|SittingInteraction|SetInteracted true)
      (Class|CharacterController|ToggleInput _asbp_character_controller false)
      (Pawn|Components|CharacterMovement|SetMovementMode _charactermovement "MOVE_None" 0)
      (Components|Movement|StopMovementImmediately _charactermovement)
      (Widget|SetRenderOpacity (Variables|/Game/TBOProject/UI/JournalWidget/W_HUDStack.W_HUDStack_C|GetHudStack (Variables|/Game/TBOProject/Core/Characters/Player/BP_CharacterController.BP_CharacterController_C|GetHud_StackWidget _asbp_character_controller)) 0.0)
      (Widget|SetVisibility (Variables|/Game/TBOProject/Core/Gamemodes/Play/GM_Play.GM_Play_C|GetHUDWidget (.AsGM%20Play (Utilities|Casting|CastToGM_Play (Game|GetGameMode)))) "Hidden")
      ;[1 0.7872 0.5462] First Fade
      (bind _returnvalue_2 (UserInterface|CreateWidget "/Game/TBOProject/UI/Cutscene/W_Fade.W_Fade_C"))
      (bind _output_get (Variables|Default|SetFadeWidget _returnvalue_2))
      (Variables|/Game/TBOProject/UI/Cutscene/W_Fade.W_Fade_C|SetFadePlayRate _output_get (Variables|SittingInteraction|GetCheckpointInteractionFadePlayRate))
      (Variables|/Game/TBOProject/UI/Cutscene/W_Fade.W_Fade_C|SetStartWithFadeOutIn _output_get true)
      (UserInterface|Viewport|AddtoViewport _output_get 0)
      (EventDispatchers|BindEventtoOnBlackScreen _output_get (delegate Custom|PositionCharacterAndCamera))
      (EventDispatchers|BindEventtoOnFadeOver _output_get (delegate Custom|ClearFadeWidget)))))

(event EventAnimateStopSign
  ;[1 0.04459 0] placeholder
  (CallFunction|FakeSaveFeedback)
  (bind _output_get (Variables|Default|SetInitialSignYaw (.yaw (Variables|/Script/Engine.SceneComponent|GetRelativeRotation (Variables|Default|GetStopSignMesh)))))
  (Variables|Default|SetTargetSignYaw (+ _output_get 3.6e+02))
  (bind _newtrack_0 (Timeline|Timeline PlayFromStart)
    (:Update
      (Transformation|SetRelativeRotation (Variables|Default|GetStopSignMesh) (Math|Rotator|MakeRotator 0.0 0.0 (Math|Float|Lerp (Variables|Default|GetInitialSignYaw) (Variables|Default|GetTargetSignYaw) _newtrack_0)) false false))))

(fn ConstructionScript)
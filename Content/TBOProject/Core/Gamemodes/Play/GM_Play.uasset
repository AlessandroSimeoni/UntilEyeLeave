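; Play game mode that sets up a gameplay session and drives the intro and final story cutscenes.
; BeginPlay attaches the game camera, creates the HUD, moves the player to the saved checkpoint and applies saved volumes through a sound mix.
; A new game from the main menu disables input and preloads the intro cutscene, played when its intro widget signals.
; The ending makes the player immortal, then a fade widget's callback requests the last two cutscenes.
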(event Custom|WaitFadeAndPlayFinalCuscenes
  (params (FadeWidget :type W%20Fade%20Object%20Reference))
  ;[0.5395 1 0.7111] FinalCutscene
  (EventDispatchers|BindEventtoOnFadeOver FadeWidget (delegate Custom|PlayFinalCutscenes)))

(event Custom|StartCutscene
  (bind _returnvalue (Subsystems|GetCutsceneSubsystem))
  ;[1 0.7508 0.1156] InitialCutscene
  (EventDispatchers|UnbindEventfromCutsceneCanStart (stale EventBeginPlay _newgameintrowidget) (delegate Custom|StartCutscene))
  (Variables|/Script/TBO_01.CutsceneSubsystem|SetTransitionWidget _returnvalue (stale EventBeginPlay _newgameintrowidget))
  (Class|CutsceneSubsystem|PlayCutscene _returnvalue "/Game/TBOProject/Maps/Level/Blockout/Sub_Level2/Cutscene_1.Cutscene_1" "/Game/Cutscenes/Cutscene1.Cutscene1"))

(event Custom|PlayFinalCutscenes
  (bind _returnvalue (Subsystems|GetCutsceneSubsystem))
  ;[0.5395 1 0.7111] FinalCutscene
  (EventDispatchers|UnbindEventfromOnFadeOver (stale Custom|WaitFadeAndPlayFinalCuscenes FadeWidget) (delegate Custom|PlayFinalCutscenes))
  (Variables|/Script/TBO_01.CutsceneSubsystem|SetTransitionWidget _returnvalue (stale Custom|WaitFadeAndPlayFinalCuscenes FadeWidget))
  (Class|CutsceneSubsystem|PlayCutscene _returnvalue "/Game/TBOProject/Maps/Level/Blockout/Sub_Level2/Cutscene_2.Cutscene_2" "/Game/Cutscenes/Cutscene2.Cutscene2")
  (Class|CutsceneSubsystem|PlayCutscene _returnvalue "/Game/TBOProject/Maps/Level/Blockout/Sub_Level2/Cutscene_3.Cutscene_3" "/Game/Cutscenes/Cutscene3.Cutscene3"))

(event EventBeginPlay
  (bind _returnvalue (Game|GetPlayerCharacter 0))
  (bind _returnvalue_2 (Game|GetPlayerController 0))
  (bind _returnvalue_3 (Subsystems|GetCutsceneSubsystem))
  (Utilities|FlowControl|Sequence
    (:then_0
      (bind _returnvalue_4 (Actor|GetActorOfClass "/Game/TBOProject/Core/Camera/BP_GameCamera.BP_GameCamera_C"))
      (bind _output_get (Variables|Default|SetGameCamera _returnvalue_4))
      (Class|GameCamera|Attach _output_get _returnvalue true)
      (bind _returnvalue_5 (UserInterface|CreateWidget "/Game/TBOProject/UI/HUD/W_HUD.W_HUD_C"))
      (Variables|Default|SetHUDWidget _returnvalue_5)
      (bind _asmain_character (Utilities|Casting|CastToMainCharacter _returnvalue))
      (Variables|/Script/TBO_01.HUDWidget|SetMainCharacter _returnvalue_5 _asmain_character)
      (UserInterface|Viewport|AddtoViewport _returnvalue_5 0)
      (Input|SetInputModeGameOnly _returnvalue_2 false)
      (Variables|/Script/Engine.PlayerController|SetbShowMouseCursor _returnvalue_2 false))
    (:then_1
      (CallFunction|TeleportPlayertoLastCheckpoint _returnvalue))
    (:then_2
      (if (and (not (Class|SaveSubsystem|DoesSaveExist (Subsystems|GetSaveSubsystem) "PlayerSaveSlot")) (Variables|/Script/TBO_01.CutsceneSubsystem|GetComingFromMainMenu _returnvalue_3))
        ;[1 0.7508 0.1156] InitialCutscene
        (Class|CharacterController|ToggleInput (.AsBP%20Character%20Controller (Utilities|Casting|CastToBP_CharacterController (Game|GetPlayerController 0))) false)
        (Variables|/Script/TBO_01.CutsceneSubsystem|SetComingFromMainMenu _returnvalue_3 false)
        (Class|CutsceneSubsystem|PreLoadCutscene _returnvalue_3 "/Game/TBOProject/Maps/Level/Blockout/Sub_Level2/Cutscene_1.Cutscene_1" "/Game/Cutscenes/Cutscene1.Cutscene1")
        (Utilities|FlowControl|DelayUntilNextTick)
        (bind _newgameintrowidget (CallFunction|ShowNewGameIntroWidget))
        (EventDispatchers|BindEventtoCutsceneCanStart _newgameintrowidget (delegate Custom|StartCutscene))))
    (:then_3
      ;[1 0.5284 0.9958] AUDIO
      (Audio|PushSoundMixModifier "/Game/TBOProject/Media/Sound/MetasoundSystems/SCM_MasterSoundMix.SCM_MasterSoundMix")
      (bind _returnvalue_6 (Class|SaveSubsystem|LoadSettings (Subsystems|GetSaveSubsystem)))
      (Audio|SetSoundMixClassOverride "/Game/TBOProject/Media/Sound/MetasoundSystems/SCM_MasterSoundMix.SCM_MasterSoundMix" "/Game/TBOProject/Media/Sound/MetasoundSystems/SC_MasterSound.SC_MasterSound" (Variables|/Script/TBO_01.TBOSaveSettings|GetMasterVolume _returnvalue_6) 1.0 0.0 true)
      (Audio|SetSoundMixClassOverride "/Game/TBOProject/Media/Sound/MetasoundSystems/SCM_MasterSoundMix.SCM_MasterSoundMix" "/Game/TBOProject/Media/Sound/MetasoundSystems/SC_MasterMusic.SC_MasterMusic" (Variables|/Script/TBO_01.TBOSaveSettings|GetMusicVolume _returnvalue_6) 1.0 0.0 true)
      (Audio|SetSoundMixClassOverride "/Game/TBOProject/Media/Sound/MetasoundSystems/SCM_MasterSoundMix.SCM_MasterSoundMix" "/Game/TBOProject/Media/Sound/MetasoundSystems/SC_MasterSFX.SC_MasterSFX" (Variables|/Script/TBO_01.TBOSaveSettings|GetEffectsVolume _returnvalue_6) 1.0 0.0 true)
      (Audio|SetSoundMixClassOverride "/Game/TBOProject/Media/Sound/MetasoundSystems/SCM_MasterSoundMix.SCM_MasterSoundMix" "/Game/TBOProject/Media/Sound/MetasoundSystems/SC_MasterInterface.SC_MasterInterface" (Variables|/Script/TBO_01.TBOSaveSettings|GetInterfaceVolume _returnvalue_6) 1.0 0.0 true))))

(fn ConstructionScript)

(fn TeleportPlayertoLastCheckpoint
  (params (PlayerCharacter :type Character%20Object%20Reference))
  (bind _returnvalue (Class|SaveSubsystem|LoadGame (Subsystems|GetSaveSubsystem)))
  (if (Utilities|Operators|NotEqual(!=) :A (Variables|/Script/TBO_01.TBOSaveGame|GetLastCheckpointLocation _returnvalue))
    (Transformation|SetActorLocation PlayerCharacter (+ (Variables|/Script/TBO_01.TBOSaveGame|GetLastCheckpointLocation _returnvalue) (Math|Vector|MakeVector 0.0 0.0 (Variables|/Script/Engine.CapsuleComponent|GetCapsuleHalfHeight (Variables|/Script/Engine.Character|GetCapsuleComponent PlayerCharacter)))) false false)))

(fn ShowNewGameIntroWidget
  (CallFunction|HideHUD)
  (bind _returnvalue (UserInterface|CreateWidget "/Game/TBOProject/Design_Blueprint/Blueprints/UI_Placeholder/WB_NewGameIntro.WB_NewGameIntro_C"))
  (UserInterface|Viewport|AddtoViewport _returnvalue 0)
  (return _returnvalue))

(fn StartFinalCutsceneSequence
  (Variables|/Script/TBO_01.LifeSystemComponent|SetImmortal (Variables|/Script/TBO_01.MainCharacter|GetLifeComponent (.AsMain%20Character (Utilities|Casting|CastToMainCharacter (Game|GetPlayerCharacter 0)))) true)
  (Class|CutsceneSubsystem|PreLoadCutscene (Subsystems|GetCutsceneSubsystem) "/Game/TBOProject/Maps/Level/Blockout/Sub_Level2/Cutscene_2.Cutscene_2" "/Game/Cutscenes/Cutscene2.Cutscene2")
  (Class|CharacterController|ToggleInput (.AsBP%20Character%20Controller (Utilities|Casting|CastToBP_CharacterController (Game|GetPlayerController 0))) false)
  (CallFunction|HideHUD)
  (bind _returnvalue (UserInterface|CreateWidget "/Game/TBOProject/UI/Cutscene/W_Fade.W_Fade_C"))
  (Variables|/Game/TBOProject/UI/Cutscene/W_Fade.W_Fade_C|SetStartWithFadeIn _returnvalue false)
  (UserInterface|Viewport|AddtoViewport _returnvalue 0)
  (CallFunction|WaitFadeandPlayFinalCuscenes _returnvalue))

(fn HideHUD
  (Widget|SetRenderOpacity (Variables|/Game/TBOProject/Core/Characters/Player/BP_CharacterController.BP_CharacterController_C|GetHud_StackWidget (.AsBP%20Character%20Controller (Utilities|Casting|CastToBP_CharacterController (Game|GetPlayerController 0)))) 0.0)
  (Widget|SetVisibility (Variables|Default|GetHUDWidget) "Hidden"))
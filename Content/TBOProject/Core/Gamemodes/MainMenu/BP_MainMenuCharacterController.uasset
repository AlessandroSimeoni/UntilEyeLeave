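; Main menu controller that runs the opening screen and camera moves between menu views.
; On BeginPlay it gets the game mode's camera aggregator and shows an opening widget in a widget stack.
; Any key clears the stack and lerps to one of two cameras, depending on whether a player save exists.
; A one-time lerp-complete check adds the main menu widget if the camera reached is the initial one, then serves that widget's lerp requests.
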(event Custom|AnyKeyPressedEvent_Event
  (if (Class|SaveSubsystem|DoesSaveExist (Subsystems|GetSaveSubsystem) "PlayerSaveSlot")
    (Class|MainMenuController|LerpCamera (Class|MainMenuCameraAggregator|GetCameraActoratIndex (Variables|Default|GetCameraAggregator) 1) (Variables|Default|GetFirstLerpTime))
    (else
      (Class|MainMenuController|LerpCamera (Class|MainMenuCameraAggregator|GetCameraActoratIndex (Variables|Default|GetCameraAggregator) 2) (Variables|Default|GetFirstLerpTime))))
  (Class|CommonActivatableWidgetContainerBase|ClearWidgets (Variables|/Game/TBOProject/UI/Main_Menu/W_MainMenuStack.W_MainMenuStack_C|GetMainMenuStack (Variables|Default|GetMainMenuStack))))

(event Custom|OnLerpRequest_Event
  (params (Camera :type Camera%20Actor%20Object%20Reference))
  (Class|MainMenuController|LerpCamera Camera (Variables|Default|GetCameraLerpTime)))

(event EventBeginPlay
  (Variables|Default|SetCameraAggregator (Variables|/Game/TBOProject/Core/Gamemodes/MainMenu/GM_MainMenuDef.GM_MainMenuDef_C|GetCameraAggregator (.AsGM%20Main%20Menu%20Def (Utilities|Casting|CastToGM_MainMenuDef (Game|GetGameMode)))))
  (Variables|Default|SetInitialCamera (Class|MainMenuCameraAggregator|GetCameraActoratIndex (Variables|Default|GetCameraAggregator)))
  (bind _returnvalue (UserInterface|CreateWidget "/Game/TBOProject/UI/Main_Menu/W_MainMenuStack.W_MainMenuStack_C"))
  (bind _output_get (Variables|Default|SetMainMenuStack _returnvalue))
  (UserInterface|Viewport|AddtoViewport _output_get 0)
  (bind _returnvalue_2 (Class|CommonActivatableWidgetContainerBase|AddWidget (Variables|/Game/TBOProject/UI/Main_Menu/W_MainMenuStack.W_MainMenuStack_C|GetMainMenuStack (Variables|Default|GetMainMenuStack)) "/Game/TBOProject/UI/Main_Menu/W_MainMenuOpeningWidget.W_MainMenuOpeningWidget_C"))
  (EventDispatchers|AssignAnyKeyPressedEvent _returnvalue_2 (delegate Custom|AnyKeyPressedEvent_Event))
  (Variables|Default|SetbShowMouseCursor true))

(event EventLerpCameraComplete
  (params (Camera :type Camera%20Actor%20Object%20Reference))
  (Utilities|FlowControl|DoOnce false
    (:Completed
      (if (== (Variables|Default|GetInitialCamera) Camera)
        (bind _returnvalue (Class|CommonActivatableWidgetContainerBase|AddWidget (Variables|/Game/TBOProject/UI/Main_Menu/W_MainMenuStack.W_MainMenuStack_C|GetMainMenuStack (Variables|Default|GetMainMenuStack)) "/Game/TBOProject/UI/Main_Menu/W_MainMenuWidget.W_MainMenuWidget_C"))
        (EventDispatchers|AssignOnLerpRequest _returnvalue (delegate Custom|OnLerpRequest_Event))))))

(fn ConstructionScript)
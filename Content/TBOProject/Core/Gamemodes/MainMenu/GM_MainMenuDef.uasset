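; Main menu game mode that prepares the menu level's camera reference and audio mix when play begins.
; On BeginPlay it finds and stores the BP_MainMenuCameraAggregator in the level.
; It then pushes the master sound mix and overrides the master, music, SFX and interface sound class volumes with values loaded through the save subsystem, with no fade.
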(event EventBeginPlay
  (bind _returnvalue (Actor|GetActorOfClass "/Game/TBOProject/UI/Main_Menu/BP_MainMenuCameraAggregator.BP_MainMenuCameraAggregator_C"))
  (Variables|Default|SetCameraAggregator _returnvalue)
  ;[0.976 0.5807 1] AUDIO
  (Audio|PushSoundMixModifier "/Game/TBOProject/Media/Sound/MetasoundSystems/SCM_MasterSoundMix.SCM_MasterSoundMix")
  (bind _returnvalue_2 (Class|SaveSubsystem|LoadSettings (Subsystems|GetSaveSubsystem)))
  (Audio|SetSoundMixClassOverride "/Game/TBOProject/Media/Sound/MetasoundSystems/SCM_MasterSoundMix.SCM_MasterSoundMix" "/Game/TBOProject/Media/Sound/MetasoundSystems/SC_MasterSound.SC_MasterSound" (Variables|/Script/TBO_01.TBOSaveSettings|GetMasterVolume _returnvalue_2) 1.0 0.0 true)
  (Audio|SetSoundMixClassOverride "/Game/TBOProject/Media/Sound/MetasoundSystems/SCM_MasterSoundMix.SCM_MasterSoundMix" "/Game/TBOProject/Media/Sound/MetasoundSystems/SC_MasterMusic.SC_MasterMusic" (Variables|/Script/TBO_01.TBOSaveSettings|GetMusicVolume _returnvalue_2) 1.0 0.0 true)
  (Audio|SetSoundMixClassOverride "/Game/TBOProject/Media/Sound/MetasoundSystems/SCM_MasterSoundMix.SCM_MasterSoundMix" "/Game/TBOProject/Media/Sound/MetasoundSystems/SC_MasterSFX.SC_MasterSFX" (Variables|/Script/TBO_01.TBOSaveSettings|GetEffectsVolume _returnvalue_2) 1.0 0.0 true)
  (Audio|SetSoundMixClassOverride "/Game/TBOProject/Media/Sound/MetasoundSystems/SCM_MasterSoundMix.SCM_MasterSoundMix" "/Game/TBOProject/Media/Sound/MetasoundSystems/SC_MasterInterface.SC_MasterInterface" (Variables|/Script/TBO_01.TBOSaveSettings|GetInterfaceVolume _returnvalue_2) 1.0 0.0 true))

(fn ConstructionScript)
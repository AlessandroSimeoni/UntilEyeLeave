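; Environment placement actor that duplicates a chosen mesh along a spline.
; The construction script fills a hierarchical instanced static mesh component, stepping along the spline by mesh X extent plus spacing.
; Each instance gets a seeded random transform from FRandomTransform, controlling position, rotation, axis flips and Z offset.
; SplineAlign optionally feeds spline rotation into that transform, and the event graph has no active logic.
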(event EventBeginPlay)

(event Collision|EventActorBeginOverlap
  (params (OtherActor :type Actor%20Object%20Reference)))

(event EventTick
  (params (DeltaSeconds :type Float%20%28single-precision%29)))

(fn ConstructionScript
  (bind _mesh (Variables|Default|GetMesh))
  (bind _spacing (Variables|Default|GetSpacing))
  (bind _random_z_offset_min_max (Variables|Default|GetRandom%20Z%20Offset%20Min%20Max))
  (bind _randomposition (Variables|Default|GetRandomPosition))
  (bind _spline (Variables|Default|GetSpline))
  (bind _randomrotation (Variables|Default|GetRandomRotation))
  (bind _random_flip_axes (Variables|Default|GetRandom%20Flip%20Axes))
  (bind _returnvalue (StaticMesh|GetBoundingBox _mesh))
  (bind _max (Utilities|Struct|BreakBox _returnvalue))
  (bind _x (Math|Vector|BreakVector _max))
  (bind _returnvalue_2 (* _x 2.0))
  (bind _returnvalue_3 (+ _returnvalue_2 _spacing))
  (bind _returnvalue_4 (AddComponent|AddHierarchicalInstancedStaticMeshComponent false))
  (Components|StaticMesh|SetStaticMesh _returnvalue_4 (Variables|Default|GetMesh))
  (Variables|Default|SetNextDistance _returnvalue_3)
  (for _index (range 0 (Math|Float|Floor (/ (Spline|GetSplineLength (Variables|Default|GetSpline)) _returnvalue_3)))
    (if (Variables|Default|GetSpline%20Align)
      (bind _t (CallFunction|FRandomTransform (+ _index (Variables|Default|GetSeed)) (Math|Transform|InverseTransformLocation (Transformation|GetActorTransform) (Spline|GetLocationatDistanceAlongSpline _spline (* _index (Variables|Default|GetNextDistance)) "World")) (Spline|GetRotationatDistanceAlongSpline _spline (* _index (Variables|Default|GetNextDistance)) "Local") _randomposition _randomrotation _random_flip_axes _random_z_offset_min_max))
      (Components|InstancedStaticMesh|AddInstance _returnvalue_4 _t false)
      (else
        (bind _t_2 (CallFunction|FRandomTransform (+ _index (Variables|Default|GetSeed)) (Math|Transform|InverseTransformLocation (Transformation|GetActorTransform) (Spline|GetLocationatDistanceAlongSpline _spline (* _index (Variables|Default|GetNextDistance)) "World")) "0, 0, 0" _randomposition _randomrotation _random_flip_axes _random_z_offset_min_max))
        (Components|InstancedStaticMesh|AddInstance _returnvalue_4 _t_2 false)))))
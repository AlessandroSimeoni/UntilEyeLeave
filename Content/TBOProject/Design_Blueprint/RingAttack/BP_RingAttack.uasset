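; BP_RingAttack is an expanding ring attack actor that damages the player on contact.
; On BeginPlay, a timeline, using ExpansionTime as its play rate, scales the Niagara system horizontally from zero to AttackRange at fixed height.
; The actor destroys itself shortly after the timeline finishes.
; Ring component overlaps with the player character apply fixed damage through BP_MainCharacter's LifeComponent.
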(event OnComponentBeginOverlap(Ring)
  (params (OverlappedComponent :type Primitive%20Component%20Object%20Reference) (OtherActor :type Actor%20Object%20Reference) (OtherComp :type Primitive%20Component%20Object%20Reference) (OtherBodyIndex :type Integer) (bFromSweep :type Boolean) (SweepResult :type Hit%20Result%20Structure%20%28by%20ref%29))
  (bind _returnvalue (Game|GetPlayerCharacter 0))
  (if (== OtherActor _returnvalue)
    (bind _asbp_main_character (Utilities|Casting|CastToBP_MainCharacter _returnvalue))
    (Class|LifeSystemComponent|ReceiveDamage (Variables|/Script/TBO_01.MainCharacter|GetLifeComponent _asbp_main_character) 0.5)))

(event EventBeginPlay
  (Components|Timeline|SetPlayRate (Variables|Default|GetTL_RingExpansion) (Variables|Default|GetExpansion%20Time))
  (bind _newtrack_0 (Timeline|TL_RingExpansion PlayFromStart)
    (:Update
      (Transformation|SetWorldScale3D (Variables|Default|GetNewNiagaraSystem) (Math|Vector|MakeVector (Math|Float|Lerp 0.0 (Variables|Default|GetAttack%20Range) _newtrack_0) (Math|Float|Lerp 0.0 (Variables|Default|GetAttack%20Range) _newtrack_0) 2.0)))
    (:Finished
      (Utilities|FlowControl|Delay 0.2)
      (Actor|DestroyActor))))

(event Collision|EventActorBeginOverlap
  (params (OtherActor :type Actor%20Object%20Reference)))

(event EventTick
  (params (DeltaSeconds :type Float%20%28single-precision%29)))

(fn ConstructionScript)
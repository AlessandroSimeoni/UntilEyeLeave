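; Main menu randomizer actor that varies the creatures and actor groups shown each time play begins.
; Spawns one of three main-menu creature variants (Stealer, MouseTrap or Birdman Shooter) at its own transform and assigns its patrol path to that creature's patrol spline component.
; Separately hides all actors in three groups, then unhides valid actors through a random group selection that is independent of the spawned creature.
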(event Custom|SpawnerRadomCreature
  (bind _returnvalue (Game|SpawnActorfromClass (Utilities|Select :Index (Math|Random|RandomIntegerinRange 0 2) :Option%200 "/Game/TBOProject/Design_Blueprint/CreaturesIA/B06_Stealer/BP_B06_Stealer_MainMenu.BP_B06_Stealer_MainMenu_C" :Option%201 "/Game/TBOProject/Design_Blueprint/CreaturesIA/B02/B02_Variants/BP_B02_MouseTrap_Creature_ChildMainMenu.BP_B02_MouseTrap_Creature_ChildMainMenu_C" :Option%202 "/Game/TBOProject/Design_Blueprint/CreaturesIA/B03/B03_Variants/BP_B03_Birdman_ShooterCreatureBase_ChildMainMenu.BP_B03_Birdman_ShooterCreatureBase_ChildMainMenu_C") (Transformation|GetActorTransform) "AdjustIfPossibleButAlwaysSpawn" "MultiplyWithRoot" 0 0))
  (bind _returnvalue_2 (Class|PatrolInterface|GetPatrolSplineComponent(Message) _returnvalue))
  (Variables|/Script/TBO_01.PatrolSplineComponent|SetAssignedPatrolPath _returnvalue_2 (Variables|Default|GetAssigned%20Patrol%20Path)))

(event Custom|ChangeCreature%20Group
  (for _array_element (Utilities|Select :Index (Math|Random|RandomIntegerinRange 0 2) :Option%200 (Variables|Default|GetGroup1) :Option%201 (Variables|Default|GetGroup2) :Option%202 (Variables|Default|GetGroup3))
    (if (Utilities|IsValid _array_element)
      (Rendering|SetActorHiddenInGame _array_element false))))

(event Custom|SetRandomCreatureGroup
  (for _array_element (Variables|Default|GetGroup1)
    (if (Utilities|IsValid _array_element)
      (Rendering|SetActorHiddenInGame _array_element true)))
  (for _array_element_2 (Variables|Default|GetGroup2)
    (if (Utilities|IsValid _array_element_2)
      (Rendering|SetActorHiddenInGame _array_element_2 true)))
  (for _array_element_3 (Variables|Default|GetGroup3)
    (if (Utilities|IsValid _array_element_3)
      (Rendering|SetActorHiddenInGame _array_element_3 true)))
  (CallFunction|CHangeCreatureGroup))

(event EventBeginPlay
  (CallFunction|SpawnerRadomCreature)
  (CallFunction|SetRandomCreatureGroup))

(fn ConstructionScript)
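; Placeholder camera trigger volume, named for removal, that applies rotation, arm length or distance-to-target modifiers to BP_GameCamera while the player character overlaps it.
; On BeginPlay it finds the camera and, unless Editable, loads its settings from a data asset.
; Length disables the distance modifier.
; Begin overlap adds each enabled modifier and stores its handle; end overlap reverts them non-immediately.
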(event OnComponentBeginOverlap(CollisionComponent)
  (params (OverlappedComponent :type Primitive%20Component%20Object%20Reference) (OtherActor :type Actor%20Object%20Reference) (OtherComp :type Primitive%20Component%20Object%20Reference) (OtherBodyIndex :type Integer) (bFromSweep :type Boolean) (SweepResult :type Hit%20Result%20Structure%20%28by%20ref%29))
  (if (== OtherActor (Game|GetPlayerCharacter 0))
    (if (Variables|Modifier1|GetRotation)
      (bind _returnvalue (Class|GameCamera|AddRotationModifier (Variables|Default|GetCamera) (Variables|Modifier1|GetDelta%20Yaw) (Variables|Modifier1|GetDelta%20Pitch) (Variables|Modifier1|GetDelta%20Roll) (Variables|Modifier1|GetDuration)))
      (Variables|Default|SetRotation_Mod _returnvalue))
    (if (Variables|Modifier2|GetLenght)
      (bind _returnvalue_2 (Class|GameCamera|AddLenghtModifier (Variables|Default|GetCamera) (Variables|Modifier2|GetDelta%20Lenght) (Variables|Modifier2|GetDuration_0)))
      (Variables|Default|SetLenght_Mod _returnvalue_2))
    (if (Variables|Modifier3|GetDistance)
      (bind _returnvalue_3 (Class|GameCamera|AddDistancetoTargetModifier (Variables|Default|GetCamera) (Variables|Modifier3|GetTarget%20Actor) (Variables|Modifier3|GetCurve) 0.0))
      (Variables|Default|SetDinstance_Mod _returnvalue_3))))

(event OnComponentEndOverlap(CollisionComponent)
  (params (OverlappedComponent :type Primitive%20Component%20Object%20Reference) (OtherActor :type Actor%20Object%20Reference) (OtherComp :type Primitive%20Component%20Object%20Reference) (OtherBodyIndex :type Integer))
  (if (== OtherActor (Game|GetPlayerCharacter 0))
    (if (Variables|Modifier1|GetRotation)
      (Class|GameCamera|RevertModifier (Variables|Default|GetCamera) (Variables|Default|GetRotation_Mod) false))
    (if (Variables|Modifier2|GetLenght)
      (Class|GameCamera|RevertModifier (Variables|Default|GetCamera) (Variables|Default|GetLenght_Mod) false))
    (if (Variables|Modifier3|GetDistance)
      (Class|GameCamera|RevertModifier (Variables|Default|GetCamera) (Variables|Default|GetDinstance_Mod) false))))

(event EventBeginPlay
  (bind _returnvalue (Actor|GetActorOfClass "/Game/TBOProject/Core/Camera/BP_GameCamera.BP_GameCamera_C"))
  (Variables|Default|SetCamera _returnvalue)
  (if (Variables|Default|GetEditable)
    _
    (else
      (CallFunction|SetCameraParameters)))
  (if (Variables|Modifier2|GetLenght)
    (Variables|Modifier3|SetDistance false)))

(event Collision|EventActorBeginOverlap
  (params (OtherActor :type Actor%20Object%20Reference)))

(event EventTick
  (params (DeltaSeconds :type Float%20%28single-precision%29)))

(fn ConstructionScript)

(fn SetCameraParameters
  (bind (_rotation _delta_yaw _delta_pitch _delta_roll _duration _lenght _delta_lenght _duration_0 _distance _curve _delta_arm_lenght) (Default|GetValue (Variables|Default|GetDataAsset)))
  (Utilities|FlowControl|Sequence
    (:then_0
      (Variables|Modifier1|SetRotation _rotation)
      (Variables|Modifier1|SetDelta%20Yaw _delta_yaw)
      (Variables|Modifier1|SetDelta%20Pitch _delta_pitch)
      (Variables|Modifier1|SetDelta%20Roll _delta_roll)
      (Variables|Modifier1|SetDuration _duration))
    (:then_1
      (Variables|Modifier2|SetLenght _lenght)
      (Variables|Modifier2|SetDelta%20Lenght _delta_lenght)
      (Variables|Modifier2|SetDuration_0 _duration_0))
    (:then_2
      (Variables|Modifier3|SetDistance _distance)
      (Variables|Modifier3|SetCurve _curve)
      (Variables|Modifier3|SetDelta%20Arm%20Lenght _delta_arm_lenght))))
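; BP_CameraModifier_DataStructure_TO_REMOVE is a placeholder data container for camera modifier settings, marked for removal by its name.
; A single GetValue function returns all stored variables at once: rotation and its yaw, pitch and roll deltas, arm length and distance values, durations, and a curve.
; It holds no camera logic and only exposes these values to callers.
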(fn GetValue
  (return (Variables|Modifier1|GetRotation) (Variables|Modifier1|GetDelta%20Yaw) (Variables|Modifier1|GetDelta%20Pitch) (Variables|Modifier1|GetDelta%20Roll) (Variables|Modifier1|GetDuration) (Variables|Modifier2|GetLenght) (Variables|Modifier2|GetDelta%20Lenght) (Variables|Modifier2|GetDuration_0) (Variables|Modifier3|GetDistance) (Variables|Modifier3|GetCurve) (Variables|Modifier3|GetDelta%20Arm%20Lenght)))
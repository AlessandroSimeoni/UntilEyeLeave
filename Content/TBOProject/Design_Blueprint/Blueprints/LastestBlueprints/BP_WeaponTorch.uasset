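; Three-pillar torch shrine that opens a door and reveals a hidden weapon collectable as pillars are activated.
; SpawnFloatingWeapon lights each pillar's Niagara flame; player overlap with pillars 1 and 2 lit opens Path3Door, saved by UniqueID and restored on BeginPlay.
; With all three lit, overlap triggers chained timelines: flames rise, converge on the uncollected weapon, reveal it, shrink, then regrow at their spawn points.
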(event OnComponentBeginOverlap(PlayerDetector)
  (params (OverlappedComponent :type Primitive%20Component%20Object%20Reference) (OtherActor :type Actor%20Object%20Reference) (OtherComp :type Primitive%20Component%20Object%20Reference) (OtherBodyIndex :type Integer) (bFromSweep :type Boolean) (SweepResult :type Hit%20Result%20Structure%20%28by%20ref%29))
  (if (== OtherActor (Game|GetPlayerCharacter 0))
    (if (Math|Boolean|ANDBoolean (Variables|Default|GetPillar1_IsActive) (Variables|Default|GetPillar2_IsActive) (not (Variables|Default|GetPillar3_IsActive)) (not (Variables|Default|GetDoorOpen)))
      (Variables|Default|SetDoorOpen true)
      (bind _path3door (Variables|Default|GetPath3Door)
        (:then
          (Class|ActionableActor|ActivateActor _path3door false)
          (bind _returnvalue (Class|SaveSubsystem|LoadGame (Subsystems|GetSaveSubsystem)))
          (Class|TBOSaveGame|AddInteractedActor _returnvalue (Variables|/Script/TBO_01.UniqueIDComponent|GetUniqueID (Variables|Default|GetUniqueID))))
        (:else))
      (elif (Math|Boolean|ANDBoolean (Variables|Default|GetPillar1_IsActive) (Variables|Default|GetPillar2_IsActive) (Variables|Default|GetPillar3_IsActive) (not (Variables|Default|GetSpawned)))
        (Variables|Default|SetSpawned true)
        (CallFunction|AttivazioneFiga)))))

(event Custom|SpawnFloatingWeapon
  (params (PillarNumber :type Integer))
  (if (> PillarNumber 0)
    (Rendering|SetVisibility (Utilities|Select :Index PillarNumber :Option%200 0 :Option%201 (Variables|Default|GetNiagara1) :Option%202 (Variables|Default|GetNiagara2) :Option%203 (Variables|Default|GetNiagara3)) true false)
    (switch int PillarNumber
      (:1
        (Variables|Default|SetPillar1_IsActive true))
      (:2
        (Variables|Default|SetPillar2_IsActive true))
      (:3
        (Variables|Default|SetPillar3_IsActive true)))))

(event Custom|PlaceFireAway
  (Transformation|SetWorldLocation (Variables|Default|GetNiagara1) (Transformation|GetWorldLocation (Variables|Default|GetSpawnPoint1)) false true)
  (Transformation|SetWorldLocation (Variables|Default|GetNiagara2) (Transformation|GetWorldLocation (Variables|Default|GetSpawnPoint2)) false true)
  (Transformation|SetWorldLocation (Variables|Default|GetNiagara3) (Transformation|GetWorldLocation (Variables|Default|GetSpawnPoint3)) false true)
  (bind (_direction _scala) (Timeline|Timeline_0 ReverseFromEnd)
    (:Update
      (Transformation|SetRelativeScale3D (Variables|Default|GetNiagara1) (Math|Vector|Lerp(Vector) "1.000000,1.000000,1.000000" "0, 0, 0" _scala)))
    (:Finished
      (switch Utilities|FlowControl|Switch|SwitchonETimelineDirection _direction
        (:Forward
          (Utilities|FlowControl|Delay 1.0)
          (CallFunction|PlaceFireAway))))))

(event Custom|ChangeCollectableStatus
  (params (On :type Boolean))
  (bind _weaponcollectable (Variables|Default|GetWeaponCollectable)
    (:then
      (Rendering|SetVisibility (Variables|/Script/Engine.Actor|GetRootComponent _weaponcollectable) On true)
      (Collision|SetActorEnableCollision _weaponcollectable On))
    (:else)))

(event Custom|AttivazioneFiga
  (bind _spawnpoint3 (Variables|Default|GetSpawnPoint3))
  (bind _spawnpoint2 (Variables|Default|GetSpawnPoint2))
  (bind _spawnpoint1 (Variables|Default|GetSpawnPoint1))
  (bind _returnvalue (Transformation|GetWorldLocation _spawnpoint3))
  (bind _returnvalue_2 (Transformation|GetWorldLocation _spawnpoint2))
  (bind _returnvalue_3 (Transformation|GetWorldLocation _spawnpoint1))
  (bind _returnvalue_4 (+ _returnvalue_3 "0.000000,0.000000,100.000000"))
  (bind _returnvalue_5 (+ _returnvalue "0.000000,0.000000,100.000000"))
  (bind _returnvalue_6 (+ _returnvalue_2 "0.000000,0.000000,100.000000"))
  (bind _weaponcollectable (Variables|Default|GetWeaponCollectable)
    (:then
      (if (not (Variables|/Script/TBO_01.CollectableItems|GetItemCollected _weaponcollectable))
        (bind _altezza_iniziale (Timeline|ActivateFlames PlayFromStart)
          (:Update
            (Transformation|SetWorldLocation (Variables|Default|GetNiagara3) (Math|Vector|Lerp(Vector) _returnvalue _returnvalue_5 _altezza_iniziale) false false)
            (Transformation|SetWorldLocation (Variables|Default|GetNiagara2) (Math|Vector|Lerp(Vector) _returnvalue_2 _returnvalue_6 _altezza_iniziale) false false)
            (Transformation|SetWorldLocation (Variables|Default|GetNiagara1) (Math|Vector|Lerp(Vector) _returnvalue_3 _returnvalue_4 _altezza_iniziale) false false))
          (:Finished
            (bind _spostamento (Timeline|Timeline PlayFromStart)
              (:Update
                (Transformation|SetWorldLocation (Variables|Default|GetNiagara3) (Math|Vector|Lerp(Vector) _returnvalue_5 (Transformation|GetWorldLocation (Variables|/Script/Engine.Actor|GetRootComponent (Variables|Default|GetWeaponCollectable))) _spostamento) false false)
                (Transformation|SetWorldLocation (Variables|Default|GetNiagara2) (Math|Vector|Lerp(Vector) _returnvalue_6 (Transformation|GetWorldLocation (Variables|/Script/Engine.Actor|GetRootComponent (Variables|Default|GetWeaponCollectable))) _spostamento) false false)
                (Transformation|SetWorldLocation (Variables|Default|GetNiagara1) (Math|Vector|Lerp(Vector) _returnvalue_4 (Transformation|GetWorldLocation (Variables|/Script/Engine.Actor|GetRootComponent (Variables|Default|GetWeaponCollectable))) _spostamento) false false))
              (:Finished
                (CallFunction|ChangeCollectableStatus true)
                (bind (_direction _scala) (Timeline|Timeline_0 PlayFromStart)
                  (:Update
                    (Transformation|SetRelativeScale3D (Variables|Default|GetNiagara1) (Math|Vector|Lerp(Vector) "1.000000,1.000000,1.000000" "0, 0, 0" _scala)))
                  (:Finished
                    (switch Utilities|FlowControl|Switch|SwitchonETimelineDirection _direction
                      (:Forward
                        (Utilities|FlowControl|Delay 1.0)
                        (CallFunction|PlaceFireAway)))))))))))
    (:else)))

(event EventBeginPlay
  (CallFunction|ChangeCollectableStatus false)
  (Rendering|SetVisibility (Variables|Default|GetNiagara1) false false)
  (CallFunction|ReadGameSaveandOpenDoor))

(fn ConstructionScript)

(fn ReadGameSaveandOpenDoor
  (bind _returnvalue (Class|SaveSubsystem|LoadGame (Subsystems|GetSaveSubsystem)))
  (bind _returnvalue_2 (Class|TBOSaveGame|FindInteractedActor _returnvalue (Variables|/Script/TBO_01.UniqueIDComponent|GetUniqueID (Variables|Default|GetUniqueID))))
  (if _returnvalue_2
    (Variables|Default|SetDoorOpen true)
    (bind _path3door (Variables|Default|GetPath3Door)
      (:then
        (Class|ActionableActor|ActivateActor _path3door true))
      (:else))))
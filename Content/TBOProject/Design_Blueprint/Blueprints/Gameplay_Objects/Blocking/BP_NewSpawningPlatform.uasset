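; A spawning platform whose four floor pieces move into place and become solid when the actor is activated.
; On BeginPlay the meshes get an emissive floating material and have collision disabled.
; ActivateActor switches to the floor material and plays a timeline that lerps each piece from its current relative location and rotation toward its paired scene component, with separate alpha tracks.
; A timeline event track turns collision back on.
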(event Custom|Move%20Piece
  (bind _staticmesh1 (Variables|Default|GetStaticMesh1))
  (bind _staticmesh2 (Variables|Default|GetStaticMesh2))
  (bind _scene4 (Variables|Default|GetScene4))
  (bind _staticmesh3 (Variables|Default|GetStaticMesh3))
  (bind _staticmesh4 (Variables|Default|GetStaticMesh4))
  (bind _staticmesh1_2 (Variables|Default|GetStaticMesh1))
  (bind _scene1 (Variables|Default|GetScene1))
  (bind _scene2 (Variables|Default|GetScene2))
  (bind _staticmesh2_2 (Variables|Default|GetStaticMesh2))
  (bind _staticmesh3_2 (Variables|Default|GetStaticMesh3))
  (bind _staticmesh4_2 (Variables|Default|GetStaticMesh4))
  (bind _scene3 (Variables|Default|GetScene3))
  (CallFunction|ChangeMaterial true)
  (bind (_direction _location _rotation) (Timeline|Timeline PlayFromStart)
    (:Update
      (Transformation|SetRelativeLocation _staticmesh1 (Math|Vector|Lerp(Vector) (Variables|/Script/Engine.SceneComponent|GetRelativeLocation _staticmesh1_2) (Variables|/Script/Engine.SceneComponent|GetRelativeLocation _scene1) _location) false false)
      (Transformation|SetRelativeRotation _staticmesh1 (Math|Rotator|Lerp(Rotator) (Variables|/Script/Engine.SceneComponent|GetRelativeRotation _staticmesh1_2) (Variables|/Script/Engine.SceneComponent|GetRelativeRotation _scene1) _rotation) false false)
      (Transformation|SetRelativeLocation _staticmesh2 (Math|Vector|Lerp(Vector) (Variables|/Script/Engine.SceneComponent|GetRelativeLocation _staticmesh2_2) (Variables|/Script/Engine.SceneComponent|GetRelativeLocation _scene2) _location) false false)
      (Transformation|SetRelativeRotation _staticmesh2 (Math|Rotator|Lerp(Rotator) (Variables|/Script/Engine.SceneComponent|GetRelativeRotation _staticmesh2_2) (Variables|/Script/Engine.SceneComponent|GetRelativeRotation _scene2) _rotation) false false)
      (Transformation|SetRelativeLocation _staticmesh3 (Math|Vector|Lerp(Vector) (Variables|/Script/Engine.SceneComponent|GetRelativeLocation _staticmesh3_2) (Variables|/Script/Engine.SceneComponent|GetRelativeLocation _scene3) _location) false false)
      (Transformation|SetRelativeRotation _staticmesh3 (Math|Rotator|Lerp(Rotator) (Variables|/Script/Engine.SceneComponent|GetRelativeRotation _staticmesh3_2) (Variables|/Script/Engine.SceneComponent|GetRelativeRotation _scene3) _rotation) false false)
      (Transformation|SetRelativeLocation _staticmesh4 (Math|Vector|Lerp(Vector) (Variables|/Script/Engine.SceneComponent|GetRelativeLocation _staticmesh4_2) (Variables|/Script/Engine.SceneComponent|GetRelativeLocation _scene4) _location) false false)
      (Transformation|SetRelativeRotation _staticmesh4 (Math|Rotator|Lerp(Rotator) (Variables|/Script/Engine.SceneComponent|GetRelativeRotation _staticmesh4_2) (Variables|/Script/Engine.SceneComponent|GetRelativeRotation _scene4) _rotation) false false))
    (:NewTrack_0
      (CallFunction|ChangeCollision true))))

(event Custom|ChangeMaterial
  (params (On :type Boolean))
  (Rendering|Material|SetMaterial (Variables|Default|GetStaticMesh1) 0 (select On "/Game/TBOProject/Art/MasterMaterial(Dont_Touch)/M_Floor_Placeholder.M_Floor_Placeholder" "/Game/TBOProject/MaterialLibrary/FloatingMaterials/MI_Floating_Floor_Emissive.MI_Floating_Floor_Emissive")))

(event Custom|ChangeCollision
  (params (Index :type Boolean))
  (Collision|SetCollisionEnabled (Variables|Default|GetStaticMesh1) (select Index "QueryAndPhysics" "NoCollision")))

(event EventBeginPlay
  (CallFunction|ChangeMaterial false)
  (CallFunction|ChangeCollision false))

(event EventActivateActor
  (params (InstantActivation :type Boolean))
  (CallFunction|MovePiece))

(fn ConstructionScript)
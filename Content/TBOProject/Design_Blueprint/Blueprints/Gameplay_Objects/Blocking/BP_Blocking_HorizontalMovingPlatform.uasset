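; Horizontal moving platform that temporarily blocks the main character with two volumes and two sliding meshes during movement.
; Non-instant activation or deactivation arms a trigger, disabled at BeginPlay; character overlap disarms it, enables both blocking volumes and plays a timeline.
; The timeline lerps both meshes' relative X toward TargetMeshHeight's X.
; When movement ends, the volumes and trigger lose collision and the timeline reverses the meshes.
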(event OnComponentBeginOverlap(TriggerBlockingVolumes)
  (params (OverlappedComponent :type Primitive%20Component%20Object%20Reference) (OtherActor :type Actor%20Object%20Reference) (OtherComp :type Primitive%20Component%20Object%20Reference) (OtherBodyIndex :type Integer) (bFromSweep :type Boolean) (SweepResult :type Hit%20Result%20Structure%20%28by%20ref%29))
  (bind _startingblockingmeshlocation1 (Variables|Default|GetStartingBlockingMeshLocation1))
  (bind _startingblockingmeshlocation2 (Variables|Default|GetStartingBlockingMeshLocation2))
  (bind _targetmeshheight (Variables|Default|GetTargetMeshHeight))
  (bind _relativelocation (Variables|/Script/Engine.SceneComponent|GetRelativeLocation _targetmeshheight))
  (if (Class|GameplayStatics|ObjectIsA OtherActor "/Game/TBOProject/Core/Characters/Player/BP_MainCharacter.BP_MainCharacter_C")
    (Collision|SetCollisionEnabled (Variables|Default|GetTriggerBlockingVolumes) "NoCollision")
    (Collision|SetCollisionEnabled (Variables|Default|GetblockingVolume1) "QueryAndPhysics")
    (Collision|SetCollisionEnabled (Variables|Default|GetblockingVolume2) "QueryAndPhysics")
    (bind _newtrack_0 (Timeline|BlockingMeshtimeline PlayFromStart)
      (:Update
        (Transformation|SetRelativeLocation (Variables|Default|GetblockingMesh1) (Math|Vector|MakeVector (Math|Float|Lerp (.x (Variables|Default|GetStartingBlockingMeshLocation1)) (.x _relativelocation) _newtrack_0) (.y _startingblockingmeshlocation1) (.z _startingblockingmeshlocation1)) false false)
        (Transformation|SetRelativeLocation (Variables|Default|GetblockingMesh2) (Math|Vector|MakeVector (Math|Float|Lerp (.x (Variables|Default|GetStartingBlockingMeshLocation2)) (.x _relativelocation) _newtrack_0) (.y _startingblockingmeshlocation2) (.z _startingblockingmeshlocation2)) false false)))))

(event Custom|ReverseBlockingMeshOnMovementEnd
  (bind _startingblockingmeshlocation1 (Variables|Default|GetStartingBlockingMeshLocation1))
  (bind _startingblockingmeshlocation2 (Variables|Default|GetStartingBlockingMeshLocation2))
  (bind _targetmeshheight (Variables|Default|GetTargetMeshHeight))
  (bind _relativelocation (Variables|/Script/Engine.SceneComponent|GetRelativeLocation _targetmeshheight))
  (bind _newtrack_0 (Timeline|BlockingMeshtimeline Reverse)
    (:Update
      (Transformation|SetRelativeLocation (Variables|Default|GetblockingMesh1) (Math|Vector|MakeVector (Math|Float|Lerp (.x (Variables|Default|GetStartingBlockingMeshLocation1)) (.x _relativelocation) _newtrack_0) (.y _startingblockingmeshlocation1) (.z _startingblockingmeshlocation1)) false false)
      (Transformation|SetRelativeLocation (Variables|Default|GetblockingMesh2) (Math|Vector|MakeVector (Math|Float|Lerp (.x (Variables|Default|GetStartingBlockingMeshLocation2)) (.x _relativelocation) _newtrack_0) (.y _startingblockingmeshlocation2) (.z _startingblockingmeshlocation2)) false false))))

(event EventActivateActor
  (params (InstantActivation :type Boolean))
  (if InstantActivation
    _
    (else
      (Collision|SetCollisionEnabled (Variables|Default|GetTriggerBlockingVolumes) "QueryOnly")))
  (|CallParentFunction InstantActivation))

(event EventDeActivateActor
  (params (InstantDeActivation :type Boolean))
  (if InstantDeActivation
    _
    (else
      (Collision|SetCollisionEnabled (Variables|Default|GetTriggerBlockingVolumes) "QueryOnly")))
  (|CallParentFunction InstantDeActivation))

(event EventBeginPlay
  (Variables|Default|SetStartingBlockingMeshLocation1 (Variables|/Script/Engine.SceneComponent|GetRelativeLocation (Variables|Default|GetblockingMesh1)))
  (Variables|Default|SetStartingBlockingMeshLocation2 (Variables|/Script/Engine.SceneComponent|GetRelativeLocation (Variables|Default|GetblockingMesh2)))
  (Components|Timeline|SetPlayRate (Variables|Default|GetblockingMeshTimeline) (Variables|Default|GetBlockingMeshPlayRate))
  (Collision|SetCollisionEnabled (Variables|Default|GetTriggerBlockingVolumes) "NoCollision"))

(fn ConstructionScript
  (|CallParentFunction))

(fn OnMovementEnd
  (|CallParentFunction)
  (Collision|SetCollisionEnabled (Variables|Default|GetblockingVolume1) "NoCollision")
  (Collision|SetCollisionEnabled (Variables|Default|GetblockingVolume2) "NoCollision")
  (Collision|SetCollisionEnabled (Variables|Default|GetTriggerBlockingVolumes) "NoCollision")
  (CallFunction|ReverseBlockingMeshonMovementEnd))
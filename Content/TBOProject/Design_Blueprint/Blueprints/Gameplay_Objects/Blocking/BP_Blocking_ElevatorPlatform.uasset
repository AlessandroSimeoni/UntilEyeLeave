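; Blocking elevator platform that moves its moving part vertically between a bottom and a top position marker.
; Activate and deactivate both toggle the state, either instantly or through a timeline scaled by MovingSpeed that lerps relative Z.
; A first-interaction flag lets an initial downward move reverse from the timeline's end.
; A sound plays on animated moves and stops when movement finishes.
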(event EventActivateActor
  (params (InstantActivation :type Boolean))
  (bind _movingpart (Variables|Default|GetMovingPart))
  (bind _relativelocation (Variables|/Script/Engine.SceneComponent|GetRelativeLocation _movingpart))
  (if InstantActivation
    (Class|MovingPlatform|InstantStateChange (not (Variables|Default|GetCurrentlyUp)))
    (else
      ;[1 1 1] Play sound
      (Audio|Components|Audio|Play (Variables|Default|GetSFX) 0.0)
      (bind _output_get (Variables|Default|SetCurrentlyUp (not (Variables|Default|GetCurrentlyUp))))
      (CallFunction|SetAnimationTime)
      (if (not _output_get)
        (if (Variables|Default|GetIsFirstInteraction)
          (Variables|Default|SetIsFirstInteraction false)
          (bind _newtrack_0 (Timeline|MoveUpAnim ReverseFromEnd)
            (:Update
              (Transformation|SetRelativeLocation _movingpart (Math|Vector|MakeVector (.x _relativelocation) (.y _relativelocation) (Math|Float|Lerp (.z (Variables|/Script/Engine.SceneComponent|GetRelativeLocation (Variables|Default|GetBottomPosition))) (.z (Variables|/Script/Engine.SceneComponent|GetRelativeLocation (Variables|Default|GetTopPosition))) _newtrack_0)) false false))
            (:Finished
              (CallFunction|OnMovementEnd)))
          (else
            (Timeline|MoveUpAnim Reverse)))
        (else
          (Variables|Default|SetIsFirstInteraction false)
          (Timeline|MoveUpAnim Play))))))

(event EventDeActivateActor
  (params (InstantDeActivation :type Boolean))
  (bind _movingpart (Variables|Default|GetMovingPart))
  (bind _relativelocation (Variables|/Script/Engine.SceneComponent|GetRelativeLocation _movingpart))
  (if InstantDeActivation
    (Class|MovingPlatform|InstantStateChange (not (Variables|Default|GetCurrentlyUp)))
    (else
      ;[1 1 1] Play sound
      (Audio|Components|Audio|Play (Variables|Default|GetSFX) 0.0)
      (bind _output_get (Variables|Default|SetCurrentlyUp (not (Variables|Default|GetCurrentlyUp))))
      (CallFunction|SetAnimationTime)
      (if (not _output_get)
        (if (Variables|Default|GetIsFirstInteraction)
          (Variables|Default|SetIsFirstInteraction false)
          (bind _newtrack_0 (Timeline|MoveUpAnim ReverseFromEnd)
            (:Update
              (Transformation|SetRelativeLocation _movingpart (Math|Vector|MakeVector (.x _relativelocation) (.y _relativelocation) (Math|Float|Lerp (.z (Variables|/Script/Engine.SceneComponent|GetRelativeLocation (Variables|Default|GetBottomPosition))) (.z (Variables|/Script/Engine.SceneComponent|GetRelativeLocation (Variables|Default|GetTopPosition))) _newtrack_0)) false false))
            (:Finished
              (CallFunction|OnMovementEnd)))
          (else
            (Timeline|MoveUpAnim Reverse)))
        (else
          (Variables|Default|SetIsFirstInteraction false)
          (Timeline|MoveUpAnim Play))))))

(fn ConstructionScript
  (|CallParentFunction))

(fn SetAnimationTime
  (Components|Timeline|SetPlayRate (Variables|Default|GetMoveUpAnim) (/ 1.0 (Variables|Default|GetMoving%20Speed))))

(fn OnMovementEnd
  ;[1 1 1] Stop sound
  (Audio|Components|Audio|Stop (Variables|Default|GetSFX)))
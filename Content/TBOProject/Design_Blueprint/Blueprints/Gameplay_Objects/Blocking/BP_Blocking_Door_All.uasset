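; Blocking double door that toggles between open and closed when activated or deactivated, playing a gate sound at its location.
; Both events share the same toggle logic, either calling InstantStateChange or running the OpenAnim timeline to swing the left and right pivots in opposite yaw directions.
; If the first interaction is a close, the timeline reverses from its end, so doors that start open animate correctly.
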(event EventActivateActor
  (params (InstantActivation :type Boolean))
  ;[1 1 1] Play SFX
  (Audio|PlaySoundatLocation "/Game/TBOProject/Media/Sound/Interactables/SFX_Gate.SFX_Gate" (Transformation|GetActorLocation) "0, 0, 0" 1.0 1.0 0.0 0 0 0 0)
  (if InstantActivation
    (Class|DoubleDoor|InstantStateChange (not (Variables|Default|GetCurrentlyOpen)))
    (else
      (bind _output_get (Variables|Default|SetCurrentlyOpen (not (Variables|Default|GetCurrentlyOpen))))
      (if (not _output_get)
        (if (Variables|Default|GetIsFirstInteraction)
          (Variables|Default|SetIsFirstInteraction false)
          (bind _newtrack_0 (Timeline|OpenAnim ReverseFromEnd)
            (:Update
              (Transformation|SetRelativeRotation (Variables|Default|GetLeftDoorPivot) (Math|Rotator|MakeRotator 0.0 0.0 (Math|Float|Lerp 0.0 9e+01 _newtrack_0)) false false)
              (Transformation|SetRelativeRotation (Variables|Default|GetRightDoorPivot) (Math|Rotator|MakeRotator 0.0 0.0 (Math|Float|Lerp 0.0 -9e+01 _newtrack_0)) false false)))
          (else
            (Timeline|OpenAnim Reverse)))
        (else
          (Variables|Default|SetIsFirstInteraction false)
          (Timeline|OpenAnim Play))))))

(event EventDeActivateActor
  (params (InstantDeActivation :type Boolean))
  ;[1 1 1] Play SFX
  (Audio|PlaySoundatLocation "/Game/TBOProject/Media/Sound/Interactables/SFX_Gate.SFX_Gate" (Transformation|GetActorLocation) "0, 0, 0" 1.0 1.0 0.0 0 0 0 0)
  (if InstantDeActivation
    (Class|DoubleDoor|InstantStateChange (not (Variables|Default|GetCurrentlyOpen)))
    (else
      (bind _output_get (Variables|Default|SetCurrentlyOpen (not (Variables|Default|GetCurrentlyOpen))))
      (if (not _output_get)
        (if (Variables|Default|GetIsFirstInteraction)
          (Variables|Default|SetIsFirstInteraction false)
          (bind _newtrack_0 (Timeline|OpenAnim ReverseFromEnd)
            (:Update
              (Transformation|SetRelativeRotation (Variables|Default|GetLeftDoorPivot) (Math|Rotator|MakeRotator 0.0 0.0 (Math|Float|Lerp 0.0 9e+01 _newtrack_0)) false false)
              (Transformation|SetRelativeRotation (Variables|Default|GetRightDoorPivot) (Math|Rotator|MakeRotator 0.0 0.0 (Math|Float|Lerp 0.0 -9e+01 _newtrack_0)) false false)))
          (else
            (Timeline|OpenAnim Reverse)))
        (else
          (Variables|Default|SetIsFirstInteraction false)
          (Timeline|OpenAnim Play))))))

(fn ConstructionScript
  (|CallParentFunction))
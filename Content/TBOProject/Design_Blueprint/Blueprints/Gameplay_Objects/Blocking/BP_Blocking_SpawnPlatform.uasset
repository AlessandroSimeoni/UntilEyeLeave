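; Blocking platform actor that assembles from four mesh pieces, or separates back into them, when activated or deactivated.
; Activation and deactivation both toggle the state, either instantly or through a timeline that lerps each piece between its starting transform and a target component.
; The animated move updates the collision box and plays a sound on finish, then either enables the CanFloat material parameter on separated pieces or sets the assembled platform to block.
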(event Custom|MovePlatformPieces
  (params (On :type Boolean))
  (Components|Timeline|SetPlayRate (Variables|Default|GetTimeline) (Variables|Default|GetPlayRate))
  (Class|SpawnPlatform|UpdateCollisionBox (not On))
  (CallFunction|SetCanFloatMeshesMaterial 0.0)
  (if On
    (if (Variables|Default|GetIsFirstInteraction)
      (Variables|Default|SetIsFirstInteraction false)
      (bind (_direction _location _rotation) (Timeline|Timeline ReverseFromEnd)
        (:Update
          (Utilities|FlowControl|Sequence
            (:then_0
              (CallFunction|MovePlatformMesh (Variables|Default|GetPlatformMeshA) (Variables|Default|GetStartingLocationMeshA) (Variables|Default|GetStartingRotationMeshA) (Variables|Default|GetMeshTargetLocationA) _location _rotation))
            (:then_1
              (CallFunction|MovePlatformMesh (Variables|Default|GetPlatformMeshB) (Variables|Default|GetStartingLocationMeshB) (Variables|Default|GetStartingRotationMeshB) (Variables|Default|GetMeshTargetLocationB) _location _rotation))
            (:then_2
              (CallFunction|MovePlatformMesh (Variables|Default|GetPlatformMeshC) (Variables|Default|GetStartingLocationMeshC) (Variables|Default|GetStartingRotationMeshC) (Variables|Default|GetMeshTargetLocationC) _location _rotation))
            (:then_3
              (CallFunction|MovePlatformMesh (Variables|Default|GetPlatformMeshD) (Variables|Default|GetStartingLocationMeshD) (Variables|Default|GetStartingRotationMeshD) (Variables|Default|GetMeshTargetLocationD) _location _rotation))))
        (:Finished
          ;[1 1 1] Play sound
          (Audio|PlaySoundatLocation "/Game/TBOProject/Media/Sound/Interactables/SFX_SpawningPlatform.SFX_SpawningPlatform" (Transformation|GetWorldLocation (Variables|Default|GetPlatformMeshA)) "0, 0, 0" 1.0 1.0 0.0 0 0 0 0)
          (if On
            (CallFunction|SetCanFloatMeshesMaterial 1.0)
            (else
              (Collision|SetCollisionProfileName (Variables|Default|GetPlatformCollision) "BlockAllDynamic" false :!class /Script/Engine.PrimitiveComponent)))))
      (else
        (Timeline|Timeline Reverse)))
    (else
      (Variables|Default|SetIsFirstInteraction false)
      (Timeline|Timeline Play))))

(event EventDeActivateActor
  (params (InstantDeActivation :type Boolean))
  (if InstantDeActivation
    (Class|SpawnPlatform|InstantStateChange (not (Variables|Default|GetCurrentlyOn)))
    (else
      (bind _output_get (Variables|Default|SetCurrentlyOn (not (Variables|Default|GetCurrentlyOn))))
      (CallFunction|MovePlatformPieces (not _output_get)))))

(event EventActivateActor
  (params (InstantActivation :type Boolean))
  (if InstantActivation
    (Class|SpawnPlatform|InstantStateChange (not (Variables|Default|GetCurrentlyOn)))
    (else
      (bind _output_get (Variables|Default|SetCurrentlyOn (not (Variables|Default|GetCurrentlyOn))))
      (CallFunction|MovePlatformPieces (not _output_get)))))

(fn ConstructionScript
  (|CallParentFunction))

(fn MovePlatformMesh
  (params (PlatformMesh :type Static%20Mesh%20Component%20Object%20Reference) (StartingMeshLocation :type Vector) (StartingMeshRotation :type Rotator) (TargetSceneComponent :type Scene%20Component%20Object%20Reference) (AlphaLocation :type Float%20%28single-precision%29) (AlphaRotation :type Float%20%28single-precision%29))
  (Transformation|SetRelativeLocation PlatformMesh (Math|Vector|Lerp(Vector) StartingMeshLocation (Variables|/Script/Engine.SceneComponent|GetRelativeLocation TargetSceneComponent) AlphaLocation) false false)
  (Transformation|SetRelativeRotation PlatformMesh (Math|Rotator|Lerp(Rotator) StartingMeshRotation (Variables|/Script/Engine.SceneComponent|GetRelativeRotation TargetSceneComponent) AlphaRotation true) false false))

(fn SetCanFloatMeshesMaterial
  (params (Value :type Float%20%28double-precision%29))
  (Utilities|FlowControl|Sequence
    (:then_0
      (Rendering|Material|SetScalarParameterValue (Variables|Default|GetMeshADynMatInstance) "CanFloat" Value :!class /Script/Engine.MaterialInstanceDynamic))
    (:then_1
      (Rendering|Material|SetScalarParameterValue (Variables|Default|GetMeshBDynMatInstance) "CanFloat" Value :!class /Script/Engine.MaterialInstanceDynamic))
    (:then_2
      (Rendering|Material|SetScalarParameterValue (Variables|Default|GetMeshCDynMatInstance) "CanFloat" Value :!class /Script/Engine.MaterialInstanceDynamic))
    (:then_3
      (Rendering|Material|SetScalarParameterValue (Variables|Default|GetMeshDDynMatInstance) "CanFloat" Value :!class /Script/Engine.MaterialInstanceDynamic))))
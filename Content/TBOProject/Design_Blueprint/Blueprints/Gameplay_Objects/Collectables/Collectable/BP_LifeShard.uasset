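; BP_LifeShard is a collectable life shard that the player picks up to progressively increase maximum health.
; On successful interaction it increments the save game's shard count and swaps the pop-up for a pickup widget on the HUD stack.
; Whenever the count reaches a multiple of the character's threshold, it raises max health, heals by that amount and resizes the health bar.
; The pickup sound event is an empty placeholder.
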(event EventPlayCollectableSFX
  ;[1 1 1] L'AUDIO VA QUI
)

(event EventInteract
  (|CallParentFunction))

(event EventOnInteractSuccess
  (bind _returnvalue (Game|GetPlayerController 0))
  (bind _returnvalue_2 (Game|GetPlayerCharacter 0))
  (bind _asbp_main_character (Utilities|Casting|CastToBP_MainCharacter _returnvalue_2))
  (bind _asbp_character_controller (Utilities|Casting|CastToBP_CharacterController _returnvalue))
  (bind _lifecomponent (Variables|/Script/TBO_01.MainCharacter|GetLifeComponent _asbp_main_character))
  (bind _result (Math|Integer|IncrementInt (Variables|/Script/TBO_01.TBOSaveGame|GetLifeShardsCollected (Variables|Default|GetTBOSaveGame)))
    (:%20%20
      (Default|RemovePopUpStack _asbp_character_controller)
      (Class|CommonActivatableWidgetContainerBase|AddWidget (Variables|/Game/TBOProject/UI/JournalWidget/W_HUDStack.W_HUDStack_C|GetHudStack (Variables|/Game/TBOProject/Core/Characters/Player/BP_CharacterController.BP_CharacterController_C|GetHud_StackWidget _asbp_character_controller)) "/Game/TBOProject/UI/JournalWidget/W_LifeShardPickUp.W_LifeShardPickUp_C")
      (if (== (Math|Integer|%(Integer) _result (Variables|/Game/TBOProject/Core/Characters/Player/BP_MainCharacter.BP_MainCharacter_C|GetHealthIncreaseLifeShards _asbp_main_character)) 0)
        ;[1 1 1] increase player health
        (bind _result_2 (Math|Float|IncrementFloat (Variables|/Script/TBO_01.LifeSystemComponent|GetMaxHealth _lifecomponent))
          (:%20%20
            (Class|LifeSystemComponent|ReceiveHeal _lifecomponent _result_2)
            (Class|PlayerHealthBar|ResizeHealthBar (Variables|/Script/TBO_01.HUDWidget|GetHealthBar (Variables|/Game/TBOProject/Core/Gamemodes/Play/GM_Play.GM_Play_C|GetHUDWidget (.AsGM%20Play (Utilities|Casting|CastToGM_Play (Game|GetGameMode))))))))))))

(fn ConstructionScript)
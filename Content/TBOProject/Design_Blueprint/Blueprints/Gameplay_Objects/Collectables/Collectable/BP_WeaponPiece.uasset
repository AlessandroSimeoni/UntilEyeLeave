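; BP_WeaponPiece is an interactable collectable that adds to the saved weapon part count and drives the player's weapon upgrades.
; A successful interaction calls ActionActors, has the linked WeaponTorch spawn a floating weapon by PathNumber, and shows a pickup widget, followed by a delayed growl sound.
; A modulo check on the count against the character's threshold raises the weapon level and swaps the weapon.
; WeaponTorchNotify can also trigger the torch spawn separately.
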(event EventPlayCollectableSFX
  ;[1 1 1] L'AUDIO VA QUI
)

(event EventWeaponTorchNotify
  (bind _weapontorch (Variables|Default|GetWeaponTorch)
    (:then
      (Default|SpawnFloatingWeapon _weapontorch (Variables|Default|GetPathNumber)))
    (:else)))

(event EventOnInteractSuccess
  (bind _returnvalue (Game|GetPlayerController 0))
  (bind _returnvalue_2 (Game|GetPlayerCharacter 0))
  (bind _asbp_main_character (Utilities|Casting|CastToBP_MainCharacter _returnvalue_2))
  (bind _asbp_character_controller (Utilities|Casting|CastToBP_CharacterController _returnvalue))
  (Utilities|FlowControl|Sequence
    (:then_0
      (Class|WeaponPiece|ActionActors false)
      (bind _result (Math|Integer|IncrementInt (Variables|/Script/TBO_01.TBOSaveGame|GetWeaponPartsCollected (Variables|Default|GetTBOSaveGame)))
        (:%20%20
          (bind _weapontorch (Variables|Default|GetWeaponTorch)
            (:then
              (Default|SpawnFloatingWeapon _weapontorch (Variables|Default|GetPathNumber)))
            (:else
              _))
          (if (== (Math|Integer|%(Integer) _result (Variables|/Game/TBOProject/Core/Characters/Player/BP_MainCharacter.BP_MainCharacter_C|GetLevelIncreaseWeaponParts _asbp_main_character)) 0)
            (bind _result_2 (Math|Float|IncrementFloat (Variables|/Script/TBO_01.MainCharacter|GetCurrentWeaponLevel _asbp_main_character))
              (:%20%20
                (Default|ChangeWeapon _asbp_main_character (Math|Float|Truncate _result_2)))))
          (Default|RemovePopUpStack _asbp_character_controller)
          (Class|CommonActivatableWidgetContainerBase|AddWidget (Variables|/Game/TBOProject/UI/JournalWidget/W_HUDStack.W_HUDStack_C|GetHudStack (Variables|/Game/TBOProject/Core/Characters/Player/BP_CharacterController.BP_CharacterController_C|GetHud_StackWidget _asbp_character_controller)) "/Game/TBOProject/UI/JournalWidget/W_WeaponPartPickUp.W_WeaponPartPickUp_C"))))
    (:then_1
      ;[1 1 1] play boss sound
      (Utilities|FlowControl|Delay 0.2)
      (Audio|PlaySound2D "/Game/TBOProject/Media/Sound/Boss/SFX_GrowlTestV2.SFX_GrowlTestV2" 0.2 1.0 0.0 0 0))))

(event EventInteract
  (|CallParentFunction))

(fn ConstructionScript)
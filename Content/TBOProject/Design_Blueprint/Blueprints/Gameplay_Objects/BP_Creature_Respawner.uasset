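; BP_Creature_Respawner is a gameplay object tied to a creature reference; this file holds only its construction-time labeling, with no respawn logic.
; After running the parent script, it checks that Creature is valid and writes its display name to the Text component.
; A chain of exact class comparisons then picks a matching Billboard icon for the Gianguscio, destructible Gianguscio, Birdman and MouseTrap variants, leaving other classes' sprites untouched.
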(fn ConstructionScript
  (bind _creature (Variables|Default|GetCreature))
  (bind _returnvalue (Utilities|GetClass _creature))
  (|CallParentFunction)
  (if (Utilities|IsValid (Variables|Default|GetCreature))
    (Rendering|Components|TextRender|SetText (Variables|Default|GetText) (Utilities|Text|ToText(String) (Utilities|GetDisplayName (Variables|Default|GetCreature))))
    (if (== _returnvalue "/Game/TBOProject/Design_Blueprint/CreaturesIA/B01_Destructible/BP_B01_Destructible_Gianguscio_ShooterCreatureBase_Child.BP_B01_Destructible_Gianguscio_ShooterCreatureBase_Child_C")
      (Rendering|Components|Sprite|SetSprite (Variables|Default|GetBillboard) "/Game/TBOProject/Design_Blueprint/Blueprints/UI_Placeholder/IconGenerator/Generated_Icons/RT_Icon_EB01.RT_Icon_EB01")
      (elif (== _returnvalue "/Game/TBOProject/Design_Blueprint/CreaturesIA/B03/BP_B03_Birdman_ShooterCreatureBase_Child.BP_B03_Birdman_ShooterCreatureBase_Child_C")
        (Rendering|Components|Sprite|SetSprite (Variables|Default|GetBillboard) "/Game/TBOProject/Design_Blueprint/Blueprints/UI_Placeholder/IconGenerator/Generated_Icons/RT_Icon_B03.RT_Icon_B03")
        (elif (== _returnvalue "/Game/TBOProject/Design_Blueprint/CreaturesIA/B02/BP_B02_MouseTrap_Creature_Child.BP_B02_MouseTrap_Creature_Child_C")
          (Rendering|Components|Sprite|SetSprite (Variables|Default|GetBillboard) "/Game/TBOProject/Design_Blueprint/Blueprints/UI_Placeholder/IconGenerator/Generated_Icons/RT_Icon_B02.RT_Icon_B02")
          (elif (== _returnvalue "/Game/TBOProject/Core/Creatures/Character/B01_Gianguscio/BP_B01_Gianguscio_CreatureBase.BP_B01_Gianguscio_CreatureBase_C")
            (Rendering|Components|Sprite|SetSprite (Variables|Default|GetBillboard) "/Game/TBOProject/Design_Blueprint/Blueprints/UI_Placeholder/IconGenerator/Generated_Icons/RT_Icon_B01.RT_Icon_B01")))))))
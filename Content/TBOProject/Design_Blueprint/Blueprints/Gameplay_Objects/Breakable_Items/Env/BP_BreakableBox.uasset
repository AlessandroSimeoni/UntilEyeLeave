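; Breakable box environment object that can drop a healing item when destroyed.
; On pre-destruction, the DropsHalfHeart and DropsFullHeart flags select a half-heart or full-heart pickup to spawn at Cube0's transform.
; CompleteDestruction follows the spawn, or runs directly when neither flag is set.
; With both flags set, nothing spawns and CompleteDestruction is not called.
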(event EventBeginPlay)

(event Collision|EventActorBeginOverlap
  (params (OtherActor :type Actor%20Object%20Reference)))

(event EventTick
  (params (DeltaSeconds :type Float%20%28single-precision%29)))

(event EventOnPreDestruction
  (bind _drops_fullheart (Variables|Default|GetDrops%20FullHeart))
  (if (Variables|Default|GetDrops%20HalfHeart)
    (if (not _drops_fullheart)
      (Game|SpawnActorfromClass "/Game/TBOProject/Core/Actor/HealingItem/BP_HealingItem_HalfHeart.BP_HealingItem_HalfHeart_C" (Transformation|GetWorldTransform (Variables|Default|GetCube_0)) "Undefined" "MultiplyWithRoot" 0 0)
      (Class|DestructibleActor|CompleteDestruction :!label _label))
    (elif _drops_fullheart
      (Game|SpawnActorfromClass "/Game/TBOProject/Core/Actor/HealingItem/BP_HealingItem_FullHeart.BP_HealingItem_FullHeart_C" (Transformation|GetWorldTransform (Variables|Default|GetCube_0)) "Undefined" "MultiplyWithRoot" 0 0)
      (goto _label)
      (else
        (goto _label)))))

(fn ConstructionScript
  (|CallParentFunction))
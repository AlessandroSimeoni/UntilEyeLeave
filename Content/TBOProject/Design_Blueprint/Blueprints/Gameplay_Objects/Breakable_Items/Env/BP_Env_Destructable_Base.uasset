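; Base Blueprint for destructible environment objects that can drop a half-heart or full-heart healing pickup when broken.
; On pre-destruction, two boolean flags choose which healing item spawns at the SpawnHeartPoint location, then CompleteDestruction runs.
; With neither flag set it completes destruction without a drop; with both set it neither spawns nor calls CompleteDestruction.
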(event EventBeginPlay)

(event Collision|EventActorBeginOverlap
  (params (OtherActor :type Actor%20Object%20Reference)))

(event EventTick
  (params (DeltaSeconds :type Float%20%28single-precision%29)))

(event EventOnPreDestruction
  (bind _dropsfullheart (Variables|Default|GetDropsFullHeart))
  (if (Variables|Default|GetDropsHalfHeart)
    (if (not _dropsfullheart)
      (Game|SpawnActorfromClass "/Game/TBOProject/Core/Actor/HealingItem/BP_HealingItem_HalfHeart.BP_HealingItem_HalfHeart_C" (Math|Transform|MakeTransform (Transformation|GetWorldLocation (Variables|Default|GetSpawnHeartPoint))) "Undefined" "MultiplyWithRoot" 0 0)
      (Class|DestructibleActor|CompleteDestruction :!label _label))
    (elif _dropsfullheart
      (Game|SpawnActorfromClass "/Game/TBOProject/Core/Actor/HealingItem/BP_HealingItem_FullHeart.BP_HealingItem_FullHeart_C" (Math|Transform|MakeTransform (Transformation|GetWorldLocation (Variables|Default|GetSpawnHeartPoint))) "Undefined" "MultiplyWithRoot" 0 0)
      (goto _label)
      (else
        (goto _label)))))

(fn ConstructionScript
  (|CallParentFunction))
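; BP_BreakableShell is a breakable environment shell whose fracture decals and resistance depend on its HardnessLevel.
; The construction script sets two decals to a level 1 or level 2 fracture material, with only the highest option using level 2.
; BeginPlay derives ResistanceLevel from HardnessLevel with a floor for low values, and OnPreDestruction calls CompleteDestruction.
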(event EventBeginPlay
  (bind _hardness_level (Variables|Default|GetHardness%20level))
  (if (<= _hardness_level 1)
    (Variables|Default|SetResistanceLevel 2)
    (else
      (Variables|Default|SetResistanceLevel _hardness_level))))

(event Collision|EventActorBeginOverlap
  (params (OtherActor :type Actor%20Object%20Reference)))

(event EventTick
  (params (DeltaSeconds :type Float%20%28single-precision%29)))

(event EventOnPreDestruction
  (Class|DestructibleActor|CompleteDestruction))

(fn ConstructionScript
  (Rendering|Components|Decal|SetDecalMaterial (Variables|Default|GetDecal) (Utilities|Select :Index (Variables|Default|GetHardness%20level) :Option%200 "/Game/TBOProject/Effects/VFX/Material/MI_Fracture_LV1.MI_Fracture_LV1" :Option%201 "/Game/TBOProject/Effects/VFX/Material/MI_Fracture_LV1.MI_Fracture_LV1" :Option%202 "/Game/TBOProject/Effects/VFX/Material/MI_Fracture_LV1.MI_Fracture_LV1" :Option%203 "/Game/TBOProject/Effects/VFX/Material/MI_Fracture_LV2.MI_Fracture_LV2")))
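; BP_BreakableWall_Little is a breakable wall with a hardness level, shown through debug-style text labels and a crack decal set at construction.
; On destruction it saves its unique ID, plays a sound, and swaps the static mesh for a geometry collection playing a cached Chaos simulation.
; A timed dissolve material fades the debris, and destruction completes when playback ends.
; On BeginPlay it destroys itself if the save records it as already broken.
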(event Custom|OnChaosReachEnd_Event
  (params (bReverse :type Boolean))
  (Class|DestructibleActor|CompleteDestruction))

(event Custom|Dissolve
  (bind _returnvalue (Rendering|Material|CreateDynamicMaterialInstance (Variables|Default|GetDissolveMaterial) "None" "None" :!class /Script/Engine.KismetMaterialLibrary))
  (Rendering|Material|SetScalarParameterValue _returnvalue "DissolveStartTime" (Utilities|Time|GetTimeSeconds) :!class /Script/Engine.MaterialInstanceDynamic)
  (Rendering|Material|SetMaterial (Variables|Default|GetGeometryCollection) 0 _returnvalue))

(event EventBeginPlay
  (CallFunction|RestoreState)
  (Class|ChaosCacheHandler|InitializeCollection (Variables|Default|GetChaosCacheHandler) (Variables|Default|GetGeometryCollection) (Variables|Default|GetCacheCollection)))

(event EventRestoreState
  (bind _returnvalue (Class|SaveSubsystem|LoadGame (Subsystems|GetSaveSubsystem)))
  (bind _returnvalue_2 (Class|TBOSaveGame|FindInteractedActor _returnvalue (Variables|/Script/TBO_01.UniqueIDComponent|GetUniqueID (Variables|Default|GetUniqueID))))
  (if _returnvalue_2
    (Actor|DestroyActor)))

(event EventOnPreDestruction
  (bind _staticmesh (Variables|Default|GetStaticMesh))
  (bind _chaoscachehandler (Variables|Default|GetChaosCacheHandler))
  (bind _returnvalue (Class|SaveSubsystem|LoadGame (Subsystems|GetSaveSubsystem)))
  (Class|TBOSaveGame|AddInteractedActor _returnvalue (Variables|/Script/TBO_01.UniqueIDComponent|GetUniqueID (Variables|Default|GetUniqueID)))
  (Audio|SpawnSoundatLocation (Variables|Default|GetSound) (Transformation|GetActorLocation) "0, 0, 0" 1.0 1.0 0.0 0 0)
  (Rendering|SetVisibility _staticmesh false true)
  (Collision|SetCollisionEnabled _staticmesh "NoCollision")
  (for _array_element (Components|GetChildrenComponents _staticmesh true)
    (bind _asstatic_mesh_component (Utilities|Casting|CastToStaticMeshComponent _array_element))
    (Collision|SetCollisionEnabled _asstatic_mesh_component "NoCollision"))
  (Rendering|SetVisibility (Variables|Default|GetDecal) false false)
  (Rendering|SetVisibility (Variables|Default|GetGeometryCollection) true false)
  (Class|ChaosCacheHandler|Play _chaoscachehandler 1.0)
  (EventDispatchers|AssignOnChaosReachEnd _chaoscachehandler (delegate Custom|OnChaosReachEnd_Event))
  (Utilities|Time|SetTimerbyEvent (delegate Custom|Dissolve) 2.0))

(fn ConstructionScript
  (Rendering|Components|TextRender|SetText (Variables|Default|GetTXT_Hardness_1) (Utilities|Text|FormatText "Hardness: {Num}" (Utilities|Text|ToText(Integer) (Variables|Default|GetHardness%20level))))
  (Rendering|Components|Decal|SetDecalMaterial (Variables|Default|GetDecal) (Utilities|Select :Index (Variables|Default|GetHardness%20level) :Option%200 "/Game/TBOProject/Effects/VFX/Material/Crack/M_TilableCrack_Lv1.M_TilableCrack_Lv1" :Option%201 "/Game/TBOProject/Effects/VFX/Material/Crack/M_TilableCrack_Lv1.M_TilableCrack_Lv1" :Option%202 "/Game/TBOProject/Effects/VFX/Material/Crack/M_TilableCrack_Lv1.M_TilableCrack_Lv1" :Option%203 "/Game/TBOProject/Effects/VFX/Material/Crack/M_TilableCrack_Lv2.M_TilableCrack_Lv2")))

(fn HasBeenActivated
  (return false))
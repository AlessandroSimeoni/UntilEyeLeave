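; BP_Breaking_Platform is a platform that shakes and shatters when the player character steps into its trigger box.
; Only a platform flagged IsMain responds to overlap, then recursively activates the other platforms in its BreakingPlatforms list.
; A timeline bobs the root vertically with sound, then the mesh is swapped for a geometry collection playing a cached Chaos fracture.
; Collision is destroyed at that point and the actor removes itself after a short delay.
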(event OnComponentBeginOverlap(Box)
  (params (OverlappedComponent :type Primitive%20Component%20Object%20Reference) (OtherActor :type Actor%20Object%20Reference) (OtherComp :type Primitive%20Component%20Object%20Reference) (OtherBodyIndex :type Integer) (bFromSweep :type Boolean) (SweepResult :type Hit%20Result%20Structure%20%28by%20ref%29))
  (if (and (== OtherActor (Game|GetPlayerCharacter 0)) (not (Variables|Default|GetActivated)))
    (if (Variables|Default|GetIsMain)
      (CallFunction|Activate))))

(event Custom|Activate
  (Variables|Default|SetActivated true)
  (if (>= (Utilities|Array|Length (Variables|Default|GetBreaking_Platforms)) 1)
    (for _array_element (Variables|Default|GetBreaking_Platforms)
      (if (Utilities|IsValid _array_element)
        (CallFunction|Activate _array_element))))
  (CallFunction|ShakeAnimation))

(event Custom|ShakeAnimation
  (bind _defaultsceneroot (Variables|Default|GetDefaultSceneRoot))
  (bind _returnvalue (Transformation|GetWorldLocation _defaultsceneroot))
  (Variables|Default|SetStartingPos _returnvalue)
  (Audio|PlaySoundatLocation "/Game/TBOProject/Media/Sound/MetasoundSystems/MS_BreakingPlatform.MS_BreakingPlatform" _returnvalue "0, 0, 0" 1.0 1.0 0.0 "/Game/TBOProject/Media/Sound/Utilities/SoundAttenuation.SoundAttenuation" 0 0 0)
  (bind _newtrack_0 (Timeline|TL_Shake PlayFromStart)
    (:Update
      (Transformation|SetWorldLocation (Variables|Default|GetDefaultSceneRoot) (Math|Vector|MakeVector (.x (Variables|Default|GetStartingPos)) (.y (Variables|Default|GetStartingPos)) (Math|Float|Lerp (.z (Variables|Default|GetStartingPos)) (+ (.z (Variables|Default|GetStartingPos)) 1e+01) _newtrack_0)) false false))
    (:Finished
      ;[1 1 1] Chaos system activation
      (CallFunction|ChaosSystemPlay)
      ;[1 1 1] Disable collision and destroy actor after some time.
      (Components|DestroyComponent (Variables|Default|GetBoxCollision))
      (Utilities|FlowControl|Delay 2.0)
      (Actor|DestroyActor))))

(event Collision|EventActorBeginOverlap
  (params (OtherActor :type Actor%20Object%20Reference)))

(event EventTick
  (params (DeltaSeconds :type Float%20%28single-precision%29)))

(fn ConstructionScript)

(fn ChaosSystemPlay
  (Class|ChaosCacheHandler|InitializeCollection (Variables|Default|GetChaosCacheHandler) (Variables|Default|GetGeometryCollection) "/Game/TBOProject/Art/Chaos/BreakingPlatform/CCC_BreakingPlatform.CCC_BreakingPlatform")
  (Rendering|SetVisibility (Variables|Default|GetStaticMesh) false false)
  (Rendering|SetVisibility (Variables|Default|GetGeometryCollection) true false)
  (Class|ChaosCacheHandler|Play (Variables|Default|GetChaosCacheHandler) 1.0))
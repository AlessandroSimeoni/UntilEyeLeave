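; BP_Interactable_StreetLight is an interactable streetlight that breaks apart when the lamp is hit.
; The hit event plays a breaking sound, hides the mesh and decal, disables mesh collision and reveals a geometry collection.
; ChaosCacheHandler plays a cached Chaos destruction on that collection.
; The construction script extends the parent's, setting a text render to show green or red lantern status from HasLantern.
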(event EventOnStreeTLampHit
  (Audio|PlaySoundatLocation "/Game/TBOProject/Media/Sound/Interactables/SFX_StreetlightBreaking.SFX_StreetlightBreaking" (Transformation|GetActorLocation) "0, 0, 0" 1.0 1.0 0.0 0 0 0 0)
  (Class|ChaosCacheHandler|InitializeCollection (Variables|Default|GetChaosCacheHandler) (Variables|Default|GetGeometryCollection) "/Game/TBOProject/Art/Chaos/Streetlight/CCC_Streetlight.CCC_Streetlight")
  (Rendering|SetVisibility (Variables|Default|GetMeshComponent) false false)
  (Collision|SetCollisionEnabled (Variables|Default|GetMeshComponent) "NoCollision")
  (Rendering|SetVisibility (Variables|Default|GetGeometryCollection) true false)
  (Class|ChaosCacheHandler|Play (Variables|Default|GetChaosCacheHandler) 1.0)
  (Rendering|SetVisibility (Variables|Default|GetDecal) false false))

(fn ConstructionScript
  (bind _textrender (Variables|Default|GetTextRender))
  (bind _haslantern (Variables|Default|GetHasLantern))
  (|CallParentFunction)
  (Rendering|Components|TextRender|SetText _textrender (Utilities|String|SelectText (Utilities|Text|FormatText "HAS 
LANTERN") (Utilities|Text|FormatText "HASN'T 
LANTERN") _haslantern))
  (Rendering|Components|TextRender|SetTextRenderColor _textrender (Math|Color|MakeColor 0 (select _haslantern 255 0) (select _haslantern 0 255) 255)))
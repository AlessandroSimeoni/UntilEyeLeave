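; Pressure plate interactable Blueprint that lowers and raises its ground collision as it is activated and deactivated.
; MoveGroundCollisions plays or reverses the PlateCollisionMovement timeline, which lerps CollisionBoxA between mirrored vertical offsets without sweeping.
; Construction defers to the parent class, and HasBeenActivated always returns false.
; The file does not show what triggers MoveGroundCollisions.
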(event EventMoveGroundCollisions
  (params (Activation :type Boolean))
  (bind _returnvalue (Math|Vector|MakeVector 0.0 0.0 12.0))
  (if Activation
    (bind _newtrack_0 (Timeline|PlateCollisionMovement Play)
      (:Update
        (Transformation|SetRelativeLocation (Variables|Default|GetCollisionBox_A) (Math|Vector|Lerp(Vector) _returnvalue (* _returnvalue -1.0) _newtrack_0) false false)))
    (else
      (Timeline|PlateCollisionMovement Reverse))))

(fn ConstructionScript
  (|CallParentFunction))

(fn HasBeenActivated
  (return false))
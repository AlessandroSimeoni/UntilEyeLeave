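; Puzzle statue that is solved when its target creature type, chosen by CreatureNumber in the construction script, dies or loses all eyes within range.
; An entering creature receives StatueInfluence, triggers hint and range VFX, and is tracked by the statue's recursive look-at loop.
; Its death spawns a soul that flies into the statue, then ActivateItem resets rotation, collapses the range, lowers the altar and calls ActionActors, skipped on restore.
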(event Custom|RotateTo
  ;[0 1 0.02101] RotateStatue
  (Transformation|SetWorldRotation (Variables|Default|GetRotatingPoint) (Math|Rotator|MakeRotator 0.0 0.0 (.yaw (Math|Rotator|FindLookatRotation (Transformation|GetWorldLocation (Variables|Default|GetRotatingPoint)) (Transformation|GetActorLocation (Variables|Default|GetCreatureIn))))) false false)
  (Utilities|FlowControl|Delay 0.1)
  (if (and (not (Variables|Default|GetSolved)) (Utilities|IsValid (Variables|Default|GetCreatureIn)))
    (CallFunction|Rotateto)))

(event Custom|ChangeVFXHeight
  (params (IsTall :type Boolean))
  (bind _rangescale (Variables|Default|GetRangeScale))
  (if IsTall
    (CallFunction|AddSizeVfx)
    (bind _newtrack_0 (Timeline|TL_HighCircle Play)
      (:Update
        (Transformation|SetRelativeScale3D (Variables|Default|GetVFX_Range) (Math|Vector|Lerp(Vector) (Math|Vector|MakeVector (.x _rangescale) (.y _rangescale) (.z _rangescale)) (Math|Vector|MakeVector (.x _rangescale) (.y _rangescale) (* (.z _rangescale) 3.0)) _newtrack_0))))
    (else
      (CallFunction|SubstractSizeVfx)
      (Timeline|TL_HighCircle Reverse))))

(event Custom|SubstractSizeVfx
  (bind _newtrack_0 (Timeline|Timeline_1 Play)
    (:Update
      (Transformation|SetRelativeScale3D (Variables|Default|GetRangeFX) (Math|Vector|Lerp(Vector) (Math|Vector|MakeVector 0.0 0.0 1.15) (Math|Vector|MakeVector 1.15 1.15 1.15) _newtrack_0)))))

(event Custom|AddSizeVfx
  (bind _newtrack_0 (Timeline|Timeline_1 ReverseFromEnd)
    (:Update
      (Transformation|SetRelativeScale3D (Variables|Default|GetRangeFX) (Math|Vector|Lerp(Vector) (Math|Vector|MakeVector 0.0 0.0 1.15) (Math|Vector|MakeVector 1.15 1.15 1.15) _newtrack_0)))))

(event Custom|UpdateMaterials
  (bind _solved (Variables|Default|GetSolved))
  ;[0 1 0.04347] Change Material
  (Rendering|SetVisibility (Variables|Default|GetPointLight) _solved false)
  (if (not _solved)
    (Rendering|Material|SetMaterial (Variables|Default|GetFakeEyeStatus) 0 (select (and (not _solved) (Variables|Default|GetISPlayerNear)) "/Game/TBOProject/Art/MasterMaterial(Dont_Touch)/MI_Ticking.MI_Ticking" "/Game/TBOProject/Art/MasterMaterial(Dont_Touch)/M_Floor_Placeholder.M_Floor_Placeholder"))))

(event Custom|ActivateItem
  ;[1 1 1] Activation
  (if (not (Variables|Default|GetSolved))
    (Variables|Default|SetSolved true)
    (CallFunction|ReturntoStartingRotation)
    (Variables|Default|SetRangeScale (Variables|/Script/Engine.SceneComponent|GetRelativeScale3D (Variables|Default|GetVFX_Range)))
    ;;[1 1 1] Play sound
    (Audio|PlaySoundatLocation "/Game/TBOProject/Media/Sound/Interactables/SFX_StatueActivated.SFX_StatueActivated" (Transformation|GetWorldLocation (Variables|Default|GetAltarMesh)) "0, 0, 0" 1.0 1.0 0.0 0 0 0 0)
    (bind _newtrack_0 (Timeline|Timeline PlayFromStart)
      (:Update
        (Transformation|SetRelativeScale3D (Variables|Default|GetVFX_Range) (Math|Vector|Lerp(Vector) (Math|Vector|MakeVector 0.0 0.0 (.z (Variables|Default|GetRangeScale))) (Math|Vector|MakeVector (.x (Variables|Default|GetRangeScale)) (.y (Variables|Default|GetRangeScale)) (.z (Variables|Default|GetRangeScale))) _newtrack_0)))
      (:Finished
        (Rendering|SetVisibility (Variables|Default|GetVFX_Range) false false)
        (CallFunction|MoveBase true)
        (CallFunction|UpdateMaterials)
        (if (not (Variables|Default|GetbRestoreState))
          (Class|ActuatorActor|ActionActors false))))))

(event Custom|ShowHint
  ;[0.7505 1 0.005986] Hint
  (Niagara|SpawnSystemAttached "/Game/TBOProject/Effects/VFX/Niagara/NS_Spotted.NS_Spotted" (Variables|Default|GetStatueMesh) "Spotted" "0, 0, 0" "0, 0, 0" "SnapToTargetIncludingScale" false))

(event Custom|ReturnToStartingRotation
  (Variables|Default|SetLastRotation (Variables|/Script/Engine.SceneComponent|GetRelativeRotation (Variables|Default|GetRotatingPoint)))
  (bind _newtrack_0 (Timeline|Timeline_0 PlayFromStart)
    (:Update
      (Transformation|SetWorldRotation (Variables|Default|GetRotatingPoint) (Math|Rotator|Lerp(Rotator) (Variables|Default|GetLastRotation) (Variables|Default|GetStartingRotation) _newtrack_0) false false))))

(event Custom|MoveBase
  (params (GoDown :type Boolean))
  (if GoDown
    (bind _newtrack_0 (Timeline|MoveBase_TL PlayFromStart)
      (:Update
        (Transformation|SetRelativeLocation (Variables|Default|GetAltarBase) (Math|Vector|Lerp(Vector) (Variables|Default|GetBaseStartingLocation) "0.000000,0.000000,-100.000000" _newtrack_0) false false)))
    (else
      (Timeline|MoveBase_TL ReverseFromEnd))))

(event Custom|CreatureEyeDeath
  (params (Eye :type Eye%20Scene%20Component%20Object%20Reference) (Instigator :type Actor%20Object%20Reference))
  (bind _creaturein (Variables|Default|GetCreatureIn))
  (bind _returnvalue (Transformation|GetActorTransform _creaturein))
  (if (and (Utilities|IsValid (Variables|Default|GetCreatureIn)) (not (Variables|Default|GetSolved)))
    (Variables|Default|GetSoul
      (:then)
      (:else
        (bind _returnvalue_2 (Game|SpawnActorfromClass "/Game/TBOProject/Design_Blueprint/Blueprints/Gameplay_Objects/BP_StatueSoul.BP_StatueSoul_C" (Math|Transform|MakeTransform (.location _returnvalue) (.rotation _returnvalue) "1.000000,1.000000,1.000000") "AlwaysSpawn" "MultiplyWithRoot" 0 0))
        (bind _output_get (Variables|Default|SetSoul _returnvalue_2))
        (Variables|Default|SetSoulSpawnLocation (Transformation|GetActorLocation _output_get))
        (bind _newtrack_0 (Timeline|Soul_TL PlayFromStart)
          (:Update
            (Transformation|SetActorLocation (Variables|Default|GetSoul) (Math|Vector|Lerp(Vector) (Variables|Default|GetSoulSpawnLocation) (Transformation|GetWorldLocation (Variables|Default|GetStatueMesh)) _newtrack_0) false false))
          (:Finished
            (Actor|DestroyActor (Variables|Default|GetSoul))
            (CallFunction|ActivateItem)))))))

(event Custom|OnDeath_Event
  (params (Actor :type Actor%20Object%20Reference) (Instigator :type Actor%20Object%20Reference))
  (bind _creaturein (Variables|Default|GetCreatureIn))
  (bind _returnvalue (Transformation|GetActorTransform _creaturein))
  (if (and (Utilities|IsValid (Variables|Default|GetCreatureIn)) (not (Variables|Default|GetSolved)))
    (Variables|Default|GetSoul
      (:then)
      (:else
        (bind _returnvalue_2 (Game|SpawnActorfromClass "/Game/TBOProject/Design_Blueprint/Blueprints/Gameplay_Objects/BP_StatueSoul.BP_StatueSoul_C" (Math|Transform|MakeTransform (.location _returnvalue) (.rotation _returnvalue) "1.000000,1.000000,1.000000") "AlwaysSpawn" "MultiplyWithRoot" 0 0))
        (bind _output_get (Variables|Default|SetSoul _returnvalue_2))
        (Variables|Default|SetSoulSpawnLocation (Transformation|GetActorLocation _output_get))
        (bind _newtrack_0 (Timeline|Soul_TL PlayFromStart)
          (:Update
            (Transformation|SetActorLocation (Variables|Default|GetSoul) (Math|Vector|Lerp(Vector) (Variables|Default|GetSoulSpawnLocation) (Transformation|GetWorldLocation (Variables|Default|GetStatueMesh)) _newtrack_0) false false))
          (:Finished
            (Actor|DestroyActor (Variables|Default|GetSoul))
            (CallFunction|ActivateItem)))))))

(event Custom|Remember
  (bind _ascreature (Utilities|Casting|CastToCreature (Variables|Default|GetCreatureIn)))
  (bind _returnvalue (Class|EyesHandlerInterface|GetEyesHandlerActorComponent _ascreature))
  (EventDispatchers|BindEventtoOnAllEyesDeath _returnvalue (delegate Custom|CreatureEyeDeath))
  (EventDispatchers|AssignOnDeath _ascreature (delegate Custom|OnDeath_Event)))

(event EventBeginPlay
  (bind _vfx_range (Variables|Default|GetVFX_Range))
  (Components|Tick|SetComponentTickEnabled (Variables|Default|GetStatueMesh) false)
  (Components|Tick|SetComponentTickEnabled (Variables|Default|GetStatueMesh1) false)
  (CallFunction|UpdateMaterials)
  (Rendering|SetVisibility (Variables|Default|GetVFX_Range) false false)
  (Variables|Default|SetStartingRotation (Variables|/Script/Engine.SceneComponent|GetRelativeRotation (Variables|Default|GetRotatingPoint)))
  (Variables|Default|SetBaseStartingLocation (Variables|/Script/Engine.SceneComponent|GetRelativeLocation (Variables|Default|GetAltarBase)))
  (Variables|Default|SetRangeScale (Variables|/Script/Engine.SceneComponent|GetRelativeScale3D _vfx_range))
  (Rendering|SetVisibility _vfx_range true false))

(event EventOnRestore
  (Variables|Default|SetbRestoreState true)
  (CallFunction|ActivateItem))

(event Collision|EventActorEndOverlap
  (params (OtherActor :type Actor%20Object%20Reference))
  (if (== OtherActor (Game|GetPlayerCharacter 0))
    (Variables|Default|SetISPlayerNear false)
    (if (not (Variables|Default|GetSolved))
      (CallFunction|UpdateMaterials))
    (elif (and (Class|GameplayStatics|ObjectIsA OtherActor (Variables|Default|GetCreatureTarget)) (not (Variables|Default|GetSolved)))
      (Utilities|IsValid (Variables|Default|GetCreatureIn)
        (:Is%20Valid
          (GameplayEffects|RemoveActiveEffectswithGrantedTags (Ability|GetAbilitySystemComponent (Variables|Default|GetCreatureIn)) "(GameplayTags=((TagName=\"Status.StatueInfluence\")))")
          (Variables|Default|SetCreatureIn 0)
          (CallFunction|ChangeVFXHeight false)
          (Development|PrintText "Creature Exit" true true "(R=1.000000,G=0.008603,B=0.000000,A=1.000000)"))))))

(event Collision|EventActorBeginOverlap
  (params (OtherActor :type Actor%20Object%20Reference))
  (if (== (Game|GetPlayerCharacter 0) OtherActor)
    (Variables|Default|SetISPlayerNear true)
    (if (not (Variables|Default|GetSolved))
      (CallFunction|UpdateMaterials))
    (elif (and (Class|GameplayStatics|ObjectIsA OtherActor (Variables|Default|GetCreatureTarget)) (not (Variables|Default|GetSolved)))
      (CallFunction|ShowHint)
      (CallFunction|ChangeVFXHeight true)
      (bind _output_get (Variables|Default|SetCreatureIn OtherActor))
      (GameplayEffects|ApplyGameplayEffectToSelf :self (Ability|GetAbilitySystemComponent _output_get) :GameplayEffectClass "/Game/TBOProject/Core/Creatures/Abilities/Effects/GE_StatueInfluence.GE_StatueInfluence_C")
      (CallFunction|Rotateto)
      (CallFunction|Remember))))

(fn ConstructionScript
  (bind _creaturenumber (Variables|Default|GetCreatureNumber))
  (bind _statuemesh (Variables|Default|GetStatueMesh))
  (bind _returnvalue (== _creaturenumber 1))
  (bind _returnvalue_2 (== _creaturenumber 0))
  (Variables|Default|SetCreatureTarget (Utilities|Select :Index (Variables|Default|GetCreatureNumber) :Option%200 "/Game/TBOProject/Core/Creatures/Character/B02_MouseTrap/BP_B02_MouseTrap_Creature.BP_B02_MouseTrap_Creature_C" :Option%201 "/Game/TBOProject/Core/Creatures/Character/B03_Birdman/BP_B03_Birdman_ShooterCreatureBase.BP_B03_Birdman_ShooterCreatureBase_C" :Option%202 "/Game/TBOProject/Core/Creatures/Character/B01_Gianguscio/BP_B01_Broken_Gianguscio_ShooterCreatureBase.BP_B01_Broken_Gianguscio_ShooterCreatureBase_C"))
  (if (== (Variables|Default|GetCreatureNumber) 2)
    (Rendering|SetVisibility (Variables|Default|GetStatueMesh1) true true)
    (Rendering|SetVisibility (Variables|Default|GetStatueMesh) false true)
    (elif (or _returnvalue_2 _returnvalue)
      (if _returnvalue_2
        (Components|SkeletalMesh|SetSkeletalMeshAsset _statuemesh "/Game/TBOProject/Art/Creatures/Mousetrap/SK_Mousetrap.SK_Mousetrap")
        (Rendering|SetVisibility (Variables|Default|GetStatueMesh1) false true :!label _label)
        (Rendering|SetVisibility (Variables|Default|GetStatueMesh) true true)
        (elif _returnvalue
          (Components|SkeletalMesh|SetSkeletalMeshAsset _statuemesh "/Game/TBOProject/Art/Creatures/Birdman/SK_Birdman.SK_Birdman")
          (goto _label))))))
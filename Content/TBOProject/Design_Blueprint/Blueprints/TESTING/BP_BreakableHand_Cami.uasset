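; Boss hand that performs repeated slam attacks, each spawning a ring attack, with HandLeft selecting mesh and phase behavior.
; PhaseActivation makes the left hand spawn a MouseTrap creature and respawner, then strike BossPoint (phase 2); the other spawns Gianguscio and strikes random boxes (phase 4).
; A looping timer line-traces downward to position a decal as a fake shadow.
; A hit from the MouseTrap creature advances the boss phase and destroys the hand.
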(event OnComponentBeginOverlap(PlayerDetector)
  (params (OverlappedComponent :type Primitive%20Component%20Object%20Reference) (OtherActor :type Actor%20Object%20Reference) (OtherComp :type Primitive%20Component%20Object%20Reference) (OtherBodyIndex :type Integer) (bFromSweep :type Boolean) (SweepResult :type Hit%20Result%20Structure%20%28by%20ref%29))
  (Utilities|Casting|CastToBP_MainCharacter OtherActor))

(event Custom|PhaseActivation
  (bind _spawnpoint (Variables|Default|GetSpawnPoint))
  (bind _returnvalue (Transformation|GetWorldTransform _spawnpoint))
  (if (Variables|Default|GetHandLeft)
    ;[1 1 1] Hand Behaviour Phase 2
    (bind _returnvalue_2 (Game|SpawnActorfromClass "/Game/TBOProject/Design_Blueprint/CreaturesIA/B02/BP_B02_MouseTrap_Creature_Child.BP_B02_MouseTrap_Creature_Child_C" _returnvalue "AdjustIfPossibleButAlwaysSpawn" "MultiplyWithRoot" 0 0))
    (Variables|Default|SetMouse _returnvalue_2)
    (Game|SpawnActorfromClass "/Game/TBOProject/Design_Blueprint/Blueprints/Gameplay_Objects/BP_Creature_Respawner.BP_Creature_Respawner_C" _returnvalue "AlwaysSpawn" "MultiplyWithRoot" 0 0)
    (Utilities|FlowControl|Delay (Variables|Default|GetAttackCooldown))
    (CallFunction|AttackBase)
    (else
      ;[1 1 1] Hand Beahaviour Phase 4
      (Game|SpawnActorfromClass "/Game/TBOProject/Design_Blueprint/CreaturesIA/B01/BP_TESTING_Gianguscio.BP_TESTING_Gianguscio_C" (Transformation|GetWorldTransform (Variables|Default|GetSpawnPoint)) "AdjustIfPossibleButAlwaysSpawn" "MultiplyWithRoot" 0 0)
      (Utilities|FlowControl|Delay (Variables|Default|GetAttackCooldown))
      (CallFunction|RandomAttack))))

(event Custom|AttackBase
  ;[1 1 1] Phase2
  (CallFunction|Attack (Variables|/Script/Engine.SceneComponent|GetRelativeLocation (Variables|Default|GetBossPoint)))
  (Utilities|FlowControl|Delay (Variables|Default|GetAttackCooldown))
  (if (> (Variables|Default|GetAttackNumbers) 0)
    (CallFunction|AttackBase)
    (else
      (Utilities|FlowControl|Delay (Variables|Default|GetWaitingTime))
      (Variables|Default|SetAttackNumbers 3)
      (CallFunction|AttackBase))))

(event Custom|RandomAttack
  ;[1 1 1] Phase4
  (switch int (Math|Random|RandomIntegerinRange 0 2)
    (:0
      (CallFunction|Attack (Variables|/Script/Engine.SceneComponent|GetRelativeLocation (Variables|Default|GetBox))))
    (:1
      (CallFunction|Attack (Variables|/Script/Engine.SceneComponent|GetRelativeLocation (Variables|Default|GetBox1))))
    (:2
      (CallFunction|Attack (Variables|/Script/Engine.SceneComponent|GetRelativeLocation (Variables|Default|GetBox2)))))
  (Utilities|FlowControl|Delay (Variables|Default|GetAttackCooldown))
  (if (> (Variables|Default|GetAttackNumbers) 0)
    (CallFunction|RandomAttack)
    (else
      (CallFunction|AttackBase)
      (Utilities|FlowControl|Delay (Variables|Default|GetWaitingTime))
      (Variables|Default|SetAttackNumbers 3)
      (CallFunction|RandomAttack))))

(event Custom|CastShadow
  (bind _handmesh (Variables|Default|GetHandMesh))
  (bind _returnvalue (Transformation|GetWorldLocation _handmesh))
  ;[1 1 1] Move decal to create a fake shadow effect
  ;;[0.1192 0.09891 0.5365] Fire event looping with timer
  (bind _outhit (Collision|LineTraceByChannel _returnvalue (- _returnvalue (Math|Vector|MakeVector 0.0 0.0 (Variables|Default|GetTraceLenght))) "TraceTypeQuery1" false 0 "None" true "(R=1.000000,G=0.000000,B=0.000000,A=1.000000)" "(R=0.000000,G=1.000000,B=0.000000,A=1.000000)" 0.5))
  ;;[0.1192 0.09891 0.5365] Move the decal to the linetrace impact location
  (Transformation|SetWorldLocation (Variables|Default|GetShadowDecal) (.location _outhit) false false))

(event Custom|Attack
  (params (TargetLocation :type Vector))
  ;[1 1 1] Move to Point 1
  (Math|Integer|DecrementInt (Variables|Default|GetAttackNumbers)
    (:%20%20
      (Transformation|SetRelativeLocation (Variables|Default|GetHandPoint) (Math|Vector|MakeVector (.x TargetLocation) (.y TargetLocation) (+ (.z TargetLocation) 3e+02)) false false)
      (Utilities|FlowControl|Delay 1.0)
      ;;[1 0 0] Attack
      (Transformation|SetRelativeLocation (Variables|Default|GetHandPoint) (Math|Vector|MakeVector (.x TargetLocation) (.y TargetLocation) 0.0) false false)
      (Game|SpawnActorfromClass "/Game/TBOProject/Design_Blueprint/RingAttack/BP_RingAttack.BP_RingAttack_C" (Transformation|GetWorldTransform (Variables|Default|GetHandPoint)) "AlwaysSpawn" "MultiplyWithRoot" 0 0))))

(event EventBeginPlay
  (bind _handmesh (Variables|Default|GetHandMesh))
  (Utilities|FlowControl|Sequence
    (:then_0
      ;[1 1 1] Move decal to create a fake shadow effect
      ;;[0.1192 0.09891 0.5365] Fire event looping with timer
      (Utilities|Time|SetTimerbyEvent (delegate Custom|CastShadow) 0.03 true))
    (:then_1
      (if (Variables|Default|GetHandLeft)
        (Components|StaticMesh|SetStaticMesh _handmesh "/Game/TBOProject/Design_Blueprint/Blueprints/TESTING/hand/source/hand.hand")
        (else
          (Components|StaticMesh|SetStaticMesh _handmesh "/Game/TBOProject/Design_Blueprint/Blueprints/TESTING/hand/source/hand2.hand2")
          (Transformation|SetRelativeRotation _handmesh "-40.000000,0.000000,180.000000" false false)
          (Transformation|SetRelativeRotation (Variables|Default|GetShadowDecal) "40.000000,0.000000,-180.000000" false false)
          (Transformation|SetRelativeRotation (Variables|Default|GetPlayerDetector) "-40.000000,0.000000,180.000000" false false))))))

(fn ConstructionScript)

(fn Hit
  (params (CharacterLevel :type Integer) (DamageValue :type Float%20%28single-precision%29) (AttackInstigator :type Actor%20Object%20Reference))
  (Utilities|Casting|CastToBP_B02_MouseTrap_Creature_Child AttackInstigator)
  (Default|ChangePhase (Variables|Default|GetBossRef))
  (Actor|DestroyActor)
  (return false))
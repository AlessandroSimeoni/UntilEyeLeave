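; BP_BulletSestr is a projectile that damages the main character on contact and is linked to a boss through a reference.
; A sphere overlap with the character applies damage through its LifeComponent and destroys the bullet, which otherwise expires after its lifetime.
; SetBulletSpeed sets both initial and maximum speed on the ProjectileMovement component.
; A pre-destruction event tells the referenced boss to change phase before completing destruction.
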(event OnComponentBeginOverlap(Sphere)
  (params (OverlappedComponent :type Primitive%20Component%20Object%20Reference) (OtherActor :type Actor%20Object%20Reference) (OtherComp :type Primitive%20Component%20Object%20Reference) (OtherBodyIndex :type Integer) (bFromSweep :type Boolean) (SweepResult :type Hit%20Result%20Structure%20%28by%20ref%29))
  (bind _asbp_main_character (Utilities|Casting|CastToBP_MainCharacter OtherActor))
  (Class|LifeSystemComponent|ReceiveDamage (Variables|/Script/TBO_01.MainCharacter|GetLifeComponent _asbp_main_character) 0.5)
  (Actor|DestroyActor))

(event Custom|SetBulletSpeed
  (params (Initial%20Speed :type Float%20%28single-precision%29))
  (bind _projectilemovement (Variables|Default|GetProjectileMovement))
  (bind _output_get (Variables|/Script/Engine.ProjectileMovementComponent|SetInitialSpeed _projectilemovement Initial%20Speed))
  (Variables|/Script/Engine.ProjectileMovementComponent|SetMaxSpeed _projectilemovement _output_get))

(event EventBeginPlay
  (Utilities|FlowControl|Delay (Variables|Default|GetLifeTime))
  (Actor|DestroyActor))

(event Collision|EventActorBeginOverlap
  (params (OtherActor :type Actor%20Object%20Reference)))

(event EventTick
  (params (DeltaSeconds :type Float%20%28single-precision%29)))

(event EventOnPreDestruction
  (Default|ChangePhase (Variables|Default|GetBossRef))
  (Class|DestructibleActor|CompleteDestruction))

(fn ConstructionScript
  (|CallParentFunction))
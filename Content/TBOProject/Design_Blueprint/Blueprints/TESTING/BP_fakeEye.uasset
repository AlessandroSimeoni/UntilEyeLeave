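; BP_fakeEye is a test actor for a boss fight, acting as a fake eye that advances the boss's phase when destroyed.
; On pre-destruction, it loses one Life only while the referenced boss is in phase 4.
; When Life reaches zero, it calls ChangePhase on the boss and completes its destruction.
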(event EventBeginPlay)

(event Collision|EventActorBeginOverlap
  (params (OtherActor :type Actor%20Object%20Reference)))

(event EventTick
  (params (DeltaSeconds :type Float%20%28single-precision%29)))

(event EventOnPreDestruction
  (bind _bossref (Variables|Default|GetBossRef))
  (bind _life (Variables|Default|GetLife))
  (if (== (Variables|/Game/TBOProject/Design_Blueprint/Blueprints/TESTING/BP_Boss.BP_Boss_C|GetActualPhase _bossref) 4)
    (Math|Integer|DecrementInt _life
      (:%20%20
        (if (== _life 0)
          (Default|ChangePhase _bossref)
          (Class|DestructibleActor|CompleteDestruction))))))

(fn ConstructionScript
  (|CallParentFunction))
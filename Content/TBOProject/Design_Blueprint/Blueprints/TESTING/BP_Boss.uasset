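; Multi-phase boss that activates after a delay when the player enters its trigger, and is destroyed after phase four.
; External ChangePhase calls advance it: phases 1 and 3 loop timed shooting patterns, while 2 and 4 activate the left and right hands.
; Shots spawn from five arrows fanned at BeginPlay by configurable spacing and angle, with special eye shots using random middle arrows.
; Hands, eye shots and a spawned fake eye receive a boss reference.
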(event OnComponentBeginOverlap(BossActivationTrigger)
  (params (OverlappedComponent :type Primitive%20Component%20Object%20Reference) (OtherActor :type Actor%20Object%20Reference) (OtherComp :type Primitive%20Component%20Object%20Reference) (OtherBodyIndex :type Integer) (bFromSweep :type Boolean) (SweepResult :type Hit%20Result%20Structure%20%28by%20ref%29))
  ;[1 1 1] Boss Acrivation
  (if (and (== OtherActor (Game|GetPlayerCharacter 0)) (not (Variables|Default|GetBoss%20Activated)))
    (Variables|Default|SetBoss%20Activated true)
    (Utilities|FlowControl|Delay (Variables|Default|GetWait%20before%20Activation))
    (CallFunction|ActivatePhase (Variables|Default|GetActualPhase))))

(event Custom|Shoot
  (params (ShootPoint :type Integer) (IsEye :type Boolean))
  (bind _returnvalue (Math|Random|RandomIntegerinRange 0 2))
  (bind _arrow0 (Variables|Default|GetArrow0))
  (bind _arrow2 (Variables|Default|GetArrow2))
  (bind _arrow3 (Variables|Default|GetArrow3))
  (bind _arrow4 (Variables|Default|GetArrow4))
  (bind _arrow1 (Variables|Default|GetArrow1))
  (bind _arrow2_2 (Variables|Default|GetArrow2))
  (bind _arrow3_2 (Variables|Default|GetArrow3))
  (bind _arrow1_2 (Variables|Default|GetArrow1))
  (bind _returnvalue_2 (Utilities|Select :Index _returnvalue :Option%200 _arrow1_2 :Option%201 _arrow2_2 :Option%202 _arrow3_2))
  (bind _returnvalue_3 (Utilities|Select :Index ShootPoint :Option%200 _arrow0 :Option%201 _arrow1 :Option%202 _arrow2 :Option%203 _arrow3 :Option%204 _arrow4))
  (bind _returnvalue_4 (Transformation|GetWorldTransform _returnvalue_2))
  (bind _returnvalue_5 (Transformation|GetWorldTransform _returnvalue_3))
  ;[1 0.3604 0.9248] Shooting mechanic
  (if IsEye
    (bind _returnvalue_6 (Game|SpawnActorfromClass "/Game/TBOProject/Design_Blueprint/Blueprints/TESTING/BP_BulletSestr.BP_BulletSestr_C" (Math|Transform|MakeTransform (.location _returnvalue_4) (.rotation _returnvalue_4) "1.000000,1.000000,1.000000") "AlwaysSpawn" "MultiplyWithRoot" 0 0))
    (Variables|/Game/TBOProject/Design_Blueprint/Blueprints/TESTING/BP_BulletSestr.BP_BulletSestr_C|SetBossRef _returnvalue_6 self)
    (Variables|/Game/TBOProject/Design_Blueprint/Blueprints/TESTING/BP_BulletSestr.BP_BulletSestr_C|SetLifeTime _returnvalue_6 (Variables|Shooting|GetWait%20before%20pattern%20restart))
    (else
      (bind _returnvalue_7 (Game|SpawnActorfromClass "/Game/TBOProject/Design_Blueprint/Blueprints/TESTING/BP_Bullet_Designers.BP_Bullet_Designers_C" (Math|Transform|MakeTransform (.location _returnvalue_5) (.rotation _returnvalue_5) "1.000000,1.000000,1.000000") "AlwaysSpawn" "MultiplyWithRoot" 0 0))
      (Variables|/Game/TBOProject/Design_Blueprint/Blueprints/TESTING/BP_Bullet_Designers.BP_Bullet_Designers_C|SetLifeTime _returnvalue_7 (Variables|Shooting|GetWait%20before%20pattern%20restart)))))

(event Custom|SetAngleBetweenMuzzle
  (bind _arrowangle (Variables|Arrow|GetArrowAngle))
  (bind _arrowangle_2 (Variables|Arrow|GetArrowAngle))
  (bind _returnvalue (* _arrowangle 2.0))
  ;[1 1 1] Angle of the arrow of projectiles
  (Transformation|SetRelativeRotation (Variables|Default|GetArrow1) (Math|Rotator|MakeRotator 0.0 0.0 _arrowangle_2) false false)
  (Transformation|SetRelativeRotation (Variables|Default|GetArrow3) (Math|Rotator|MakeRotator 0.0 0.0 (* _arrowangle_2 -1.0)) false false)
  (Transformation|SetRelativeRotation (Variables|Default|GetArrow0) (Math|Rotator|MakeRotator 0.0 0.0 _returnvalue) false false)
  (Transformation|SetRelativeRotation (Variables|Default|GetArrow4) (Math|Rotator|MakeRotator 0.0 0.0 (* _returnvalue -1.0)) false false))

(event Custom|Phase_3
  ;[1 1 1] Phase 3
  (CallFunction|Shoot 2 false)
  (Utilities|FlowControl|Delay (Variables|Burst|GetBurstCadence))
  (CallFunction|Shoot 2 false)
  (Utilities|FlowControl|Delay (Variables|Burst|GetBurstCadence))
  (CallFunction|Shoot 2 false)
  (Utilities|FlowControl|Delay (Variables|Shooting|GetGeneral%20Shooting%20Cooldown))
  (CallFunction|Shoot 0 false)
  (CallFunction|Shoot 2 false)
  (CallFunction|Shoot 4 false)
  (Utilities|FlowControl|Delay (Variables|Shooting|GetGeneral%20Shooting%20Cooldown))
  (CallFunction|Shoot 1 false)
  (CallFunction|Shoot 3 false)
  (CallFunction|Shoot 0 false)
  (CallFunction|Shoot 2 false)
  (CallFunction|Shoot 4 false)
  (Utilities|FlowControl|Delay (Variables|Shooting|GetGeneral%20Shooting%20Cooldown))
  (CallFunction|Shoot 2 true)
  (Utilities|FlowControl|Delay (Variables|Shooting|GetWait%20before%20pattern%20restart))
  (if (== (Variables|Default|GetActualPhase) 3)
    (CallFunction|Phase3)))

(event Custom|ChangePhase
  (bind _actualphase (Variables|Default|GetActualPhase))
  ;[1 1 1] Change phase
  (Math|Integer|IncrementInt _actualphase
    (:%20%20
      (if (== _actualphase 5)
        (Actor|DestroyActor (Variables|Default|GetRightHand))
        (Actor|DestroyActor)
        (else
          (CallFunction|ActivatePhase _actualphase))))))

(event Custom|Phase_1
  ;[1 1 1] Phase 1
  (CallFunction|Shoot 0 false)
  (CallFunction|Shoot 2 false)
  (CallFunction|Shoot 4 false)
  (Utilities|FlowControl|Delay (Variables|Shooting|GetGeneral%20Shooting%20Cooldown))
  (CallFunction|Shoot 1 false)
  (CallFunction|Shoot 3 false)
  (Utilities|FlowControl|Delay (Variables|Shooting|GetGeneral%20Shooting%20Cooldown))
  (CallFunction|Shoot 1 true)
  (Utilities|FlowControl|Delay (Variables|Shooting|GetWait%20before%20pattern%20restart))
  (if (== (Variables|Default|GetActualPhase) 1)
    (CallFunction|Phase1)))

(event Custom|SetDistance%20between%20Muzzle
  (bind _arrow1 (Variables|Default|GetArrow1))
  (bind _distancebetweenarrows (Variables|Arrow|GetDistanceBetweenArrows))
  (bind _arrow3 (Variables|Default|GetArrow3))
  (bind _arrow0 (Variables|Default|GetArrow0))
  (bind _arrow4 (Variables|Default|GetArrow4))
  (bind _distancebetweenarrows_2 (Variables|Arrow|GetDistanceBetweenArrows))
  (bind _returnvalue (Transformation|GetWorldLocation _arrow4))
  (bind _returnvalue_2 (Transformation|GetWorldLocation _arrow1))
  (bind _returnvalue_3 (Transformation|GetWorldLocation _arrow3))
  (bind _returnvalue_4 (Transformation|GetWorldLocation _arrow0))
  (bind _returnvalue_5 (* _distancebetweenarrows_2 2.0))
  ;[1 1 1] Distance between arrows of projectiles
  (Transformation|SetWorldLocation _arrow1 (Math|Vector|MakeVector (.x _returnvalue_2) (+ (.y _returnvalue_2) _distancebetweenarrows) (.z _returnvalue_2)) false false)
  (Transformation|SetWorldLocation _arrow3 (Math|Vector|MakeVector (.x _returnvalue_3) (+ (.y _returnvalue_3) (* _distancebetweenarrows -1.0)) (.z _returnvalue_3)) false false)
  (Transformation|SetWorldLocation _arrow0 (Math|Vector|MakeVector (.x _returnvalue_4) (+ (.y _returnvalue_4) _returnvalue_5) (.z _returnvalue_4)) false false)
  (Transformation|SetWorldLocation _arrow4 (Math|Vector|MakeVector (.x _returnvalue) (+ (.y _returnvalue) (* _returnvalue_5 -1.0)) (.z _returnvalue)) false false))

(event Custom|ActivatePhase
  (params (Selection :type Integer))
  ;[1 1 1] Phase Activation
  (switch int Selection
    (:1
      (CallFunction|Phase1))
    (:2
      (Default|PhaseActivation (Variables|Default|GetLeftHand))
      (Components|DestroyComponent (Variables|Default|GetSphere1)))
    (:3
      ;;[1 0 0] DO NOT REMOVE
      (Utilities|FlowControl|Delay 0.2)
      (Actor|DestroyActor (Variables|Default|GetmOUSE))
      (CallFunction|Phase3)
      (Components|DestroyComponent (Variables|Default|GetSphere)))
    (:4
      (Default|PhaseActivation (Variables|Default|GetRightHand)))))

(event EventBeginPlay
  (bind _self self)
  (bind _centraleyepoint (Variables|Default|GetCentralEyePoint))
  (bind _returnvalue (Transformation|GetWorldTransform _centraleyepoint))
  (CallFunction|SetDistanceBetweenMuzzle)
  (CallFunction|SetAngleBetweenMuzzle)
  (Variables|/Game/TBOProject/Design_Blueprint/Blueprints/TESTING/BP_BreakableHand_Cami.BP_BreakableHand_Cami_C|SetBossRef (Variables|Default|GetLeftHand) _self)
  (Variables|/Game/TBOProject/Design_Blueprint/Blueprints/TESTING/BP_BreakableHand_Cami.BP_BreakableHand_Cami_C|SetBossRef (Variables|Default|GetRightHand) _self)
  (bind _returnvalue_2 (Game|SpawnActorfromClass "/Game/TBOProject/Design_Blueprint/Blueprints/TESTING/BP_fakeEye.BP_fakeEye_C" (Math|Transform|MakeTransform (.location _returnvalue) (.rotation _returnvalue) "3.000000,3.000000,3.000000") "AlwaysSpawn" "MultiplyWithRoot" 0 0))
  (Variables|/Game/TBOProject/Design_Blueprint/Blueprints/TESTING/BP_fakeEye.BP_fakeEye_C|SetBossRef _returnvalue_2 self))

(fn ConstructionScript)
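; Placeable window actor that snaps itself to a nearby wall when play begins, with a randomly chosen round or square mesh.
; BeginPlay picks the mesh, then runs a short sphere trace at its own location to find the surface.
; The root aligns to the hit normal at DistanceFromWall, and the window shifts sideways by WeaponLocation and turns 180 degrees in yaw.
; The hit result is never checked, and the Mesh override is unconnected.
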(event Custom|RandomizeWindow
  (bind _window (Variables|Default|GetWindow))
  (if (== (Math|Random|RandomIntegerinRange 0 1) 0)
    (Components|StaticMesh|SetStaticMesh _window "/Game/TBOProject/Art/Enviroment/StaticMesh_Enviroment/SM_WindowRound.SM_WindowRound")
    (else
      (Components|StaticMesh|SetStaticMesh _window "/Game/TBOProject/Art/Enviroment/StaticMesh_Enviroment/SM_WindowSquare.SM_WindowSquare"))))

(event EventBeginPlay
  (bind _defaultsceneroot (Variables|Default|GetDefaultSceneRoot))
  (bind _window (Variables|Default|GetWindow))
  (bind _returnvalue (Transformation|GetWorldLocation _defaultsceneroot))
  (bind _returnvalue_2 (Transformation|GetWorldRotation _window))
  (CallFunction|RandomizeWindow)
  (bind _outhit (Collision|SphereTraceByChannel _returnvalue (+ _returnvalue "1.000000,1.000000,1.000000") 3e+01 "TraceTypeQuery1" false 0 "None"))
  (Variables|Default|SetOut%20Hit%20Impact%20Point (.impactpoint _outhit))
  (bind _output_get (Variables|Default|SetRotationFromXVector (Math|Conversions|RotationFromXVector (.normal _outhit))))
  (Transformation|SetWorldTransform (Variables|Default|GetDefaultSceneRoot) (Math|Transform|MakeTransform (+ (.impactpoint _outhit) (* (Math|Vector|GetForwardVector (Math|Conversions|RotationFromXVector (.normal _outhit))) (Variables|Default|GetDistanceFromWall))) _output_get "1.000000,1.000000,1.000000") false false)
  (Transformation|SetWorldTransform (Variables|Default|GetWindow) (Math|Transform|MakeTransform (+ (Variables|Default|GetOut%20Hit%20Impact%20Point) (* (Math|Vector|GetRightVector (Variables|Default|GetRotationFromXVector)) (Variables|Default|GetWeaponLocation))) (Math|Rotator|MakeRotator (.roll _returnvalue_2) (.pitch _returnvalue_2) (+ (.yaw _returnvalue_2) 1.8e+02)) "1.000000,1.000000,1.000000") false false))

(event Collision|EventActorBeginOverlap
  (params (OtherActor :type Actor%20Object%20Reference)))

(event EventTick
  (params (DeltaSeconds :type Float%20%28single-precision%29)))

(fn ConstructionScript)
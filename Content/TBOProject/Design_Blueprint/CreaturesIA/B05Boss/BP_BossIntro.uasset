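; Boss intro and arena manager for the B05 boss fight, driven by the boss head controller's phase changes.
; Entering while the boss sleeps switches to boss music, reframes the camera and locks input, then a timer advances the phase; Phase 1 adjusts the camera and restores input.
; Each phase activates its elevator platforms, Intro closes the starting elevator door, and Death resets both and changes the music.
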(event Custom|OnPhaseChange_Event
  (params (BossPhase :type EBossPhase%20Enum :default "Sleep"))
  (bind _game_camera (Variables|Default|GetGame%20Camera))
  (switch Utilities|FlowControl|Switch|SwitchonEBossPhase BossPhase
    (:Phase1
      (Class|GameCamera|SetManualOffset _game_camera (Variables|CameraAfterIntro|GetOffset%20After%20Intro) false)
      (Class|GameCamera|ChangeRotation _game_camera (Variables|CameraAfterIntro|GetRotation%20After%20Intro))
      (Class|GameCamera|ChangeLenght _game_camera (Variables|CameraAfterIntro|GetLenghtAfterIntro))
      (Class|CharacterController|ToggleInput (.AsBP%20Character%20Controller (Utilities|Casting|CastToBP_CharacterController (Game|GetPlayerController 0))) true))))

(event Custom|CustomEvent
  (bind _as_bp_b05_boss_head_controller (Variables|Default|GetAs%20BP%20B05%20Boss%20Head%20Controller))
  (Class|B05BossHeadController|NextPhase _as_bp_b05_boss_head_controller)
  (EventDispatchers|AssignOnPhaseChange _as_bp_b05_boss_head_controller (delegate Custom|OnPhaseChange_Event)))

(event Custom|ManagePlatforms
  (params (Activate :type Boolean) (InstantAction :type Boolean) (Phase :type Integer))
  (for _array_element (Utilities|Select :Index Phase :Option%200 0 :Option%201 (Variables|Default|GetElevators_Phase_1) :Option%202 (Variables|Default|GetElevators_Phase_2) :Option%203 (Variables|Default|GetElevators_Phase_3) :Option%204 (Variables|Default|GetElevators_Phase_4))
    (if (Utilities|IsValid _array_element)
      (if Activate
        (Class|ActionableActor|ActivateActor _array_element InstantAction)
        (else
          (Class|ActionableActor|DeActivateActor _array_element InstantAction))))))

(event Custom|ManageInteractables
  (params (BossPhase :type EBossPhase%20Enum :default "Sleep"))
  (switch Utilities|FlowControl|Switch|SwitchonEBossPhase BossPhase
    (:Intro
      (CallFunction|ManageDoor true false))
    (:Phase1
      (CallFunction|ManagePlatforms true false 1))
    (:Phase2
      (CallFunction|ManagePlatforms true false 2))
    (:Phase3
      (CallFunction|ManagePlatforms true false 3))
    (:Phase4
      (CallFunction|ManagePlatforms true false 4))
    (:Death
      (CallFunction|ManageDoor false false)
      (CallFunction|ManagePlatforms false false 1)
      (CallFunction|ManagePlatforms false false 2)
      (CallFunction|ManagePlatforms false false 3)
      (CallFunction|ManagePlatforms false false 4)
      (CallFunction|ChangeMusicEvent "SFX_Extra2"))))

(event Custom|ManageDoor
  (params (Close :type Boolean) (InstantAction :type Boolean))
  (bind _starting_elevator (Variables|Default|GetStarting_Elevator)
    (:then
      (if Close
        (Class|ActionableActor|ActivateActor _starting_elevator InstantAction)
        (else
          (Class|ActionableActor|DeActivateActor _starting_elevator InstantAction))))
    (:else)))

(event Custom|ChangeMusicEvent
  (params (Music :type ESFXType%20Enum :default "SFX_MainMenu"))
  ;[1 1 1] change music custom event
  (Class|AudioSubsystem|ChangeMusic (Subsystems|GetAudioSubsystem) Music))

(event EventBeginPlay
  (Utilities|FlowControl|Delay 0.1)
  (bind _bosshead (Variables|Default|GetBossHead)
    (:then
      (bind _asbp_b05_boss_head_controller (Utilities|Casting|CastToBP_B05_BossHead_Controller (Pawn|GetController _bosshead)))
      (Variables|Default|SetAs%20BP%20B05%20Boss%20Head%20Controller _asbp_b05_boss_head_controller)
      (EventDispatchers|AssignOnPhaseChange (Variables|Default|GetAs%20BP%20B05%20Boss%20Head%20Controller) (delegate Custom|ManageInteractables))
      (switch Utilities|FlowControl|Switch|SwitchonEBossPhase (Variables|/Script/TBO_01.B05_BossHead_Controller|GetCurrentPhase (Variables|Default|GetAs%20BP%20B05%20Boss%20Head%20Controller))
        (:Sleep
          _)))
    (:else
      _))
  (CallFunction|ManageDoor false true)
  (CallFunction|ManagePlatforms false true 1)
  (CallFunction|ManagePlatforms false true 2)
  (CallFunction|ManagePlatforms false true 3)
  (CallFunction|ManagePlatforms false true 4))

(event EventOnCharacterEnter
  (params (GameCamera :type Game%20Camera%20Object%20Reference))
  (bind _returnvalue (Game|GetPlayerController 0))
  (bind _asbp_character_controller (Utilities|Casting|CastToBP_CharacterController _returnvalue))
  (Variables|Default|SetGame%20Camera GameCamera)
  (bind _as_bp_b05_boss_head_controller (Variables|Default|GetAs%20BP%20B05%20Boss%20Head%20Controller)
    (:then
      (switch Utilities|FlowControl|Switch|SwitchonEBossPhase (Variables|/Script/TBO_01.B05_BossHead_Controller|GetCurrentPhase _as_bp_b05_boss_head_controller)
        (:Sleep
          (CallFunction|ChangeMusicEvent "SFX_Boss")
          (Class|GameCamera|SetManualOffset (Variables|Default|GetGame%20Camera) (Variables|CameraIntro|GetOffset%20during%20Intro) true)
          (Class|GameCamera|ChangeRotation (Variables|Default|GetGame%20Camera) (Variables|CameraIntro|GetRotation%20during%20Intro))
          (Class|CharacterController|ToggleInput _asbp_character_controller false)
          (Variables|/Game/TBOProject/Core/Characters/Player/BP_CharacterController.BP_CharacterController_C|SetBossfightActivated _asbp_character_controller true)
          (Utilities|Time|SetTimerbyEvent (delegate Custom|CustomEvent) (Variables|Default|GetTime)))))
    (:else)))

(fn ConstructionScript)